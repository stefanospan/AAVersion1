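; BP_CombatTarget is an actor that serves as a combat target with team and stat components and a floating health widget.
; On BeginPlay, where cosmetic events can run, it binds the stat component to the WBP_Stat widget.
; Each Tick it rotates the widget to face the local player camera.
; GetTeam exposes the team component's value.
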(event `self.ReceiveBeginPlay`
  (`/Engine/EditorBlueprintResources/StandardMacros.Can Execute Cosmetic Events`
    (:`True`
      (bind _aswbp_stat (cast `/Game/Core/Widgets/Gameplay/Stat/WBP_Stat` (`WidgetComponent.GetUserWidgetObject` (`self.HealthWidget`))))
      (`/Game/Core/Widgets/Gameplay/Stat/WBP_Stat.InitStatComponent` _aswbp_stat (`self.BPC_StatComponent`)))))

(event `self.ReceiveTick`
  (params (DeltaSeconds :type "Float (single-precision)"))
  (`/Engine/EditorBlueprintResources/StandardMacros.Can Execute Cosmetic Events`
    (:`True`
      (`SceneComponent.K2_SetWorldRotation` (`self.HealthWidget`) (`KismetMathLibrary.FindLookAtRotation` (`SceneComponent.K2_GetComponentLocation` (`self.HealthWidget`)) (`self.K2_GetActorLocation` (`GameplayStatics.GetPlayerCameraManager` 0))) false false))))

(fn `GetTeam`
  (returns (Team :type Integer))
  (return (`/Game/Core/Blueprints/Gameplay/Components/TeamComponent/BPC_TeamComponent.GetTeam` (`self.BPC_TeamComponent`))))

(fn `UserConstructionScript`)