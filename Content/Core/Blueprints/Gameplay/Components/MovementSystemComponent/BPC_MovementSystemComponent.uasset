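; BPC_MovementSystemComponent is an actor component that drives a Character's walk speed from its MoveSpeed attribute.
; On BeginPlay it caches the owning Character, finds its BPC_AttributeComponent and binds to its attribute update event, then applies the current values once.
; Each update sets MaxWalkSpeed to DefaultSpeed scaled by the MoveSpeed attribute, and setup stops if the owner is not a Character.
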(event `self.ReceiveBeginPlay`
  (`self.Init`))

(fn `Init`
  (bind _attributecomponent (`self.AttributeComponent`))
  (bind _ascharacter (cast `Character` (`self.GetOwner`)))
  (set `self.OwnerCharacter` _ascharacter)
  (set `self.AttributeComponent` (`Actor.GetComponentByClass` (`self.GetOwner`) "/Game/Core/Blueprints/Gameplay/Components/AttributeComponent/BPC_AttributeComponent.BPC_AttributeComponent_C"))
  (add `/Game/Core/Blueprints/Gameplay/Components/AttributeComponent/BPC_AttributeComponent.OnUpdatedAttributes` _attributecomponent (`|CreateDelegate` :!event `OnUpdatedAttributes`))
  (`self.OnUpdatedAttributes` (`/Game/Core/Blueprints/Gameplay/Components/AttributeComponent/BPC_AttributeComponent.GetAttributes` _attributecomponent)))

(fn `OnUpdatedAttributes`
  (params (Attributes :type "Array of /Game/Core/Blueprints/Gameplay/Components/AttributeComponent/Structures/ST_AttributeData Structure (by ref)"))
  (set `CharacterMovementComponent.MaxWalkSpeed` (* (`self.DefaultSpeed`) (`.Value_5_5382FAD64776275FF614BEB1A224EFA3` (break `/Game/Core/Blueprints/Gameplay/Components/AttributeComponent/Structures/ST_AttributeData` (`/Game/Core/Blueprints/Gameplay/Components/AttributeComponent/BPC_AttributeComponent.GetAttribute` (`self.AttributeComponent`) (struct :`TagName` "Attribute.MoveSpeed"))))) (`Character.CharacterMovement` (`self.OwnerCharacter`))))