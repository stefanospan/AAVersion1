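; Actor component that tracks a player's or owner's rune fragment count as a replicated currency.
; Add and Remove functions adjust the count, with removal clamped so it never drops below zero.
; A RepNotify on the count fires an updated dispatcher so listeners receive the new value, and a getter exposes the current amount.
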(fn `AddRuneFragments`
  (params (Amount :type Integer))
  (set `self.CurrentRuneFragments` (+ Amount (`self.CurrentRuneFragments`))))

(fn `GetCurrentRuneFragments`
  (returns (CurrentRuneFragments :type Integer))
  (return (`self.CurrentRuneFragments`)))

(fn `OnRep_CurrentRuneFragments`
  (`self.OnUpdatedCurrentRuneFragments` (`self.CurrentRuneFragments`)))

(fn `RemoveRuneFragments`
  (params (Amount :type Integer))
  (set `self.CurrentRuneFragments` (`KismetMathLibrary.Max` (- (`self.CurrentRuneFragments`) Amount))))