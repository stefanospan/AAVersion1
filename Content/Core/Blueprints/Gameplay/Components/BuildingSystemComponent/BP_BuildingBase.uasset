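; Base actor for placeable buildings that constructs itself over time and is destroyed when its stat component reports death.
; The authority advances build progress each tick using the build time from BuildingData, and the OnRep broadcasts the value through an update dispatcher.
; Where cosmetic events can run, it initializes a world-space stat widget, shows it only near the local camera and rotates it to face that camera.
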(event `self.ReceiveBeginPlay`
  (`/Engine/EditorBlueprintResources/StandardMacros.Can Execute Cosmetic Events`
    (:`True`
      (bind _aswbp_building_stat (cast `/Game/Core/Blueprints/Gameplay/Components/BuildingSystemComponent/WBP_BuildingStat` (`WidgetComponent.GetUserWidgetObject` (`self.StatWidget`))))
      (`/Game/Core/Blueprints/Gameplay/Components/BuildingSystemComponent/WBP_BuildingStat.InitBuilding` _aswbp_building_stat self))))

(event `self.ReceiveTick`
  (params (DeltaSeconds :type "Float (single-precision)"))
  (bind _returnvalue (<= (`KismetMathLibrary.Vector_Distance` (`self.K2_GetActorLocation` (`GameplayStatics.GetPlayerCameraManager` 0)) (`self.K2_GetActorLocation`)) 850.0))
  (`|ExecutionSequence`
    (:`then_0`
      (`/Engine/EditorBlueprintResources/ActorMacros.Switch Has Authority`
        (:`Authority`
          (if (< (`self.CurrentBuildProgress`) 1.0)
            (set `self.CurrentBuildProgress` (`KismetMathLibrary.FMin` (+ (`self.CurrentBuildProgress`) (* DeltaSeconds (/ 1.0 (`.BuildTime_17_4B58D9D740CF11516C6C4393D8CFCC6F` (break `/Game/Core/Blueprints/Gameplay/Components/BuildingSystemComponent/Structures/ST_BuildingData` (`self.BuildingData`)))))) 1.0))))))
    (:`then_1`
      (`/Engine/EditorBlueprintResources/StandardMacros.Can Execute Cosmetic Events`
        (:`True`
          (`|ExecutionSequence`
            (:`then_0`
              (if (!= _returnvalue (`SceneComponent.IsVisible` (`self.StatWidget`)))
                (`SceneComponent.SetVisibility` (`self.StatWidget`) _returnvalue false)))
            (:`then_1`
              (if (`SceneComponent.IsVisible` (`self.StatWidget`))
                (`SceneComponent.K2_SetWorldRotation` (`self.StatWidget`) (`KismetMathLibrary.FindLookAtRotation` (`SceneComponent.K2_GetComponentLocation` (`self.StatWidget`)) (`self.K2_GetActorLocation` (`GameplayStatics.GetPlayerCameraManager` 0))) false false)))))))))

(event `self.BPC_StatComponent.OnDeath`
  (`self.K2_DestroyActor`))

(fn `GetCurrentBuildProgress`
  (returns (CurrentBuildProgress :type "Float (double-precision)"))
  (return (`self.CurrentBuildProgress`)))

(fn `OnRep_CurrentBuildProgress`
  (`self.OnUpdatedCurrentBuildProgress` (`self.CurrentBuildProgress`)))

(fn `UserConstructionScript`)