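; BP_BuildingHologram is the hologram preview actor for the building system, showing a building's mesh and whether its placement is valid.
; The construction script creates a dynamic instance of M_Hologram.
; SetBuilding copies the static mesh from the building class defaults and applies that instance to material slot 0.
; ToggleValidPlacement switches the instance's Color parameter between blue for valid and dark red for invalid.
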(fn `SetBuilding`
  (params (Building :type "/Game/Core/Blueprints/Gameplay/Components/BuildingSystemComponent/BP_BuildingBase Class Reference"))
  (`StaticMeshComponent.SetStaticMesh` (`self.StaticMesh`) (`.StaticMesh_14_3177F2634EA6C11F6805D689A58AEDD6` (break `/Game/Core/Blueprints/Gameplay/Components/BuildingSystemComponent/Structures/ST_BuildingData` (defaults `Object` Building))))
  (`PrimitiveComponent.SetMaterial` (`self.StaticMesh`) 0 (`self.DMI`)))

(fn `ToggleValidPlacement`
  (params (IsValid :type Boolean))
  (`MaterialInstanceDynamic.SetVectorParameterValue` (`self.DMI`) "Color" (select `bool` IsValid :`false` (struct :`R` 0.427083 :`A` 1.0) :`true` (struct :`G` 0.549379 :`B` 1.0 :`A` 1.0) :!type "LinearColor Structure")))

(fn `UserConstructionScript`
  (bind _returnvalue (`KismetMaterialLibrary.CreateDynamicMaterialInstance` "/Game/Core/Blueprints/Gameplay/Components/BuildingSystemComponent/M_Hologram.M_Hologram"))
  (set `self.DMI` _returnvalue))