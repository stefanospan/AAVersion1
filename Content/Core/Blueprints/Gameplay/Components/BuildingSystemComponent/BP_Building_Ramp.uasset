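; BP_Building_Ramp is a wooden ramp piece for the building system, derived from a parent building Blueprint.
; Its construction script runs the parent's script, then registers its Sphere component as a foundation component.
; Damage reported by BPC_StatComponent plays a wood impact sound at the static mesh, and destruction plays a wood destroyed sound there.
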(event `self.BPC_StatComponent.OnReceivedDamage`
  (`GameplayStatics.PlaySoundAtLocation` "/Game/Magic_Spell_SFX_Pack_Vol1/General_Spells_and_Effects/cue/Impact_Wood_01.Impact_Wood_01" (`SceneComponent.GetSocketLocation` (`self.StaticMesh`) "None") (struct) 0.8 1.0 0.0 null null null null))

(event `self.ReceiveDestroyed`
  (`GameplayStatics.PlaySoundAtLocation` "/Game/Magic_Spell_SFX_Pack_Vol1/Additional_and_Loops/cue/Destroyed_Wood_01.Destroyed_Wood_01" (`SceneComponent.GetSocketLocation` (`self.StaticMesh`) "None") (struct) 0.8 1.0 0.0 null null null null))

(fn `UserConstructionScript`
  (`parent.UserConstructionScript`)
  (`self.RegisterFoundationComponents` (`|MakeArray` (`self.Sphere`))))