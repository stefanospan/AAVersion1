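; Character component for placing buildings, previewed by a grid-snapped hologram at the camera trace.
; Selecting a building briefly spawns it to cache check transforms; tick then tests free space and landscape or foundation support.
; The server rechecks costs but not placement, consumes items, spawns the building and scales build time and health by attributes.
; One build runs at a time until completion or end play, and placement sound is multicast.
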(event `self.ReceiveBeginPlay`
  ; Init
  (`self.Init`))

(event `self.ReceiveTick`
  (params (DeltaSeconds :type "Float (single-precision)"))
  ; Tick
  (`self.HandleBuilding`))

(event `ServerPlace`
  (params (Building :type "/Game/Core/Blueprints/Gameplay/Components/BuildingSystemComponent/BP_BuildingBase Class Reference") (Transform :type "Transform Structure"))
  ; Handles placing building on server
  (if (`self.CanBuildBuilding` Building)
    (`self.ConsumeBuildingCosts` Building)
    (bind _returnvalue (`|SpawnActorFromClass` Building Transform "AlwaysSpawn" "MultiplyWithRoot" null null))
    (bind _buildingdata (`/Game/Core/Blueprints/Gameplay/Components/BuildingSystemComponent/BP_BuildingBase.BuildingData` _returnvalue))
    (setmembers `/Game/Core/Blueprints/Gameplay/Components/BuildingSystemComponent/Structures/ST_BuildingData` :`StructRef` _buildingdata :`BuildTime` (* (`.BuildTime_17_4B58D9D740CF11516C6C4393D8CFCC6F` (break `/Game/Core/Blueprints/Gameplay/Components/BuildingSystemComponent/Structures/ST_BuildingData` _buildingdata)) (`.Value_5_5382FAD64776275FF614BEB1A224EFA3` (break `/Game/Core/Blueprints/Gameplay/Components/AttributeComponent/Structures/ST_AttributeData` (`/Game/Core/Blueprints/Gameplay/Components/AttributeComponent/BPC_AttributeComponent.GetAttribute` (`self.AttributeComponent`) (struct :`TagName` "Attribute.BuildingTimeMultiplier"))))))
    (bind _bpc_statcomponent (`/Game/Core/Blueprints/Gameplay/Components/BuildingSystemComponent/BP_BuildingBase.BPC_StatComponent` _returnvalue))
    (`/Game/Core/Blueprints/Gameplay/Components/StatComponent/BPC_StatComponent.SetStatMaxValue` _bpc_statcomponent (struct :`TagName` "Stat.Health") (* (`.MaxValue_9_B98E4DE245B99F0442DD6F99ED378288` (break `/Game/Core/Blueprints/Gameplay/Components/StatComponent/Structures/ST_StatDefinitionData` (`/Game/Core/Blueprints/Gameplay/Components/StatComponent/BPC_StatComponent.GetStatDefinition` _bpc_statcomponent (struct :`TagName` "Stat.Health")))) (`.Value_5_5382FAD64776275FF614BEB1A224EFA3` (break `/Game/Core/Blueprints/Gameplay/Components/AttributeComponent/Structures/ST_AttributeData` (`/Game/Core/Blueprints/Gameplay/Components/AttributeComponent/BPC_AttributeComponent.GetAttribute` (`self.AttributeComponent`) (struct :`TagName` "Attribute.BuildingHealthMultiplier"))))) false)
    (add `/Game/Core/Blueprints/Gameplay/Components/BuildingSystemComponent/BP_BuildingBase.OnBuildingCompleted` _returnvalue (`|CreateDelegate` :!event `OnBuildingCompleted`))
    (add `Actor.OnEndPlay` _returnvalue (`|CreateDelegate` :!event `OnBuildingEndPlay`))
    (set `self.IsBuildingInProgress` true)
    (`self.MulticastPlace`)))

(event `MulticastPlace`
  ; Plays for all except dedicated and local player
  (if (not (`Pawn.IsLocallyControlled` (`self.OwnerCharacter`)))
    (`/Engine/EditorBlueprintResources/StandardMacros.Can Execute Cosmetic Events`
      (:`True`
        (`GameplayStatics.PlaySoundAtLocation` (`self.BuildingPlaceSound`) (`Actor.K2_GetActorLocation` (`self.GetOwner`)) (struct) 1.0 1.0 0.0 "/Game/UltraDynamicSky/Sound/Attenuation/UDS_Interact_Sound_Attenuation.UDS_Interact_Sound_Attenuation" null null null)))))

(fn `CanBuildBuilding`
  (params (Building :type "/Game/Core/Blueprints/Gameplay/Components/BuildingSystemComponent/BP_BuildingBase Class Reference"))
  (returns (Success :type Boolean))
  (if (`self.IsBuildingInProgress`)
    (return false)
    (else
      (`|ExecutionSequence`
        (:`then_0`
          (for _array_element (`.Cost_10_3495C4A24CEB849D9FE78889E6295DC5` (break `/Game/Core/Blueprints/Gameplay/Components/BuildingSystemComponent/Structures/ST_BuildingData` (defaults `Object` (`local.Building`))))
            (bind (_item _amount) (break `/Game/Core/Blueprints/Gameplay/Components/InventoryComponent/Structures/ST_InventorySlot` _array_element))
            (if (not (>= (`/Game/Core/Blueprints/Gameplay/Components/InventoryComponent/BPC_InventoryComponent.GetAmountForItem` (`self.InventoryComponent`) _item) _amount))
              (return false))))
        (:`then_1`
          (return true))))))

(fn `ConsumeBuildingCosts`
  (params (Building :type "/Game/Core/Blueprints/Gameplay/Components/BuildingSystemComponent/BP_BuildingBase Class Reference"))
  (for _array_element (`.Cost_10_3495C4A24CEB849D9FE78889E6295DC5` (break `/Game/Core/Blueprints/Gameplay/Components/BuildingSystemComponent/Structures/ST_BuildingData` (defaults `Object` Building)))
    (bind (_item _amount) (break `/Game/Core/Blueprints/Gameplay/Components/InventoryComponent/Structures/ST_InventorySlot` _array_element))
    (`/Game/Core/Blueprints/Gameplay/Components/InventoryComponent/BPC_InventoryComponent.RemoveItem` (`self.InventoryComponent`) _item _amount)))

(fn `GetBuildingTransform`
  (returns (Transform :type "Transform Structure"))
  (bind _gridsize (`self.GridSize`))
  (return (`KismetMathLibrary.MakeTransform` (`KismetMathLibrary.MakeVector` (`KismetMathLibrary.GridSnap_Float` (.x (`self.GetCameraHitLocation`)) _gridsize) (`KismetMathLibrary.GridSnap_Float` (.y (`self.GetCameraHitLocation`)) _gridsize) (`KismetMathLibrary.GridSnap_Float` (.z (`self.GetCameraHitLocation`)) _gridsize)) (`KismetMathLibrary.MakeRotator` 0.0 0.0 (`KismetMathLibrary.GridSnap_Float` (.yaw (`Actor.K2_GetActorRotation` (`GameplayStatics.GetPlayerCameraManager` 0))) 90.0)))))

(fn `GetCameraHitLocation`
  (returns (Location :type "Vector Structure"))
  (bind _returnvalue (`Actor.K2_GetActorLocation` (`self.GetOwner`)))
  (bind _outhit (`KismetSystemLibrary.LineTraceSingle` :`Start` _returnvalue :`End` (+ _returnvalue (* (`Actor.GetActorForwardVector` (`GameplayStatics.GetPlayerCameraManager` 0)) (`self.ForwardOffset`))) :`TraceChannel` "TraceTypeQuery1" :`DrawDebugType` "ForOneFrame"))
  (bind (_bblockinghit _binitialoverlap _time _distance _location _impactpoint _normal _impactnormal _physmat _hitactor _hitcomponent _hitbonename _bonename _hititem _elementindex _faceindex _tracestart _traceend) (`GameplayStatics.BreakHitResult` _outhit))
  (return (select `bool` _bblockinghit :`false` _traceend :`true` _location)))

(fn `GetHologramActor`
  (returns (HologramActor :type "/Game/Core/Blueprints/Gameplay/Components/BuildingSystemComponent/BP_BuildingHologram Object Reference"))
  (bind _hologramactor (`self.HologramActor`)
    (:`then`
      (return _hologramactor))
    (:`else`
      (bind _returnvalue (`|SpawnActorFromClass` "/Game/Core/Blueprints/Gameplay/Components/BuildingSystemComponent/BP_BuildingHologram.BP_BuildingHologram_C" (`KismetMathLibrary.MakeTransform` (0.0 0.0 0.0)) "AlwaysSpawn" "MultiplyWithRoot" null null))
      (bind _output_get (set `self.HologramActor` _returnvalue))
      (return _output_get))))

(fn `GetIsBuilding`
  (returns (IsBuilding :type Boolean))
  (return (`self.IsBuilding`)))

(fn `GetSelectedBuilding`
  (returns (SelectedBuilding :type Integer))
  (return (`self.SelectedBuilding`)))

(fn `HandleBuilding`
  (locals (Found :type Boolean))
  (bind _placementlocationchecktransform_location (`KismetMathLibrary.BreakTransform` (`self.PlacementLocationCheckTransform`)))
  (if (`self.IsBuilding`)
    (`|ExecutionSequence`
      (:`then_0`
        (`Actor.K2_SetActorTransform` (`self.GetHologramActor`) (`self.GetBuildingTransform`) false false))
      (:`then_1`
        (if (`self.IsLocationFree` (`KismetMathLibrary.TransformLocation` (`Actor.GetTransform` (`self.GetHologramActor`)) _placementlocationchecktransform_location))
          (if (> (`KismetArrayLibrary.Array_Length` (`Actor.GetOverlappingActors` (`self.GetHologramActor`) "/Script/Landscape.Landscape")) 0)
            (set `self.IsValidPlacement` true)
            (else
              (for _array_element (`self.FoundationTransforms`)
                (bind _returnvalue (`KismetMathLibrary.TransformLocation` (`Actor.GetTransform` (`self.GetHologramActor`)) (.location _array_element)))
                (if (or (`self.IsLocationFoundation` _returnvalue) (`self.IsLocationLandscape` _returnvalue))
                  (set `local.Found` true)
                  (set `self.IsValidPlacement` true)))
              (if (not (`local.Found`))
                (set `self.IsValidPlacement` false))))
          (else
            (set `self.IsValidPlacement` false))))
      (:`then_2`
        (`/Game/Core/Blueprints/Gameplay/Components/BuildingSystemComponent/BP_BuildingHologram.ToggleValidPlacement` (`self.GetHologramActor`) (`self.IsValidPlacement`))))))

(fn `Init`
  (`|ExecutionSequence`
    (:`then_0`
      (set `self.InventoryComponent` (`Actor.GetComponentByClass` (`self.GetOwner`) "/Game/Core/Blueprints/Gameplay/Components/InventoryComponent/BPC_InventoryComponent.BPC_InventoryComponent_C")))
    (:`then_1`
      (set `self.AttributeComponent` (`Actor.GetComponentByClass` (`self.GetOwner`) "/Game/Core/Blueprints/Gameplay/Components/AttributeComponent/BPC_AttributeComponent.BPC_AttributeComponent_C")))
    (:`then_2`
      (bind _ascharacter (cast `Character` (`self.GetOwner`)))
      (set `self.OwnerCharacter` _ascharacter))))

(fn `InputPlace`
  (if (`self.IsBuilding`)
    (if (`self.IsBuildingInProgress`)
      _
      (elif (`self.IsValidPlacement`)
        (if (`self.CanBuildBuilding` (`|GetArrayItem` (`self.Buildings`) (`self.SelectedBuilding`)))
          (`self.ServerPlace` (`|GetArrayItem` (`self.Buildings`) (`self.SelectedBuilding`)) (`self.GetBuildingTransform`))
          (`GameplayStatics.PlaySoundAtLocation` (`self.BuildingPlaceSound`) (`Actor.K2_GetActorLocation` (`self.GetOwner`)) (struct) 1.0 1.0 0.0 "/Game/UltraDynamicSky/Sound/Attenuation/UDS_Interact_Sound_Attenuation.UDS_Interact_Sound_Attenuation" null null null))))))

(fn `IsLocationFoundation`
  (params (Location :type "Vector Structure"))
  (returns (Success :type Boolean))
  (bind _outactors (`KismetSystemLibrary.SphereOverlapActors` Location 50.0 (`|MakeArray` "ObjectTypeQuery1" "ObjectTypeQuery2" "ObjectTypeQuery3" :!type "EObjectTypeQuery Enum") "/Game/Core/Blueprints/Gameplay/Components/BuildingSystemComponent/BP_BuildingBase.BP_BuildingBase_C" (`|MakeArray` (`self.HologramActor`) :!type "Actor Object Reference")))
  (return (> (`KismetArrayLibrary.Array_Length` _outactors) 0)))

(fn `IsLocationFree`
  (params (Location :type "Vector Structure"))
  (returns (Success :type Boolean))
  (bind _outactors (`KismetSystemLibrary.SphereOverlapActors` Location 50.0 (`|MakeArray` "ObjectTypeQuery1" "ObjectTypeQuery2" "ObjectTypeQuery3" :!type "EObjectTypeQuery Enum") null (`|MakeArray` (`self.HologramActor`) :!type "Actor Object Reference")))
  (for _array_element _outactors
    (cast `Landscape` _array_element
      (:`CastFailed`
        (if (not (`Actor.ActorHasTag` _array_element "Buildable"))
          (return false)))))
  (return true))

(fn `IsLocationLandscape`
  (params (Location :type "Vector Structure"))
  (returns (Success :type Boolean))
  (bind _outhits (`KismetSystemLibrary.SphereTraceMultiForObjects` Location (+ Location (0.0 0.0 1.0)) 50.0 (`|MakeArray` "ObjectTypeQuery1" "ObjectTypeQuery2" "ObjectTypeQuery3" :!type "EObjectTypeQuery Enum") false (`|MakeArray` (`self.HologramActor`) :!type "Actor Object Reference") "ForOneFrame"))
  (for _array_element _outhits
    (bind (_bblockinghit _binitialoverlap _time _distance _location _impactpoint _normal _impactnormal _physmat _hitactor) (`GameplayStatics.BreakHitResult` _array_element))
    (cast `Landscape` _hitactor
      (:`then`
        (return true))
      (:`CastFailed`
        (if (`Actor.ActorHasTag` _hitactor "Buildable")
          (return true)))))
  (return false))

(fn `OnBuildingCompleted`
  (params (Building :type "/Game/Core/Blueprints/Gameplay/Components/BuildingSystemComponent/BP_BuildingBase Object Reference"))
  (remove `/Game/Core/Blueprints/Gameplay/Components/BuildingSystemComponent/BP_BuildingBase.OnBuildingCompleted` Building (`|CreateDelegate` :!event `OnBuildingCompleted`))
  (remove `Actor.OnEndPlay` (`local.Building`) (`|CreateDelegate` :!event `OnBuildingEndPlay`))
  (set `self.IsBuildingInProgress` false))

(fn `OnBuildingEndPlay`
  (params (Actor :type "Actor Object Reference") (EndPlayReason :type "EEndPlayReason Enum" :default "Destroyed"))
  (bind _asbp_building_base (cast `/Game/Core/Blueprints/Gameplay/Components/BuildingSystemComponent/BP_BuildingBase` Actor))
  (remove `/Game/Core/Blueprints/Gameplay/Components/BuildingSystemComponent/BP_BuildingBase.OnBuildingCompleted` _asbp_building_base (`|CreateDelegate` :!event `OnBuildingCompleted`))
  (remove `Actor.OnEndPlay` _asbp_building_base (`|CreateDelegate` :!event `OnBuildingEndPlay`))
  (set `self.IsBuildingInProgress` false))

(fn `SetSelectedBuilding`
  (params (BuildingIndex :type Integer))
  (locals (Temp :type "/Game/Core/Blueprints/Gameplay/Components/BuildingSystemComponent/BP_BuildingBase Object Reference"))
  (if (!= BuildingIndex (`self.SelectedBuilding`))
    (bind _output_get (set `self.SelectedBuilding` (`local.BuildingIndex`)))
    (`self.OnUpdatedSelectedBuilding` _output_get)
    (set `self.IsBuilding` true)
    (`/Game/Core/Blueprints/Gameplay/Components/BuildingSystemComponent/BP_BuildingHologram.SetBuilding` (`self.GetHologramActor`) (`|GetArrayItem` (`self.Buildings`) (`self.SelectedBuilding`)))
    (`self.SetComponentTickEnabled` true)
    (bind _returnvalue (`|SpawnActorFromClass` (`|GetArrayItem` (`self.Buildings`) (`self.SelectedBuilding`)) (`KismetMathLibrary.MakeTransform` (0.0 0.0 0.0)) "AlwaysSpawn" "MultiplyWithRoot" null null))
    (set `local.Temp` _returnvalue)
    (set `self.PlacementLocationCheckTransform` (`SceneComponent.GetRelativeTransform` (`/Game/Core/Blueprints/Gameplay/Components/BuildingSystemComponent/BP_BuildingBase.PlacementLocationCheck` _returnvalue)))
    (for _array_element (`/Game/Core/Blueprints/Gameplay/Components/BuildingSystemComponent/BP_BuildingBase.GetFoundationComponents` _returnvalue)
      (`KismetArrayLibrary.Array_Add` (`self.FoundationTransforms`) (`SceneComponent.GetRelativeTransform` _array_element)))
    (`Actor.K2_DestroyActor` (`local.Temp`))
    (else
      (`self.StopBuilding`))))

(fn `SnapFloatToGrid`
  (params (FloatIn :type "Float (double-precision)"))
  (returns (FloatOut :type "Float (double-precision)"))
  (return (* (`KismetMathLibrary.FFloor` (/ FloatIn (`self.GridSize`))) (`self.GridSize`))))

(fn `SnapL:ocationToGrid`
  (params (Location :type "Vector Structure"))
  (returns (GridLocation :type "Vector Structure"))
  (return (`KismetMathLibrary.MakeVector` (`self.SnapFloatToGrid` (.x Location)) (`self.SnapFloatToGrid` (.y Location)) (`self.SnapFloatToGrid` (.z Location)))))

(fn `StopBuilding`
  (`|ExecutionSequence`
    (:`then_0`
      (bind _hologramactor (`self.HologramActor`)
        (:`then`
          (`Actor.K2_DestroyActor` _hologramactor)
          (set `self.HologramActor` null))
        (:`else`)))
    (:`then_1`
      (`self.SetComponentTickEnabled` false))
    (:`then_2`
      (set `self.IsBuilding` false))
    (:`then_3`
      (bind _output_get (set `self.SelectedBuilding` -1))
      (`self.OnUpdatedSelectedBuilding` _output_get))))