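; Character component that manages primary/secondary weapon switching, per-slot ammo and aim-down-sights.
; Equipment or slot changes refresh the current weapon; the server swaps its GAS-style ability and returns loaded ammo to inventory, from which Reload draws.
; Aim and slot inputs go through server RPCs, with OnReps updating strafe rotation and weapon.
; A server timer samples control pitch for interpolation, while Tick blends local camera offset and FOV for ADS.
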(event `self.ReceiveBeginPlay`
  ; Init
  (`self.Init`))

(event `ServerSetIsADS`
  (params (IsADS :type Boolean))
  ; Sets ADS on server
  (set `self.IsAiming` IsADS))

(event `ServerSetEquippedSlot`
  (params (EquippedSlot :type "/Game/Core/Blueprints/Gameplay/Components/EquipmentComponent/Enums/E_EquipmentSlots Enum" :default "NewEnumerator0"))
  ; Sets equipped slot on server machine
  (set `self.EquippedSlot` EquippedSlot))

(event `self.ReceiveTick`
  (params (DeltaSeconds :type "Float (single-precision)"))
  ; Tick
  (`self.HandlePitch` DeltaSeconds)
  (`self.HandleADS` DeltaSeconds))

(fn `BroadcastPitch`
  (set `self.TargetPitch` (.pitch (`Pawn.GetControlRotation` (`self.OwnerCharacter`)))))

(fn `CanReload`
  (returns (Success :type Boolean))
  (`self.SwitchOnRangedWeapon`
    (:`IsRanged`
      (if (< (`self.GetCurrentAmmo`) (`.MagazineAmmo_5_12AEF0674BE50D36A1C584A0BE9AA58A` (break `/Game/Core/Blueprints/Gameplay/Components/WeaponSystemComponent/Structures/ST_RangedWeaponItemData` (defaults `Object` (`self.CurrentRangedWeapon`)))))
        (return (> (`/Game/Core/Blueprints/Gameplay/Components/InventoryComponent/BPC_InventoryComponent.GetAmountForItem` (`self.InventoryComponent`) (`.AmmoItem_2_6709851D4FC20DF02EC096B47D4C1DF0` (break `/Game/Core/Blueprints/Gameplay/Components/WeaponSystemComponent/Structures/ST_RangedWeaponItemData` (defaults `Object` (`self.CurrentRangedWeapon`))))) 0))
        (else
          (return false))))
    (:`NotRanged`
      (return false))))

(fn `GetCurrentAmmo`
  (returns (Output :type "Integer (by ref)"))
  (return (`|GetArrayItem` (`self.LoadedAmmo`) (select `bool` (`|EnumEquality` (`self.EquippedSlot`) "NewEnumerator0") :`false` 1))))

(fn `GetCurrentPitch`
  (returns (CurrentPitch :type "Float (double-precision)"))
  (return (`self.CurrentPitch`)))

(fn `GetCurrentRangedWeapon`
  (returns (CurrentRangedWeapon :type "/Game/Core/Blueprints/Gameplay/Components/WeaponSystemComponent/BP_RangedWeaponItemBase Class Reference"))
  (return (`self.CurrentRangedWeapon`)))

(fn `GetCurrentStance`
  (returns (Stance :type "/Game/Core/Blueprints/Gameplay/Components/WeaponSystemComponent/Enums/E_CharacterStances Enum"))
  (`self.EquipmentComponent`
    (:`then`
      (bind _asbp_weapon_item_base (castclass `/Game/Core/Blueprints/Gameplay/Components/WeaponSystemComponent/BP_WeaponItemBase` (`.EquipmentItem_6_6AB0AAAF45B76011F96BD2AAF6AEDC54` (break `/Game/Core/Blueprints/Gameplay/Components/EquipmentComponent/Structures/ST_EquipmentSlot` (`/Game/Core/Blueprints/Gameplay/Components/EquipmentComponent/BPC_EquipmentComponent.GetEquipmentSlot` (`self.EquipmentComponent`) (`self.EquippedSlot`)))))
        (:`then`
          (return (`.Stance_6_232CFC4F486D6F8E0B4361A424CEEC47` (break `/Game/Core/Blueprints/Gameplay/Components/WeaponSystemComponent/Structures/ST_WeaponItemData` (defaults `Object` _asbp_weapon_item_base)))))
        (:`CastFailed`
          _)))
    (:`else`
      _))
  (return "NewEnumerator0"))

(fn `GetEquippedSlot`
  (returns (EquippedSlot :type "/Game/Core/Blueprints/Gameplay/Components/EquipmentComponent/Enums/E_EquipmentSlots Enum"))
  (return (`self.EquippedSlot`)))

(fn `GetIsAiming`
  (returns (IsAiming :type Boolean))
  (return (`self.IsAiming`)))

(fn `GetLoadedAmmo`
  (returns (LoadedAmmo :type "Array of Integer"))
  (return (`self.LoadedAmmo`)))

(fn `GetTargetPitch`
  (returns (TargetPitch :type "Float (double-precision)"))
  (bind _ownercharacter (`self.OwnerCharacter`))
  (bind (_returnvalue_roll _returnvalue_pitch) (`KismetMathLibrary.BreakRotator` (`Pawn.GetControlRotation` _ownercharacter)))
  (return (select `bool` (`Pawn.IsLocallyControlled` _ownercharacter) :`false` (`self.TargetPitch`) :`true` _returnvalue_pitch :!type "Float (double-precision)")))

(fn `HandleADS`
  (params (DeltaSeconds :type "Float (double-precision)"))
  (if (`Pawn.IsLocallyControlled` (`self.OwnerCharacter`))
    (`self.SwitchOnRangedWeapon`
      (:`IsRanged`
        (set `self.ADSProgress` (`KismetMathLibrary.FClamp` (+ (`self.ADSProgress`) (* (* (`local.DeltaSeconds`) (/ 1.0 (`self.ADSTime`))) (select `bool` (`self.IsAiming`) :`false` -1.0 :`true` 1.0)))))
        (set `SpringArmComponent.SocketOffset` (`KismetMathLibrary.VLerp` (`self.DefaultSocketOffset`) (`.ADSOffset_25_1236F78B4EEF254B22D9FAA06815475A` (break `/Game/Core/Blueprints/Gameplay/Components/WeaponSystemComponent/Structures/ST_RangedWeaponItemData` (defaults `Object` (`self.CurrentRangedWeapon`)))) (`self.ADSProgress`)) (`self.SpringArmComponent`))
        (`CameraComponent.SetFieldOfView` (`self.CameraComponent`) (`KismetMathLibrary.Lerp` (`self.DefaultFOV`) (`.ADSFoV_28_F886F78C48C6219C72DEE2BC1B9C8EB4` (break `/Game/Core/Blueprints/Gameplay/Components/WeaponSystemComponent/Structures/ST_RangedWeaponItemData` (defaults `Object` (`self.CurrentRangedWeapon`)))) (`self.ADSProgress`)))))))

(fn `HandlePitch`
  (params (DeltaSeconds :type "Float (double-precision)"))
  (bind _returnvalue_roll (`KismetMathLibrary.BreakRotator` (`KismetMathLibrary.RInterpTo` (`KismetMathLibrary.MakeRotator` (`self.CurrentPitch`)) (`KismetMathLibrary.MakeRotator` (`self.GetTargetPitch`)) (`local.DeltaSeconds`) 5.0)))
  (set `self.CurrentPitch` _returnvalue_roll))

(fn `Init`
  (`|ExecutionSequence`
    (:`then_0`
      (set `self.AbilitySystemComponent` (`Actor.GetComponentByClass` (`self.GetOwner`) "/Game/Core/Blueprints/Gameplay/Components/AbilitySystemComponent/BPC_AbilitySystemComponent.BPC_AbilitySystemComponent_C"))
      (bind _output_get (set `self.EquipmentComponent` (`Actor.GetComponentByClass` (`self.GetOwner`) "/Game/Core/Blueprints/Gameplay/Components/EquipmentComponent/BPC_EquipmentComponent.BPC_EquipmentComponent_C")))
      (add `/Game/Core/Blueprints/Gameplay/Components/EquipmentComponent/BPC_EquipmentComponent.OnUpdatedEquipmentSlots` _output_get (`|CreateDelegate` :!event `OnUpdatedEquipmentSlots`))
      (`self.UpdateCurrentWeapon`))
    (:`then_1`
      (bind _asbp_character_base (cast `/Game/Core/Blueprints/Gameplay/Characters/BP_CharacterBase` (`self.GetOwner`)))
      (set `self.OwnerCharacter` _asbp_character_base)
      (`self.UpdateStrafe`)
      (set `self.InventoryComponent` (`Actor.GetComponentByClass` (`self.GetOwner`) "/Game/Core/Blueprints/Gameplay/Components/InventoryComponent/BPC_InventoryComponent.BPC_InventoryComponent_C")))
    (:`then_2`
      (`/Engine/EditorBlueprintResources/ActorComponentMacros.Switch Has Authority`
        (:`Authority`
          (bind _returnvalue (`KismetSystemLibrary.K2_SetTimerDelegate` (`|CreateDelegate` :!event `BroadcastPitch`) (`self.ReplicatePitchRate`)))
          (set `self.PitchTimer` _returnvalue))))
    (:`then_3`
      (bind _output_get_2 (set `self.SpringArmComponent` (`Actor.GetComponentByClass` (`self.GetOwner`) "/Script/Engine.SpringArmComponent")))
      (`/Engine/EditorBlueprintResources/StandardMacros.IsValid` _output_get_2
        (:`Is Valid`
          (set `self.DefaultSocketOffset` (`SpringArmComponent.SocketOffset` _output_get_2))
          (bind _output_get_3 (set `self.CameraComponent` (`Actor.GetComponentByClass` (`self.GetOwner`) "/Script/Engine.CameraComponent")))
          (set `self.DefaultFOV` (`CameraComponent.FieldOfView` _output_get_3)))))))

(fn `InputADS`
  (params (IsADS :type Boolean))
  (if IsADS
    (`self.SwitchOnRangedWeapon`
      (:`IsRanged`
        (bind _output_get (set `self.IsAiming` true))
        (`self.ServerSetIsADS` _output_get)
        (`self.OnUpdatedIsAiming` true)))
    (elif (`self.IsAiming`)
      (bind _output_get_2 (set `self.IsAiming` false))
      (`self.ServerSetIsADS` _output_get_2)
      (`self.OnUpdatedIsAiming` false))))

(fn `LocalInit`)

(fn `OnRep_EquippedSlot`
  (`self.OnUpdatedEquippedSlot` (`self.EquippedSlot`))
  (`self.UpdateCurrentWeapon`))

(fn `OnRep_IsAiming`
  (`self.UpdateStrafe`))

(fn `OnRep_LoadedAmmo`
  (`self.OnUpdatedLoadedAmmo` (`self.LoadedAmmo`)))

(fn `OnUpdatedEquipmentSlots`
  (params (EquipmentSlots :type "Array of /Game/Core/Blueprints/Gameplay/Components/EquipmentComponent/Structures/ST_EquipmentSlot Structure (by ref)"))
  (`self.UpdateCurrentWeapon`))

(fn `Reload`
  (locals (AmountToReload :type Integer :default 0))
  (bind _returnvalue (select `bool` (`|EnumEquality` (`self.EquippedSlot`) "NewEnumerator0") :`false` 1))
  (if (`self.CanReload`)
    (set `local.AmountToReload` (`KismetMathLibrary.Min` (- (`.MagazineAmmo_5_12AEF0674BE50D36A1C584A0BE9AA58A` (break `/Game/Core/Blueprints/Gameplay/Components/WeaponSystemComponent/Structures/ST_RangedWeaponItemData` (defaults `Object` (`self.CurrentRangedWeapon`)))) (`self.GetCurrentAmmo`)) (`/Game/Core/Blueprints/Gameplay/Components/InventoryComponent/BPC_InventoryComponent.GetAmountForItem` (`self.InventoryComponent`) (`.AmmoItem_2_6709851D4FC20DF02EC096B47D4C1DF0` (break `/Game/Core/Blueprints/Gameplay/Components/WeaponSystemComponent/Structures/ST_RangedWeaponItemData` (defaults `Object` (`self.CurrentRangedWeapon`)))))))
    (`/Game/Core/Blueprints/Gameplay/Components/InventoryComponent/BPC_InventoryComponent.RemoveItem` (`self.InventoryComponent`) (`.AmmoItem_2_6709851D4FC20DF02EC096B47D4C1DF0` (break `/Game/Core/Blueprints/Gameplay/Components/WeaponSystemComponent/Structures/ST_RangedWeaponItemData` (defaults `Object` (`self.CurrentRangedWeapon`)))) (`local.AmountToReload`))
    (`KismetArrayLibrary.Array_Set` (`self.LoadedAmmo`) _returnvalue (+ (`|GetArrayItem` (`self.LoadedAmmo`) _returnvalue) (`local.AmountToReload`)))
    (set `self.LoadedAmmo` (`self.LoadedAmmo`))))

(fn `RemoveAmmo`
  (bind _returnvalue (select `bool` (`|EnumEquality` (`self.EquippedSlot`) "NewEnumerator0") :`false` 1))
  (`KismetArrayLibrary.Array_Set` (`self.LoadedAmmo`) _returnvalue (`KismetMathLibrary.Max` (- (`|GetArrayItem` (`self.LoadedAmmo`) _returnvalue) 1)))
  (set `self.LoadedAmmo` (`self.LoadedAmmo`)))

(fn `SetEquippedSlot`
  (params (EquippedSlot :type "/Game/Core/Blueprints/Gameplay/Components/EquipmentComponent/Enums/E_EquipmentSlots Enum" :default "NewEnumerator0"))
  (bind _output_get (set `self.EquippedSlot` EquippedSlot))
  (`self.ServerSetEquippedSlot` _output_get))

(fn `SwapEquippedSlot`
  (`self.SetEquippedSlot` (select `bool` (`|EnumEquality` (`self.EquippedSlot`) "NewEnumerator0") :`false` "NewEnumerator0" :`true` "NewEnumerator1" :!type "/Game/Core/Blueprints/Gameplay/Components/EquipmentComponent/Enums/E_EquipmentSlots Enum")))

(fn `UpdateCurrentWeapon`
  (bind _weaponabilityclass (break `/Game/Core/Blueprints/Gameplay/Components/WeaponSystemComponent/Structures/ST_WeaponItemData` (defaults `Object` (`self.LastWeapon`))))
  (bind _output (`|GetArrayItem` (`self.LoadedAmmo`) (select `/Game/Core/Blueprints/Gameplay/Components/EquipmentComponent/Enums/E_EquipmentSlots` (`self.LastEquippedSlot`) :`NewEnumerator1` 1)))
  (if (!= (`.EquipmentItem_6_6AB0AAAF45B76011F96BD2AAF6AEDC54` (break `/Game/Core/Blueprints/Gameplay/Components/EquipmentComponent/Structures/ST_EquipmentSlot` (`/Game/Core/Blueprints/Gameplay/Components/EquipmentComponent/BPC_EquipmentComponent.GetEquipmentSlot` (`self.EquipmentComponent`) (`self.EquippedSlot`)))) (`self.LastWeapon`))
    (`|ExecutionSequence`
      (:`then_0`
        (`/Engine/EditorBlueprintResources/ActorComponentMacros.Switch Has Authority`
          (:`Authority`
            (if (`KismetSystemLibrary.IsValidClass` (`self.LastWeapon`))
              (`/Game/Core/Blueprints/Gameplay/Components/AbilitySystemComponent/BPC_AbilitySystemComponent.UnequipAbility` (`self.AbilitySystemComponent`) (struct :`TagName` "AbilitySlot.Weapon"))
              (bind _asbp_ranged_weapon_item_base (castclass `/Game/Core/Blueprints/Gameplay/Components/WeaponSystemComponent/BP_RangedWeaponItemBase` (`self.LastWeapon`)))
              (if (> _output 0)
                (`/Game/Core/Blueprints/Gameplay/Components/InventoryComponent/BPC_InventoryComponent.AddItem` (`self.InventoryComponent`) (`.AmmoItem_2_6709851D4FC20DF02EC096B47D4C1DF0` (break `/Game/Core/Blueprints/Gameplay/Components/WeaponSystemComponent/Structures/ST_RangedWeaponItemData` (defaults `Object` _asbp_ranged_weapon_item_base))) _output)
                (`KismetArrayLibrary.Array_Set` (`self.LoadedAmmo`) (select `/Game/Core/Blueprints/Gameplay/Components/EquipmentComponent/Enums/E_EquipmentSlots` (`self.LastEquippedSlot`) :`NewEnumerator1` 1))
                (set `self.LoadedAmmo` (`self.LoadedAmmo`)))))))
      (:`then_1`
        (bind _asbp_weapon_item_base (castclass `/Game/Core/Blueprints/Gameplay/Components/WeaponSystemComponent/BP_WeaponItemBase` (`.EquipmentItem_6_6AB0AAAF45B76011F96BD2AAF6AEDC54` (break `/Game/Core/Blueprints/Gameplay/Components/EquipmentComponent/Structures/ST_EquipmentSlot` (`/Game/Core/Blueprints/Gameplay/Components/EquipmentComponent/BPC_EquipmentComponent.GetEquipmentSlot` (`self.EquipmentComponent`) (`self.EquippedSlot`)))))
          (:`then`
            (set `self.LastWeapon` _asbp_weapon_item_base)
            (set `self.LastEquippedSlot` (`self.EquippedSlot`))
            (`|ExecutionSequence`
              (:`then_0`
                (`/Engine/EditorBlueprintResources/ActorComponentMacros.Switch Has Authority`
                  (:`Authority`
                    (if (`KismetSystemLibrary.IsValidClass` _weaponabilityclass)
                      (`/Game/Core/Blueprints/Gameplay/Components/AbilitySystemComponent/BPC_AbilitySystemComponent.EquipAbility` (`self.AbilitySystemComponent`) (make `/Game/Core/Blueprints/Gameplay/Components/AbilitySystemComponent/Structures/ST_AbilityEquipData` (struct :`TagName` "AbilitySlot.Weapon") _weaponabilityclass))))))
              (:`then_1`
                (bind _asbp_ranged_weapon_item_base_2 (castclass `/Game/Core/Blueprints/Gameplay/Components/WeaponSystemComponent/BP_RangedWeaponItemBase` (`self.LastWeapon`))
                  (:`then`
                    (set `self.CurrentRangedWeapon` _asbp_ranged_weapon_item_base_2))
                  (:`CastFailed`
                    (set `self.CurrentRangedWeapon` null))))))
          (:`CastFailed`
            (set `self.LastWeapon` null)
            (set `self.CurrentRangedWeapon` null)))))))

(fn `UpdateStrafe`
  (set `Pawn.bUseControllerRotationYaw` (`self.IsAiming`) (`self.OwnerCharacter`))
  (set `CharacterMovementComponent.bOrientRotationToMovement` (not (`self.IsAiming`)) (`Character.CharacterMovement` (`self.OwnerCharacter`))))