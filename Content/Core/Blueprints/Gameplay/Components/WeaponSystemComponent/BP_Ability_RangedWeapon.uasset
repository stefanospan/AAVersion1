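; Ranged weapon ability that fires the character's current weapon as a single shot or timer-driven automatic fire while left mouse is held.
; The local client traces from the camera to aim from the muzzle socket, predicts ammo use and plays sound immediately.
; The server rechecks ammo, spawns the damage-carrying projectile, multicasts sound to others and ends the ability on request.
; Weapon settings come from class defaults, ammo from the weapon system component.
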(event `self.OnAbilityActivated`
  (bind ((`FireRate_16_0EB20F33478E0131901A5CB54F7B03B4` _firerate) (`FireType_19_4015A62E41D72FED9D569C9F9F1A5077` _firetype)) (break `/Game/Core/Blueprints/Gameplay/Components/WeaponSystemComponent/Structures/ST_RangedWeaponItemData` (defaults `Object` (`self.GetCurrentRangedWeapon`))))
  (`self.CommitAbility`)
  (if (`self.IsLocal`)
    (switch `/Game/Core/Blueprints/Gameplay/Components/WeaponSystemComponent/Enums/E_FireTypes` _firetype
      (:`NewEnumerator0`
        (`self.Fire`)
        (`self.ServerEnd`))
      (:`NewEnumerator1`
        (`self.Fire`)
        (bind _asbp_player_character_base (cast `/Game/Core/Blueprints/Gameplay/Characters/PlayerCharacters/BP_PlayerCharacterBase` (`self.GetOwnerCharacter`)))
        (if (`/Game/Core/Blueprints/Gameplay/Characters/PlayerCharacters/BP_PlayerCharacterBase.GetIsLeftMousePressed` _asbp_player_character_base)
          (add `/Game/Core/Blueprints/Gameplay/Characters/PlayerCharacters/BP_PlayerCharacterBase.OnUpdatedIsLeftMousePressed` _asbp_player_character_base (`|CreateDelegate` :!event `OnUpdatedIsLeftMousePressed`))
          (bind _returnvalue (`KismetSystemLibrary.K2_SetTimerDelegate` (`|CreateDelegate` :!event `Fire`) _firerate true))
          (set `self.FireTimer` _returnvalue)
          (else
            (`self.ServerEnd`)))))))

(event `OnUpdatedIsLeftMousePressed`
  (params (IsLeftMousePressed :type Boolean))
  (if (not IsLeftMousePressed)
    (bind _asbp_player_character_base (cast `/Game/Core/Blueprints/Gameplay/Characters/PlayerCharacters/BP_PlayerCharacterBase` (`self.GetOwnerCharacter`)))
    (remove `/Game/Core/Blueprints/Gameplay/Characters/PlayerCharacters/BP_PlayerCharacterBase.OnUpdatedIsLeftMousePressed` _asbp_player_character_base (`|CreateDelegate` :!event `OnUpdatedIsLeftMousePressed`))
    (`KismetSystemLibrary.K2_ClearAndInvalidateTimerHandle` (`self.FireTimer`))
    (`self.ServerEnd`)))

(event `Fire`
  (if (`self.HsaAmmo`)
    (`/Engine/EditorBlueprintResources/ActorMacros.Switch Has Authority`
      (:`Authority`
        _)
      (:`Remote`
        (`self.RemoveAmmo`)))
    (bind (_location _direction) (`self.GetFireVectors`))
    (`self.ServerFire` _location _direction)
    (`self.PlayFireSound`)
    (elif (`KismetSystemLibrary.K2_IsValidTimerHandle` (`self.FireTimer`))
      (`KismetSystemLibrary.K2_ClearAndInvalidateTimerHandle` (`self.FireTimer`))
      (bind _asbp_player_character_base (cast `/Game/Core/Blueprints/Gameplay/Characters/PlayerCharacters/BP_PlayerCharacterBase` (`self.GetOwnerCharacter`)))
      (remove `/Game/Core/Blueprints/Gameplay/Characters/PlayerCharacters/BP_PlayerCharacterBase.OnUpdatedIsAbility1Pressed` _asbp_player_character_base (`|CreateDelegate` :!event `OnUpdatedIsLeftMousePressed`))
      (`self.ServerEnd`))))

(event `ServerFire`
  (params (Location :type "Vector Structure") (Direction :type "Vector Structure"))
  (bind ((`ProjectileClass_13_996BDA2E4644CEEB5834B2A75B7EFC74` _projectileclass) (`Damage_22_38D8D57A43F189E4349EA8B90801D66A` _damage)) (break `/Game/Core/Blueprints/Gameplay/Components/WeaponSystemComponent/Structures/ST_RangedWeaponItemData` (defaults `Object` (`self.GetCurrentRangedWeapon`))))
  (if (`self.HsaAmmo`)
    (`self.RemoveAmmo`)
    (`|SpawnActorFromClass` _projectileclass (`KismetMathLibrary.MakeTransform` Location (`KismetMathLibrary.Conv_VectorToRotator` Direction)) "AlwaysSpawn" "MultiplyWithRoot" (`self.GetOwnerCharacter`) _damage null)
    (`self.MulticastFire`)))

(event `ServerEnd`
  (`self.EndAbility`))

(event `MulticastFire`
  (if (not (`self.IsLocal`))
    (`self.PlayFireSound`)))

(event `PlayFireSound`
  (`GameplayStatics.SpawnSoundAtLocation` (`.FireSound_33_0C095A9348FA4FEC7705EABC1A07E147` (break `/Game/Core/Blueprints/Gameplay/Components/WeaponSystemComponent/Structures/ST_RangedWeaponItemData` (defaults `Object` (`self.GetCurrentRangedWeapon`)))) (`self.K2_GetActorLocation` (`self.GetOwnerCharacter`)) (struct) 1.0 1.0 0.0 "/Game/UltraDynamicSky/Sound/Attenuation/UDS_Interact_Sound_Attenuation.UDS_Interact_Sound_Attenuation" null))

(fn `GetCurrentRangedWeapon`
  (returns (CurrentRangedWeapon :type "/Game/Core/Blueprints/Gameplay/Components/WeaponSystemComponent/BP_RangedWeaponItemBase Class Reference"))
  (return (`/Game/Core/Blueprints/Gameplay/Components/WeaponSystemComponent/BPC_WeaponSystemComponent.GetCurrentRangedWeapon` (`/Game/Core/Blueprints/Gameplay/Characters/BP_CharacterBase.BPC_WeaponSystemComponent` (`self.GetOwnerCharacter`)))))

(fn `GetFireVectors`
  (returns (Location :type "Vector Structure") (Direction :type "Vector Structure"))
  (locals (HitLocation :type "Vector Structure" :default (0.0 0.0 0.0)))
  (bind _ownercharacter (`self.GetOwnerCharacter`))
  (bind _returnvalue (`GameplayStatics.GetPlayerCameraManager` 0))
  (bind _returnvalue_2 (`self.K2_GetActorLocation` _returnvalue))
  (bind _returnvalue_3 (`SceneComponent.GetSocketLocation` (`/Game/Core/Blueprints/Gameplay/Components/EquipmentComponent/BP_EquipmentItemMesh.EquipmentMesh` (`BlueprintMapLibrary.Map_Find` (`/Game/Core/Blueprints/Gameplay/Components/EquipmentComponent/BPC_EquipmentComponent.GetEquipmentMeshActors` (`/Game/Core/Blueprints/Gameplay/Characters/BP_CharacterBase.BPC_EquipmentComponent` _ownercharacter)) (`/Game/Core/Blueprints/Gameplay/Components/WeaponSystemComponent/BPC_WeaponSystemComponent.GetEquippedSlot` (`/Game/Core/Blueprints/Gameplay/Characters/BP_CharacterBase.BPC_WeaponSystemComponent` _ownercharacter)))) "Projectile"))
  (bind _outhit (`KismetSystemLibrary.LineTraceSingle` _returnvalue_2 (+ _returnvalue_2 (* (`self.GetActorForwardVector` _returnvalue) 25000.0)) "TraceTypeQuery1"))
  (bind (_bblockinghit _binitialoverlap _time _distance _location _impactpoint _normal _impactnormal _physmat _hitactor _hitcomponent _hitbonename _bonename _hititem _elementindex _faceindex _tracestart _traceend) (`GameplayStatics.BreakHitResult` _outhit))
  (if _bblockinghit
    (set `local.HitLocation` _location)
    (else
      (set `local.HitLocation` _traceend)))
  (return _returnvalue_3 (`KismetMathLibrary.Conv_RotatorToVector` (`KismetMathLibrary.FindLookAtRotation` _returnvalue_3 (`local.HitLocation`)))))

(fn `HsaAmmo`
  (returns (ReturnValue :type Boolean))
  (return (> (`/Game/Core/Blueprints/Gameplay/Components/WeaponSystemComponent/BPC_WeaponSystemComponent.GetCurrentAmmo` (`/Game/Core/Blueprints/Gameplay/Characters/BP_CharacterBase.BPC_WeaponSystemComponent` (`self.GetOwnerCharacter`))) 0)))

(fn `RemoveAmmo`
  (`/Game/Core/Blueprints/Gameplay/Components/WeaponSystemComponent/BPC_WeaponSystemComponent.RemoveAmmo` (`/Game/Core/Blueprints/Gameplay/Characters/BP_CharacterBase.BPC_WeaponSystemComponent` (`self.GetOwnerCharacter`))))

(fn `UserConstructionScript`
  (`parent.UserConstructionScript`))