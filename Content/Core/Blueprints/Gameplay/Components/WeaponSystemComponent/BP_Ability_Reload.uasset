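; Reload ability that lets a character reload the current ranged weapon through its BPC_WeaponSystemComponent.
; Activation is gated by the component's CanReload check.
; On authority, it commits and plays the reload montage read from the current weapon's class defaults.
; When the montage ends, authority calls Reload on the component and ends the ability, so the reload applies only after the animation.
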(event `self.OnAbilityActivated`
  (`/Engine/EditorBlueprintResources/ActorMacros.Switch Has Authority`
    (:`Authority`
      (`self.CommitAbility`)
      (`self.PlayAnimMontage` (`.ReloadAnimMontage_10_991675364C6C47403DD0D48C2EDAA035` (break `/Game/Core/Blueprints/Gameplay/Components/WeaponSystemComponent/Structures/ST_RangedWeaponItemData` (defaults `Object` (`/Game/Core/Blueprints/Gameplay/Components/WeaponSystemComponent/BPC_WeaponSystemComponent.GetCurrentRangedWeapon` (`self.GetComponentByClass` (`self.GetOwnerCharacter`) "/Game/Core/Blueprints/Gameplay/Components/WeaponSystemComponent/BPC_WeaponSystemComponent.BPC_WeaponSystemComponent_C")))))))))

(event `self.OnAnimMontageEnded`
  (`/Engine/EditorBlueprintResources/ActorMacros.Switch Has Authority`
    (:`Authority`
      (`/Game/Core/Blueprints/Gameplay/Components/WeaponSystemComponent/BPC_WeaponSystemComponent.Reload` (`self.GetComponentByClass` (`self.GetOwnerCharacter`) "/Game/Core/Blueprints/Gameplay/Components/WeaponSystemComponent/BPC_WeaponSystemComponent.BPC_WeaponSystemComponent_C"))
      (`self.EndAbility`))))

(fn `CanActivate`
  (returns (Success :type Boolean))
  (return (`/Game/Core/Blueprints/Gameplay/Components/WeaponSystemComponent/BPC_WeaponSystemComponent.CanReload` (`self.GetComponentByClass` (`self.GetOwnerCharacter`) "/Game/Core/Blueprints/Gameplay/Components/WeaponSystemComponent/BPC_WeaponSystemComponent.BPC_WeaponSystemComponent_C"))))

(fn `UserConstructionScript`
  (`parent.UserConstructionScript`))