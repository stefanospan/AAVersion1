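; Axe melee attack ability that, on the server, commits, plays a downward swing montage and ends when it finishes.
; Montage notify windows toggle actor tick, which sphere-traces just in front of the owning character.
; Hit actors on another team, or without the teams interface, take damage scaled by the DamageMultiplier attribute.
; An AddUnique list, cleared on each toggle, limits damage to once per actor per swing.
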(event `self.OnAbilityActivated`
  (`/Engine/EditorBlueprintResources/ActorMacros.Switch Has Authority`
    (:`Authority`
      (`self.CommitAbility`)
      (`self.PlayAnimMontage` "/Game/Core/Animations/Axe/StandingMeleeAttackDownward_UE_Montage.StandingMeleeAttackDownward_UE_Montage"))))

(event `self.OnAnimMontageEnded`
  (`/Engine/EditorBlueprintResources/ActorMacros.Switch Has Authority`
    (:`Authority`
      (`self.EndAbility`))))

(event `self.OnNotifyBegin`
  (params (NotifyName :type Name))
  (`/Engine/EditorBlueprintResources/ActorMacros.Switch Has Authority`
    (:`Authority`
      (switch `name` NotifyName
        (:`Trace`
          (`self.ToggleTrace` true))))))

(event `self.OnNotifyEnd`
  (params (NotifyName :type Name))
  (`/Engine/EditorBlueprintResources/ActorMacros.Switch Has Authority`
    (:`Authority`
      (switch `name` NotifyName
        (:`Trace`
          (`self.ToggleTrace` false))))))

(event `ToggleTrace`
  (params (IsTrace :type Boolean))
  (set `self.IsTrace` IsTrace)
  (`KismetArrayLibrary.Array_Clear` (`self.AttackedActors`))
  (`self.SetActorTickEnabled` (`self.IsTrace`)))

(event `self.ReceiveTick`
  (params (DeltaSeconds :type "Float (single-precision)"))
  (bind _ownercharacter (`self.GetOwnerCharacter`))
  (bind _returnvalue (- (`self.K2_GetActorLocation` _ownercharacter) (0.0 0.0 25.0)))
  (`/Engine/EditorBlueprintResources/ActorMacros.Switch Has Authority`
    (:`Authority`
      (bind _team (message `/Game/Core/Blueprints/Gameplay/Components/TeamComponent/BPI_Teams.GetTeam` (`self.GetOwnerCharacter`)))
      (bind _outhits (`KismetSystemLibrary.SphereTraceMulti` _returnvalue (+ _returnvalue (* (`self.GetActorForwardVector` _ownercharacter) 50.0)) 50.0 "TraceTypeQuery1" false (`|MakeArray` (`self.GetOwnerCharacter`) :!type "Actor Object Reference")))
      (for _array_element _outhits
        (bind (_bblockinghit _binitialoverlap _time _distance _location _impactpoint _normal _impactnormal _physmat _hitactor) (`GameplayStatics.BreakHitResult` _array_element))
        (bind _team_2 (message `/Game/Core/Blueprints/Gameplay/Components/TeamComponent/BPI_Teams.GetTeam` _hitactor))
        (if (or (!= _team_2 _team) (not (`KismetSystemLibrary.DoesImplementInterface` _hitactor "/Game/Core/Blueprints/Gameplay/Components/TeamComponent/BPI_Teams.BPI_Teams_C")))
          (bind _returnvalue_2 (`KismetArrayLibrary.Array_AddUnique` (`self.AttackedActors`) _hitactor))
          (if (>= _returnvalue_2 0)
            (`GameplayStatics.ApplyDamage` _hitactor (* (`self.Damage`) (`.Value_5_5382FAD64776275FF614BEB1A224EFA3` (break `/Game/Core/Blueprints/Gameplay/Components/AttributeComponent/Structures/ST_AttributeData` (`self.GetAttribute` (struct :`TagName` "Attribute.DamageMultiplier"))))) null (`self.GetOwnerCharacter`))))))))

(fn `UserConstructionScript`
  (`parent.UserConstructionScript`))