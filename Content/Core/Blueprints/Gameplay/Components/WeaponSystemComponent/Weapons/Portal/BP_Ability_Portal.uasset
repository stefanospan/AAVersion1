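; Weapon-system ability that spawns a portal in front of the owning character.
; On activation the server commits it, removes blue ore stone from the inventory and plays a sword-attack montage.
; The notify event makes the server spawn BP_Portal at a ground-traced point ahead, unequip the current slot and end the ability.
; CanActivate always returns true, as the ore-amount check is left unconnected.
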(event `self.OnAbilityActivated`
  (`GameplayStatics.PlaySound2D` "/Game/UltraDynamicSky/Sound/Dust/Dust_4.Dust_4" 1.0 1.0 0.0 null null)
  (`/Engine/EditorBlueprintResources/ActorMacros.Switch Has Authority`
    (:`Authority`
      (`self.CommitAbility`)
      (`/Game/Core/Blueprints/Gameplay/Components/InventoryComponent/BPC_InventoryComponent.RemoveItem` (`self.GetComponentByClass` (`self.GetOwnerCharacter`) "/Game/Core/Blueprints/Gameplay/Components/InventoryComponent/BPC_InventoryComponent.BPC_InventoryComponent_C") "/Game/Core/Blueprints/Gameplay/Resources/OreStone/BP_Item_OreStone_Blue.BP_Item_OreStone_Blue_C" 200)
      (`self.PlayAnimMontage` "/Game/Placeholder-Assets/3D/Wood_Monster/Animations/Warrior_Sword_Attack_04_Anim_Montage.Warrior_Sword_Attack_04_Anim_Montage"))))

(event `self.OnNotifyBegin`
  (params (NotifyName :type Name))
  (bind _ownercharacter (`self.GetOwnerCharacter`))
  (`/Engine/EditorBlueprintResources/ActorMacros.Switch Has Authority`
    (:`Authority`
      (bind _transform (`self.GetPortalSpawnTransform`))
      (`|SpawnActorFromClass` "/Game/Core/Blueprints/Gameplay/Components/WeaponSystemComponent/Weapons/Portal/BP_Portal.BP_Portal_C" _transform "AlwaysSpawn" "MultiplyWithRoot" null null)
      (`/Game/Core/Blueprints/Gameplay/Components/EquipmentComponent/BPC_EquipmentComponent.UnequipSlot` (`/Game/Core/Blueprints/Gameplay/Characters/BP_CharacterBase.BPC_EquipmentComponent` _ownercharacter) (`/Game/Core/Blueprints/Gameplay/Components/WeaponSystemComponent/BPC_WeaponSystemComponent.GetEquippedSlot` (`/Game/Core/Blueprints/Gameplay/Characters/BP_CharacterBase.BPC_WeaponSystemComponent` _ownercharacter)))
      (`self.EndAbility`))))

(fn `CanActivate`
  (returns (Success :type Boolean))
  (return true))

(fn `GetPortalSpawnTransform`
  (returns (Transform :type "Transform Structure"))
  (bind _ownercharacter (`self.GetOwnerCharacter`))
  (bind _ownercharacter_2 (`self.GetOwnerCharacter`))
  (bind _returnvalue (+ (`self.K2_GetActorLocation` _ownercharacter_2) (* (`self.GetActorForwardVector` _ownercharacter_2) 150.0)))
  (bind _outhit (`KismetSystemLibrary.LineTraceSingle` (+ _returnvalue (0.0 0.0 500.0)) (- _returnvalue (0.0 0.0 500.0)) "TraceTypeQuery1"))
  (bind (_bblockinghit _binitialoverlap _time _distance _location) (`GameplayStatics.BreakHitResult` _outhit))
  (return (`KismetMathLibrary.MakeTransform` (select `bool` _bblockinghit :`false` (+ (`self.K2_GetActorLocation` _ownercharacter) (* (`self.GetActorForwardVector` _ownercharacter) 150.0)) :`true` _location) (`self.K2_GetActorRotation` (`self.GetOwnerCharacter`)))))

(fn `UserConstructionScript`
  (`parent.UserConstructionScript`))