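; BPC_TimerComponent is a reusable countdown timer component.
; StartTimer sets the remaining time and starts a looping one-second timer, with HandleTimer decrementing the value and clamping it at zero.
; The RepNotify on RemainingTime broadcasts each update to listeners.
; On reaching zero, it clears the timer handle and broadcasts completion.
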(fn `GetRemainingTime`
  (returns (RemainingTime :type "Float (double-precision)"))
  (return (`self.RemainingTime`)))

(fn `HandleTimer`
  (bind _output_get (set `self.RemainingTime` (`KismetMathLibrary.FMax` (- (`self.RemainingTime`) 1.0))))
  (if (== _output_get 0.0)
    (`self.OnTimerEnded`)))

(fn `OnRep_RemainingTime`
  (`self.OnUpdatedRemainingTime` (`self.RemainingTime`)))

(fn `OnTimerEnded`
  (`KismetSystemLibrary.K2_ClearAndInvalidateTimerHandle` (`self.Timer`))
  (`self.OnTimerCompleted`))

(fn `StartTimer`
  (params (Time :type "Float (double-precision)"))
  (set `self.RemainingTime` Time)
  (bind _returnvalue (`KismetSystemLibrary.K2_SetTimerDelegate` (`|CreateDelegate` :!event `Handletimer`) 1.0 true))
  (set `self.Timer` _returnvalue))