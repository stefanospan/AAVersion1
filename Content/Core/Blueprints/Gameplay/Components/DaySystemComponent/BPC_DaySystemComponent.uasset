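; Actor component that tracks the current in-game day from Ultra Dynamic Sky and announces day changes across the network.
; On the authority, a looping one-second timer polls the sky's elapsed-day count and updates CurrentDay when it increases.
; A multicast event then fires the next-day dispatcher, while CurrentDay's RepNotify broadcasts the updated value through a second dispatcher.
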(event `self.ReceiveBeginPlay`
  (`self.Init`))

(event `MulticastOnNextDay`
  (`self.OnNextDay`))

(fn `GetCurrentDay`
  (returns (CurrentDay :type Integer))
  (return (`self.CurrentDay`)))

(fn `HandleDay`
  (if (> (`/Game/UltraDynamicSky/Blueprints/Ultra_Dynamic_Sky.Total Days Elapsed` (`self.UDS`)) (`self.CurrentDay`))
    (set `self.CurrentDay` (`/Game/UltraDynamicSky/Blueprints/Ultra_Dynamic_Sky.Total Days Elapsed` (`self.UDS`)))
    (`self.MulticastOnNextDay`)))

(fn `Init`
  (`/Engine/EditorBlueprintResources/ActorComponentMacros.Switch Has Authority`
    (:`Authority`
      (bind _uds (`/Game/UltraDynamicSky/Blueprints/Functions/UltraDynamicSky_Functions.Get Ultra Dynamic Sky`))
      (set `self.UDS` _uds)
      (bind _returnvalue (`KismetSystemLibrary.K2_SetTimerDelegate` (`|CreateDelegate` :!event `HandleDay`) 1.0 true))
      (set `self.Timer` _returnvalue))))

(fn `OnRep_CurrentDay`
  (`self.OnUpdatedCurrentDay` (`self.CurrentDay`)))