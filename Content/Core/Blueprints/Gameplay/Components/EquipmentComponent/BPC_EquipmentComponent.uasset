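; Character component that manages equipment slots, filled with items taken from inventory.
; The authority builds one slot per enum value, and a RepNotify broadcasts changes and refreshes meshes.
; Equipping validates the item's allowed slots, returns any current item to the owner's inventory, then removes one from the source.
; Mesh refresh respawns attached actors, showing only the weapon system's active slot, and also runs when that slot changes.
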(event `self.ReceiveBeginPlay`
  (`self.Init`))

(fn `EquipFromInventory`
  (params (FromInventoryComponent :type "/Game/Core/Blueprints/Gameplay/Components/InventoryComponent/BPC_InventoryComponent Object Reference") (FromSlotIndex :type Integer) (ToEquipmentSlot :type "/Game/Core/Blueprints/Gameplay/Components/EquipmentComponent/Enums/E_EquipmentSlots Enum" :default "NewEnumerator0"))
  (returns (Success :type Boolean))
  (locals (EquipmentItem :type "/Game/Core/Blueprints/Gameplay/Components/EquipmentComponent/BP_EquipmentItemBase Class Reference"))
  (bind (_item _amount) (break `/Game/Core/Blueprints/Gameplay/Components/InventoryComponent/Structures/ST_InventorySlot` (`/Game/Core/Blueprints/Gameplay/Components/InventoryComponent/BPC_InventoryComponent.GetSlotAtIndex` FromInventoryComponent FromSlotIndex)))
  (bind ((`EquipmentItem_6_6AB0AAAF45B76011F96BD2AAF6AEDC54` _equipmentitem)) (break `/Game/Core/Blueprints/Gameplay/Components/EquipmentComponent/Structures/ST_EquipmentSlot` (`self.GetEquipmentSlot` (`local.ToEquipmentSlot`))))
  (if (and (`KismetSystemLibrary.IsValidClass` _item) (> _amount 0))
    (bind _asbp_equipment_item_base (castclass `/Game/Core/Blueprints/Gameplay/Components/EquipmentComponent/BP_EquipmentItemBase` _item)
      (:`then`
        (if (`KismetArrayLibrary.Array_Contains` (`.EquipmentSlots_7_6935A6884F10E5555D7EA08A8C07B139` (break `/Game/Core/Blueprints/Gameplay/Components/EquipmentComponent/Structures/ST_EquipmentItemData` (defaults `Object` _asbp_equipment_item_base))) (`local.ToEquipmentSlot`))
          (set `local.EquipmentItem` _asbp_equipment_item_base)
          (`|ExecutionSequence`
            (:`then_0`
              (if (`KismetSystemLibrary.IsValidClass` _equipmentitem)
                (bind _remainingamount (`/Game/Core/Blueprints/Gameplay/Components/InventoryComponent/BPC_InventoryComponent.AddItem` (`self.InventoryComponent`) _equipmentitem 1))
                (if (== _remainingamount 1)
                  (return false))))
            (:`then_1`
              (`self.EquipSlot` (`local.ToEquipmentSlot`) (`local.EquipmentItem`))
              (`/Game/Core/Blueprints/Gameplay/Components/InventoryComponent/BPC_InventoryComponent.RemoveAmountAtSlot` (`self.InventoryComponent`) (`local.FromSlotIndex`) 1)
              (return true)))
          (else
            (return false))))
      (:`CastFailed`
        (return false)))
    (else
      (return false))))

(fn `EquipSlot`
  (params (EquipmentSlot :type "/Game/Core/Blueprints/Gameplay/Components/EquipmentComponent/Enums/E_EquipmentSlots Enum" :default "NewEnumerator0") (EquipmentItem :type "/Game/Core/Blueprints/Gameplay/Components/EquipmentComponent/BP_EquipmentItemBase Class Reference"))
  (returns (Success :type Boolean))
  (if (`KismetArrayLibrary.Array_Contains` (`.EquipmentSlots_7_6935A6884F10E5555D7EA08A8C07B139` (break `/Game/Core/Blueprints/Gameplay/Components/EquipmentComponent/Structures/ST_EquipmentItemData` (defaults `Object` EquipmentItem))) (`local.EquipmentSlot`))
    (for (_array_element _array_index) (`self.EquipmentSlots`)
      (if (`|EnumEquality` (`.EquipmentSlot_2_97606E0E4EB21C4D6FF811B809D5AECA` (break `/Game/Core/Blueprints/Gameplay/Components/EquipmentComponent/Structures/ST_EquipmentSlot` _array_element)) (`local.EquipmentSlot`))
        (setmembers `/Game/Core/Blueprints/Gameplay/Components/EquipmentComponent/Structures/ST_EquipmentSlot` :`StructRef` (`|GetArrayItem` (`self.EquipmentSlots`) _array_index) :`EquipmentItem` (`local.EquipmentItem`))
        (set `self.EquipmentSlots` (`self.EquipmentSlots`))
        (`self.OnEquipped` (`local.EquipmentSlot`) (`local.EquipmentItem`))
        (return true)))
    (return false)
    (else
      (return false))))

(fn `GetEquipmentMeshActors`
  (returns (EquipmentMeshActors :type "Map of /Game/Core/Blueprints/Gameplay/Components/EquipmentComponent/Enums/E_EquipmentSlots Enum to /Game/Core/Blueprints/Gameplay/Components/EquipmentComponent/BP_EquipmentItemMesh Object Reference"))
  (return (`self.EquipmentMeshActors`)))

(fn `GetEquipmentSlot`
  (params (Slot :type "/Game/Core/Blueprints/Gameplay/Components/EquipmentComponent/Enums/E_EquipmentSlots Enum" :default "NewEnumerator0"))
  (returns (EquipmentSlot :type "/Game/Core/Blueprints/Gameplay/Components/EquipmentComponent/Structures/ST_EquipmentSlot Structure"))
  (for _array_element (`self.EquipmentSlots`)
    (if (`|EnumEquality` (`.EquipmentSlot_2_97606E0E4EB21C4D6FF811B809D5AECA` (break `/Game/Core/Blueprints/Gameplay/Components/EquipmentComponent/Structures/ST_EquipmentSlot` _array_element)) (`local.Slot`))
      (return _array_element)))
  (return))

(fn `GetEquipmentSlots`
  (returns (EquipmentSlots :type "Array of /Game/Core/Blueprints/Gameplay/Components/EquipmentComponent/Structures/ST_EquipmentSlot Structure"))
  (return (`self.EquipmentSlots`)))

(fn `Init`
  (locals (EquipmentSlotsTemp :type "Array of /Game/Core/Blueprints/Gameplay/Components/EquipmentComponent/Structures/ST_EquipmentSlot Structure"))
  (`|ExecutionSequence`
    (:`then_0`
      (`/Engine/EditorBlueprintResources/ActorComponentMacros.Switch Has Authority`
        (:`Authority`
          (bind _enumvalue (foreach `/Game/Core/Blueprints/Gameplay/Components/EquipmentComponent/Enums/E_EquipmentSlots` false)
            (:`LoopBody`
              (`KismetArrayLibrary.Array_Add` (`local.EquipmentSlotsTemp`) (make `/Game/Core/Blueprints/Gameplay/Components/EquipmentComponent/Structures/ST_EquipmentSlot` _enumvalue null)))
            (:`then`
              (set `self.EquipmentSlots` (`local.EquipmentSlotsTemp`)))))))
    (:`then_1`
      (set `self.InventoryComponent` (`Actor.GetComponentByClass` (`self.GetOwner`) "/Game/Core/Blueprints/Gameplay/Components/InventoryComponent/BPC_InventoryComponent.BPC_InventoryComponent_C")))
    (:`then_2`
      (bind _asbp_character_base (cast `/Game/Core/Blueprints/Gameplay/Characters/BP_CharacterBase` (`self.GetOwner`)))
      (set `self.OwnerCharacter` _asbp_character_base))
    (:`then_3`
      (bind _output_get (set `self.WeaponSystemComponent` (`Actor.GetComponentByClass` (`self.GetOwner`) "/Game/Core/Blueprints/Gameplay/Components/WeaponSystemComponent/BPC_WeaponSystemComponent.BPC_WeaponSystemComponent_C")))
      (add `/Game/Core/Blueprints/Gameplay/Components/WeaponSystemComponent/BPC_WeaponSystemComponent.OnUpdatedEquippedSlot` _output_get (`|CreateDelegate` :!event `OnUpdatedEquippedSlot`)))
    (:`then_4`
      (`self.UpdateEquipmentMeshes`))))

(fn `OnRep_EquipmentSlots`
  (`self.OnUpdatedEquipmentSlots` (`self.EquipmentSlots`))
  (`self.UpdateEquipmentMeshes`))

(fn `OnUpdatedEquippedSlot`
  (params (EquippedSlot :type "/Game/Core/Blueprints/Gameplay/Components/EquipmentComponent/Enums/E_EquipmentSlots Enum" :default "NewEnumerator0"))
  (`self.UpdateEquipmentMeshes`))

(fn `UnequipSlot`
  (params (EquipmentSlot :type "/Game/Core/Blueprints/Gameplay/Components/EquipmentComponent/Enums/E_EquipmentSlots Enum" :default "NewEnumerator0"))
  (for (_array_element _array_index) (`self.EquipmentSlots`)
    (if (`|EnumEquality` (`.EquipmentSlot_2_97606E0E4EB21C4D6FF811B809D5AECA` (break `/Game/Core/Blueprints/Gameplay/Components/EquipmentComponent/Structures/ST_EquipmentSlot` _array_element)) (`local.EquipmentSlot`))
      (setmembers `/Game/Core/Blueprints/Gameplay/Components/EquipmentComponent/Structures/ST_EquipmentSlot` :`StructRef` (`|GetArrayItem` (`self.EquipmentSlots`) _array_index) :`EquipmentItem` null)
      (set `self.EquipmentSlots` (`self.EquipmentSlots`))
      (return)))
  (return))

(fn `UpdateEquipmentMeshes`
  (`self.OwnerCharacter`
    (:`then`
      (`|ExecutionSequence`
        (:`then_0`
          (bind _values (`BlueprintMapLibrary.Map_Values` (`self.EquipmentMeshActors`)))
          (for _array_element _values
            (`Actor.K2_DestroyActor` _array_element))
          (`BlueprintMapLibrary.Map_Clear` (`self.EquipmentMeshActors`)))
        (:`then_1`
          (for _array_element_2 (`self.EquipmentSlots`)
            (bind (_equipmentslot _equipmentitem) (break `/Game/Core/Blueprints/Gameplay/Components/EquipmentComponent/Structures/ST_EquipmentSlot` _array_element_2))
            (if (`|EnumEquality` _equipmentslot (`/Game/Core/Blueprints/Gameplay/Components/WeaponSystemComponent/BPC_WeaponSystemComponent.GetEquippedSlot` (`self.WeaponSystemComponent`)))
              (if (`KismetSystemLibrary.IsValidClass` _equipmentitem)
                (bind (_equipmentitemdata _itemdata) (defaults `Object` _equipmentitem))
                (bind _returnvalue (`|SpawnActorFromClass` "/Game/Core/Blueprints/Gameplay/Components/EquipmentComponent/BP_EquipmentItemMesh.BP_EquipmentItemMesh_C" (`KismetMathLibrary.MakeTransform` (0.0 0.0 0.0)) "AlwaysSpawn" "MultiplyWithRoot" null (`.ItemMesh_14_FE008AFC4E8A84E40564718AEDF885CD` (break `/Game/Core/Blueprints/Gameplay/Components/InventoryComponent/Structures/ST_ItemData` _itemdata)) null))
                (`Actor.K2_AttachToComponent` _returnvalue (`Character.Mesh` (`self.OwnerCharacter`)) (`.AttachSocket_5_41E345654F1BC0C0F011C18BF5955C01` (break `/Game/Core/Blueprints/Gameplay/Components/EquipmentComponent/Structures/ST_EquipmentItemData` _equipmentitemdata)) "SnapToTarget" "SnapToTarget" "KeepWorld" true)
                (`BlueprintMapLibrary.Map_Add` (`self.EquipmentMeshActors`) _equipmentslot _returnvalue)))))))
    (:`else`)))