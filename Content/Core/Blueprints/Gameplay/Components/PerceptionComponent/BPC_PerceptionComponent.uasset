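; Actor component that gives its owner sight-based perception of nearby Characters, updated every tick on the server.
; It sphere-overlaps Pawns within SightDistance, keeps those within SightAngle of the owner's forward vector, then confirms line of sight with a Visibility trace.
; The resulting list of perceived actors is passed to CallOnUpdatedPerception.
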(event `self.ReceiveTick`
  (params (DeltaSeconds :type "Float (single-precision)"))
  (`/Engine/EditorBlueprintResources/ActorComponentMacros.Switch Has Authority`
    (:`Authority`
      (`self.UpdatePerception`))))

(fn `CheckActorTrace`
  (params (Actor :type "Actor Object Reference"))
  (returns (Success :type Boolean))
  (bind _outhit (`KismetSystemLibrary.LineTraceSingle` (`Actor.K2_GetActorLocation` (`self.GetOwner`)) (`Actor.K2_GetActorLocation` (`local.Actor`)) "TraceTypeQuery1"))
  (return (== (`.HitActor` (`GameplayStatics.BreakHitResult` _outhit)) (`local.Actor`))))

(fn `UpdatePerception`
  (locals (PerceivedActorsTemp :type "Array of Actor Object Reference") (ActorTemp :type "Actor Object Reference"))
  (bind _returnvalue (`self.GetOwner`))
  (bind _outactors (`KismetSystemLibrary.SphereOverlapActors` (`Actor.K2_GetActorLocation` (`self.GetOwner`)) (`self.SightDistance`) (`|MakeArray` "ObjectTypeQuery3" :!type "EObjectTypeQuery Enum") "/Script/Engine.Character"))
  (for _array_element _outactors
    (set `local.ActorTemp` _array_element)
    (if (<= (`KismetMathLibrary.DegAcos` (`KismetMathLibrary.Dot_VectorVector` (`KismetMathLibrary.Normal` (- (`Actor.K2_GetActorLocation` _array_element) (`Actor.K2_GetActorLocation` _returnvalue))) (`Actor.GetActorForwardVector` _returnvalue))) (`self.SightAngle`))
      (bind _success (`self.CheckActorTrace` (`local.ActorTemp`)))
      (if _success
        (`KismetArrayLibrary.Array_Add` (`local.PerceivedActorsTemp`) (`local.ActorTemp`)))))
  (`self.OnUpdatedPerception` (`local.PerceivedActorsTemp`)))