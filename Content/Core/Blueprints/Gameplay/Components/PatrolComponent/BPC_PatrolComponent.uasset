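; BPC_PatrolComponent is a component that tracks an actor's progress along a looping patrol route defined by an array of point actors.
; It exposes the current index and the world location of the current patrol point.
; IncreasePatrolIndex advances the index with a modulo on the array length, wrapping back to the first point, with no guard for an empty array.
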(fn `GetCurrentPatrolIndex`
  (returns (CurrentPatrolIndex :type Integer))
  (return (`self.CurrentPatrolIndex`)))

(fn `GetTargetLocation`
  (returns (Location :type "Vector Structure"))
  (return (`Actor.K2_GetActorLocation` (`|GetArrayItem` (`self.PatrolPoints`) (`self.CurrentPatrolIndex`)))))

(fn `IncreasePatrolIndex`
  (set `self.CurrentPatrolIndex` (mod (+ (`self.CurrentPatrolIndex`) 1) (`KismetArrayLibrary.Array_Length` (`self.PatrolPoints`)))))