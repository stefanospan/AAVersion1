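; Pawn component that finds the nearest interactable around its owner and lets the locally controlled player interact with it.
; It turns on ticking only for local control, checked at BeginPlay or when the pawn restarts.
; Each tick, a sphere overlap picks the closest actor returning a valid interactable and broadcasts hover changes.
; InputInteract calls the hovered interactable's client interact event, passing itself.
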(event `self.ReceiveBeginPlay`
  (`self.Init`))

(event `self.ReceiveTick`
  (params (DeltaSeconds :type "Float (single-precision)"))
  (`self.HandleHover`))

(fn `FindClosestInteractable`
  (returns (Found :type Boolean) (Interactable :type "/Game/Core/Blueprints/Gameplay/Components/InteractionSystemComponent/BPC_Interactable Object Reference"))
  (locals (IsFirst :type Boolean :default true) (ClosestInteractable :type "/Game/Core/Blueprints/Gameplay/Components/InteractionSystemComponent/BPC_Interactable Object Reference") (ClosestDistance :type "Float (double-precision)"))
  (bind _closestinteractable (`local.ClosestInteractable`))
  (bind _outactors (`KismetSystemLibrary.SphereOverlapActors` (`Actor.K2_GetActorLocation` (`self.GetOwner`)) (`self.InteractionRadius`) (`|MakeArray` "ObjectTypeQuery1" "ObjectTypeQuery2" "ObjectTypeQuery3" :!type "EObjectTypeQuery Enum") "/Script/Engine.Actor" (`|MakeArray` (`self.GetOwner`))))
  (for _array_element _outactors
    (bind _interactable (message `/Game/Core/Blueprints/Gameplay/Components/InteractionSystemComponent/BPI_Interact.GetInteractable` _array_element))
    (`/Engine/EditorBlueprintResources/StandardMacros.IsValid` _interactable
      (:`Is Valid`
        (bind _returnvalue (`KismetMathLibrary.Vector_Distance` (`Actor.K2_GetActorLocation` _array_element) (`Actor.K2_GetActorLocation` (`self.GetOwner`))))
        (if (or (< _returnvalue (`local.ClosestDistance`)) (`local.IsFirst`))
          (set `local.IsFirst` false)
          (set `local.ClosestInteractable` _interactable)
          (set `local.ClosestDistance` _returnvalue)))))
  (return (`KismetSystemLibrary.IsValid` _closestinteractable) _closestinteractable))

(fn `HandleHover`
  (bind (_found _interactable) (`self.FindClosestInteractable`))
  (if _found
    (bind _hoveredinteractable (`self.HoveredInteractable`)
      (:`then`
        (if (!= _hoveredinteractable _interactable)
          (`self.OnUpdatedHover` false)
          (bind _output_get (set `self.HoveredInteractable` _interactable :!label _label))
          (`self.OnUpdatedHover` true _output_get)))
      (:`else`
        (set `self.IsHover` true)
        (goto _label)))
    (elif (`self.IsHover`)
      (set `self.IsHover` false)
      (set `self.HoveredInteractable` null)
      (`self.OnUpdatedHover` false))))

(fn `Init`
  (bind _aspawn (cast `Pawn` (`self.GetOwner`)))
  (if (`Pawn.IsLocallyControlled` _aspawn)
    (`self.LocalInit`)
    (else
      (add `Pawn.ReceiveRestartedDelegate` _aspawn (`|CreateDelegate` :!event `OnReceiveRestarted`)))))

(fn `InputInteract`
  (bind _hoveredinteractable (`self.HoveredInteractable`)
    (:`then`
      (`/Game/Core/Blueprints/Gameplay/Components/InteractionSystemComponent/BPC_Interactable.ClientOnInteract` _hoveredinteractable self))
    (:`else`)))

(fn `LocalInit`
  (set `self.IsLocal` true)
  (`self.SetComponentTickEnabled` true))

(fn `OnReceiveRestarted`
  (params (Pawn :type "Pawn Object Reference"))
  (if (`Pawn.IsLocallyControlled` Pawn)
    (`self.LocalInit`)))