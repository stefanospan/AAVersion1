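; BP_EffectBase is the base Blueprint for gameplay effects tied to an effect component.
; It exposes getters for its owning effect component, instigator actor and remaining time, plus a setter for the time.
; Remaining time is replicated, with its RepNotify broadcasting OnUpdatedRemainingTime to listeners.
; The applied and removed events are empty hooks, and the base contains no countdown or effect logic.
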(event `OnEffectApplied`)

(event `OnEffectRemoved`)

(fn `GetEffectComponent`
  (returns (EffectComponent :type "/Game/Core/Blueprints/Gameplay/Components/EffectComponent/BPC_EffectComponent Object Reference"))
  (return (`self.EffectComponent`)))

(fn `GetInstigatorActor`
  (returns (InstigatorActor :type "Actor Object Reference"))
  (return (`self.InstigatorActor`)))

(fn `GetRemainingTime`
  (returns (RemainingTime :type "Float (double-precision)"))
  (return (`self.RemainingTime`)))

(fn `OnRep_RemainingTime`
  (`self.OnUpdatedRemainingTime` (`self.RemainingTime`)))

(fn `SetRemainingTime`
  (params (RemainingTime :type "Float (double-precision)"))
  (set `self.RemainingTime` RemainingTime))

(fn `UserConstructionScript`)