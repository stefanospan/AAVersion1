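; Actor component that manages timed gameplay effects on its owner, such as buffs or debuffs.
; ApplyEffect spawns effect actors, respecting stacking rules, then feeds stats and additive attributes to sibling components and attaches optional visuals.
; Shared looping timers drive duration countdowns and periodic stat reapplication, clearing when their lists empty.
; Removal reverts attributes but not stats, and replicated ActiveEffects notifies listeners through OnRep.
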(event `self.ReceiveBeginPlay`
  (`self.Init`))

(event `self.ReceiveEndPlay`
  (params (EndPlayReason :type "EEndPlayReason Enum" :default "Destroyed"))
  (`/Engine/EditorBlueprintResources/ActorComponentMacros.Switch Has Authority`
    (:`Authority`
      (for _array_element (`self.ActiveEffects`)
        (`Actor.K2_DestroyActor` _array_element))
      (`KismetArrayLibrary.Array_Clear` (`self.ActiveEffects`)))))

(fn `ApplyEffect`
  (params (Effect :type "/Game/Core/Blueprints/Gameplay/Components/EffectComponent/BP_EffectBase Class Reference") (InstigatorActor :type "Actor Object Reference"))
  (returns (Success :type Boolean))
  (locals (EffectTemp :type "/Game/Core/Blueprints/Gameplay/Components/EffectComponent/BP_EffectBase Object Reference"))
  (bind ((`EffectVisual_26_2C98AB8F410855E19D6BF7BE89EB1847` _effectvisual)) (break `/Game/Core/Blueprints/Gameplay/Components/EffectComponent/Structures/ST_EffectData` (`/Game/Core/Blueprints/Gameplay/Components/EffectComponent/BP_EffectBase.EffectData` (`local.EffectTemp`))))
  (bind ((`Icon_23_9111025444A9D5A5D59F2BA2957031D7` _icon) (`RepeatRate_13_4749ECE0481191AC71A885A560C73C53` _repeatrate)) (break `/Game/Core/Blueprints/Gameplay/Components/EffectComponent/Structures/ST_EffectData` (`/Game/Core/Blueprints/Gameplay/Components/EffectComponent/BP_EffectBase.EffectData` (`local.EffectTemp`))))
  (if (or (`.CanStack_22_693FFD554A43B5AD5465118BF2FDFCC6` (break `/Game/Core/Blueprints/Gameplay/Components/EffectComponent/Structures/ST_EffectData` (defaults `Object` Effect))) (not (`self.HasEffect` Effect)))
    (bind _returnvalue (`|SpawnActorFromClass` (`local.Effect`) (`KismetMathLibrary.MakeTransform` (0.0 0.0 0.0)) "AlwaysSpawn" "MultiplyWithRoot" (`self.GetOwner`) self (`local.InstigatorActor`) null))
    (bind _output_get (set `local.EffectTemp` _returnvalue))
    (`/Game/Core/Blueprints/Gameplay/Components/EffectComponent/BP_EffectBase.SetRemainingTime` _output_get (`.Duration_15_751B006441C44630FFE50E8372555D15` (break `/Game/Core/Blueprints/Gameplay/Components/EffectComponent/Structures/ST_EffectData` (defaults `Object` (`local.Effect`)))))
    (`KismetArrayLibrary.Array_Add` (`self.ActiveEffects`) (`local.EffectTemp`))
    (set `self.ActiveEffects` (`self.ActiveEffects`))
    (`/Game/Core/Blueprints/Gameplay/Components/EffectComponent/BP_EffectBase.OnEffectApplied` (`local.EffectTemp`))
    (`|ExecutionSequence`
      (:`then_0`
        (`self.ApplyEffectStats` (`local.EffectTemp`)))
      (:`then_1`
        (for _array_element (`.ActiveAdditiveAttributes_20_5BEBDC294E2A46C26B27898069AB169A` (break `/Game/Core/Blueprints/Gameplay/Components/EffectComponent/Structures/ST_EffectData` (`/Game/Core/Blueprints/Gameplay/Components/EffectComponent/BP_EffectBase.EffectData` (`local.EffectTemp`))))
          (`/Game/Core/Blueprints/Gameplay/Components/AttributeComponent/BPC_AttributeComponent.AddAdditiveAttribute` (`self.AttributeComponent`) _array_element)))
      (:`then_2`
        (if (> _repeatrate 0.0)
          (`BlueprintMapLibrary.Map_Add` (`self.RepeatEffects`) (`local.EffectTemp`) _repeatrate)
          (if (not (`KismetSystemLibrary.K2_IsValidTimerHandle` (`self.RepeatEffectsTimer`)))
            (bind _returnvalue_2 (`KismetSystemLibrary.K2_SetTimerDelegate` (`|CreateDelegate` :!event `HandleRepeatEffects`) (`self.RefreshRate`) true))
            (set `self.RepeatEffectsTimer` _returnvalue_2))))
      (:`then_3`
        (if (not (`KismetSystemLibrary.K2_IsValidTimerHandle` (`self.EffectsTimer`)))
          (bind _returnvalue_3 (`KismetSystemLibrary.K2_SetTimerDelegate` (`|CreateDelegate` :!event `HandleEffects`) (`self.RefreshRate`) true))
          (set `self.EffectsTimer` _returnvalue_3)))
      (:`then_4`
        (if (`KismetSystemLibrary.IsValidClass` _effectvisual)
          (bind _returnvalue_4 (`|SpawnActorFromClass` _effectvisual (`KismetMathLibrary.MakeTransform` (`Actor.K2_GetActorLocation` (`self.GetOwner`))) "AlwaysSpawn" "MultiplyWithRoot" null null))
          (`Actor.K2_AttachToActor` _returnvalue_4 (`self.GetOwner`) "None" "SnapToTarget" "SnapToTarget" "KeepWorld" true)
          (`BlueprintMapLibrary.Map_Add` (`self.EffectVisualActors`) (`local.EffectTemp`) _returnvalue_4)))
      (:`then_5`
        (return true)))
    (else
      (return false))))

(fn `ApplyEffectStats`
  (params (Effect :type "/Game/Core/Blueprints/Gameplay/Components/EffectComponent/BP_EffectBase Object Reference"))
  (for _array_element (`.Stats_9_2399B0664AB0E027458A9793E492566C` (break `/Game/Core/Blueprints/Gameplay/Components/EffectComponent/Structures/ST_EffectData` (`/Game/Core/Blueprints/Gameplay/Components/EffectComponent/BP_EffectBase.EffectData` Effect)))
    (bind (_stattag _value) (break `/Game/Core/Blueprints/Gameplay/Components/StatComponent/Structures/ST_StatData` _array_element))
    (`/Game/Core/Blueprints/Gameplay/Components/StatComponent/BPC_StatComponent.AddStat` (`self.StatComponent`) _stattag _value)))

(fn `GetActiveEffects`
  (returns (ActiveEffects :type "Array of /Game/Core/Blueprints/Gameplay/Components/EffectComponent/BP_EffectBase Object Reference"))
  (return (`self.ActiveEffects`)))

(fn `HandleEffects`
  (locals (ActiveEffectsTemp :type "Array of /Game/Core/Blueprints/Gameplay/Components/EffectComponent/BP_EffectBase Object Reference"))
  (for _array_element (`self.ActiveEffects`)
    (bind _remainingtime (`/Game/Core/Blueprints/Gameplay/Components/EffectComponent/BP_EffectBase.GetRemainingTime` _array_element))
    (if (> _remainingtime 0.0)
      (`/Game/Core/Blueprints/Gameplay/Components/EffectComponent/BP_EffectBase.SetRemainingTime` _array_element (`KismetMathLibrary.FMax` (- _remainingtime (`self.RefreshRate`))))
      (if (> _remainingtime 0.0)
        (`KismetArrayLibrary.Array_Add` (`local.ActiveEffectsTemp`) _array_element)
        (else
          (`self.RemoveEffect` _array_element)))
      (else
        (`KismetArrayLibrary.Array_Add` (`local.ActiveEffectsTemp`) _array_element))))
  (bind _output_get (set `self.ActiveEffects` (`local.ActiveEffectsTemp`)))
  (if (== (`KismetArrayLibrary.Array_Length` _output_get) 0)
    (`KismetSystemLibrary.K2_ClearAndInvalidateTimerHandle` (`self.EffectsTimer`))))

(fn `HandleRepeatEffects`
  (bind _repeateffects (`self.RepeatEffects`))
  (bind _keys (`BlueprintMapLibrary.Map_Keys` (`self.RepeatEffects`)))
  (for _array_element _keys
    (`BlueprintMapLibrary.Map_Add` _repeateffects _array_element (`KismetMathLibrary.FMax` (- (`BlueprintMapLibrary.Map_Find` (`self.RepeatEffects`) _array_element) (`self.RefreshRate`))))
    (if (== (`BlueprintMapLibrary.Map_Find` _repeateffects _array_element) 0.0)
      (`self.ApplyEffectStats` _array_element)
      (`BlueprintMapLibrary.Map_Add` (`self.RepeatEffects`) _array_element (`.Duration_15_751B006441C44630FFE50E8372555D15` (break `/Game/Core/Blueprints/Gameplay/Components/EffectComponent/Structures/ST_EffectData` (`/Game/Core/Blueprints/Gameplay/Components/EffectComponent/BP_EffectBase.EffectData` _array_element)))))))

(fn `HasEffect`
  (params (Effect :type "/Game/Core/Blueprints/Gameplay/Components/EffectComponent/BP_EffectBase Class Reference"))
  (returns (Success :type Boolean))
  (for _array_element (`self.ActiveEffects`)
    (if (== (`GameplayStatics.GetObjectClass` _array_element) (`local.Effect`))
      (return true)))
  (return false))

(fn `Init`
  (set `self.StatComponent` (`Actor.GetComponentByClass` (`self.GetOwner`) "/Game/Core/Blueprints/Gameplay/Components/StatComponent/BPC_StatComponent.BPC_StatComponent_C"))
  (set `self.AttributeComponent` (`Actor.GetComponentByClass` (`self.GetOwner`) "/Game/Core/Blueprints/Gameplay/Components/AttributeComponent/BPC_AttributeComponent.BPC_AttributeComponent_C")))

(fn `OnRep_ActiveEffects`
  (`self.OnUpdatedActiveEffects` (`self.ActiveEffects`)))

(fn `RemoveEffect`
  (params (Effect :type "/Game/Core/Blueprints/Gameplay/Components/EffectComponent/BP_EffectBase Object Reference"))
  (bind _value (`BlueprintMapLibrary.Map_Find` (`self.EffectVisualActors`) (`local.Effect`)))
  (`|ExecutionSequence`
    (:`then_0`
      (for _array_element (`.ActiveAdditiveAttributes_20_5BEBDC294E2A46C26B27898069AB169A` (break `/Game/Core/Blueprints/Gameplay/Components/EffectComponent/Structures/ST_EffectData` (`/Game/Core/Blueprints/Gameplay/Components/EffectComponent/BP_EffectBase.EffectData` (`local.Effect`))))
        (`/Game/Core/Blueprints/Gameplay/Components/AttributeComponent/BPC_AttributeComponent.RemoveAdditiveAttribute` (`self.AttributeComponent`) _array_element)))
    (:`then_1`
      (if (> (`.RepeatRate_13_4749ECE0481191AC71A885A560C73C53` (break `/Game/Core/Blueprints/Gameplay/Components/EffectComponent/Structures/ST_EffectData` (`/Game/Core/Blueprints/Gameplay/Components/EffectComponent/BP_EffectBase.EffectData` (`local.Effect`)))) 0.0)
        (bind _returnvalue (`BlueprintMapLibrary.Map_Remove` (`self.RepeatEffects`) (`local.Effect`)))
        (if _returnvalue
          (if (== (`BlueprintMapLibrary.Map_Length` (`self.RepeatEffects`)) 0)
            (`KismetSystemLibrary.K2_ClearAndInvalidateTimerHandle` (`self.RepeatEffectsTimer`))))))
    (:`then_2`
      (`/Engine/EditorBlueprintResources/StandardMacros.IsValid` _value
        (:`Is Valid`
          (`Actor.K2_DestroyActor` _value)
          (`BlueprintMapLibrary.Map_Remove` (`self.EffectVisualActors`) (`local.Effect`)))))
    (:`then_3`
      (`/Game/Core/Blueprints/Gameplay/Components/EffectComponent/BP_EffectBase.OnEffectRemoved` (`local.Effect`)))
    (:`then_4`
      (`Actor.K2_DestroyActor` (`local.Effect`)))))

(fn `RemoveEffectByClass`
  (params (Effect :type "/Game/Core/Blueprints/Gameplay/Components/EffectComponent/BP_EffectBase Class Reference"))
  (for _array_element (`self.ActiveEffects`)
    (if (== (`GameplayStatics.GetObjectClass` _array_element) (`local.Effect`))
      (`self.RemoveEffect` _array_element)
      (`KismetArrayLibrary.Array_RemoveItem` (`self.ActiveEffects`) _array_element)
      (set `self.ActiveEffects` (`self.ActiveEffects`))
      (`|ExecutionSequence`
        (:`then_0`
          (if (== (`KismetArrayLibrary.Array_Length` (`self.ActiveEffects`)) 0)
            (`KismetSystemLibrary.K2_ClearAndInvalidateTimerHandle` (`self.EffectsTimer`))))
        (:`then_1`
          (return))))))