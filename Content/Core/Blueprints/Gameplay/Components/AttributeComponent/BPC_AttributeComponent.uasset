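; Actor component that holds gameplay-tagged attribute values, copied from defaults on BeginPlay or when new defaults are set.
; Additive or multiply modifiers are logged and applied directly to the matching value.
; Removal applies the inverse operation, even without a logged match, so mixed modifier types are order-sensitive.
; Modifier edits re-assign the array to trigger its RepNotify, which broadcasts OnUpdatedAttributes.
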(event `self.ReceiveBeginPlay`
  (`self.Init`))

(fn `AddAdditiveAttribute`
  (params (AdditiveAttribute :type "/Game/Core/Blueprints/Gameplay/Components/AttributeComponent/Structures/ST_AdditiveAttributeData Structure"))
  (locals (IndexTemp :type Integer) (ValueTemp :type "Float (double-precision)"))
  (bind (_attributetag _additivetype _value) (break `/Game/Core/Blueprints/Gameplay/Components/AttributeComponent/Structures/ST_AdditiveAttributeData` (`local.AdditiveAttribute`)))
  (`KismetArrayLibrary.Array_Add` (`self.AdditiveAttributes`) (`local.AdditiveAttribute`))
  (for (_array_element _array_index) (`self.Attributes`)
    (set `local.IndexTemp` _array_index)
    (bind (_attributetag_2 _value_2) (break `/Game/Core/Blueprints/Gameplay/Components/AttributeComponent/Structures/ST_AttributeData` _array_element))
    (if (== _attributetag_2 _attributetag)
      (set `local.ValueTemp` _value_2)
      (`|ExecutionSequence`
        (:`then_0`
          (switch `/Game/Core/Blueprints/Gameplay/Components/AttributeComponent/Enums/E_AttributeAdditiveTypes` _additivetype
            (:`NewEnumerator0`
              (set `local.ValueTemp` (+ (`local.ValueTemp`) _value)))
            (:`NewEnumerator1`
              (set `local.ValueTemp` (* (`local.ValueTemp`) _value)))))
        (:`then_1`
          (setmembers `/Game/Core/Blueprints/Gameplay/Components/AttributeComponent/Structures/ST_AttributeData` :`StructRef` (`|GetArrayItem` (`self.Attributes`) (`local.IndexTemp`)) :`Value` (`local.ValueTemp`))
          (set `self.Attributes` (`self.Attributes`)))
        (:`then_2`
          (return))))))

(fn `GetAttribute`
  (params (AttributeTag :type "GameplayTag Structure"))
  (returns (Attribute :type "/Game/Core/Blueprints/Gameplay/Components/AttributeComponent/Structures/ST_AttributeData Structure"))
  (for _array_element (`self.Attributes`)
    (if (== (`.AttributeTag_2_4B3A00D94E5A22AAF7FA67A62D3C031A` (break `/Game/Core/Blueprints/Gameplay/Components/AttributeComponent/Structures/ST_AttributeData` _array_element)) (`local.AttributeTag`))
      (return _array_element)))
  (return))

(fn `GetAttributes`
  (returns (Attributes :type "Array of /Game/Core/Blueprints/Gameplay/Components/AttributeComponent/Structures/ST_AttributeData Structure"))
  (return (`self.Attributes`)))

(fn `Init`
  (set `self.Attributes` (`self.DefaultAttributes`)))

(fn `OnRep_Attributes`
  (`self.OnUpdatedAttributes` (`self.Attributes`)))

(fn `RemoveAdditiveAttribute`
  (params (AdditiveAttribute :type "/Game/Core/Blueprints/Gameplay/Components/AttributeComponent/Structures/ST_AdditiveAttributeData Structure"))
  (locals (IndexTemp :type Integer) (ValueTemp :type "Float (double-precision)"))
  (bind (_attributetag _additivetype _value) (break `/Game/Core/Blueprints/Gameplay/Components/AttributeComponent/Structures/ST_AdditiveAttributeData` (`local.AdditiveAttribute`)))
  (bind (_attributetag_2 _additivetype_2 _value_2) (break `/Game/Core/Blueprints/Gameplay/Components/AttributeComponent/Structures/ST_AdditiveAttributeData` (`local.AdditiveAttribute`)))
  (`|ExecutionSequence`
    (:`then_0`
      (for (_array_element _array_index) (`self.AdditiveAttributes`)
        (bind (_attributetag_3 _additivetype_3 _value_3) (break `/Game/Core/Blueprints/Gameplay/Components/AttributeComponent/Structures/ST_AdditiveAttributeData` _array_element))
        (if (and (== _attributetag_3 _attributetag_2) (`|EnumEquality` _additivetype_3 _additivetype_2) (== _value_3 _value_2))
          (`KismetArrayLibrary.Array_Remove` (`self.AdditiveAttributes`) _array_index)
          (break))))
    (:`then_1`
      (for (_array_element_2 _array_index_2) (`self.Attributes`)
        (set `local.IndexTemp` _array_index_2)
        (bind (_attributetag_4 _value_4) (break `/Game/Core/Blueprints/Gameplay/Components/AttributeComponent/Structures/ST_AttributeData` _array_element_2))
        (if (== _attributetag_4 _attributetag)
          (set `local.ValueTemp` _value_4)
          (`|ExecutionSequence`
            (:`then_0`
              (switch `/Game/Core/Blueprints/Gameplay/Components/AttributeComponent/Enums/E_AttributeAdditiveTypes` _additivetype
                (:`NewEnumerator0`
                  (set `local.ValueTemp` (- (`local.ValueTemp`) _value)))
                (:`NewEnumerator1`
                  (set `local.ValueTemp` (/ (`local.ValueTemp`) _value)))))
            (:`then_1`
              (setmembers `/Game/Core/Blueprints/Gameplay/Components/AttributeComponent/Structures/ST_AttributeData` :`StructRef` (`|GetArrayItem` (`self.Attributes`) (`local.IndexTemp`)) :`Value` (`local.ValueTemp`))
              (set `self.Attributes` (`self.Attributes`)))
            (:`then_2`
              (return))))))))

(fn `SetDefaultAttributes`
  (params (DefaultAttributes :type "Array of /Game/Core/Blueprints/Gameplay/Components/AttributeComponent/Structures/ST_AttributeData Structure"))
  (bind _output_get (set `self.DefaultAttributes` DefaultAttributes))
  (set `self.Attributes` _output_get))