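; Character manager component that keeps a replicated registry of characters for other systems to read.
; Register and unregister functions add uniquely to or remove from RegisteredCharacters, and a getter returns the list.
; Each change reassigns the array to itself so its RepNotify fires, which broadcasts OnUpdatedRegisteredCharacters with the current list.
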(fn `GetRegisteredCharacters`
  (returns (RegisteredCharacters :type "Array of /Game/Core/Blueprints/Gameplay/Characters/BP_CharacterBase Object Reference"))
  (return (`self.RegisteredCharacters`)))

(fn `OnRep_RegisteredCharacters`
  (`self.OnUpdatedRegisteredCharacters` (`self.RegisteredCharacters`)))

(fn `RegisterCharacter`
  (params (Character :type "/Game/Core/Blueprints/Gameplay/Characters/BP_CharacterBase Object Reference (by ref)"))
  (`KismetArrayLibrary.Array_AddUnique` (`self.RegisteredCharacters`) (`local.Character`))
  (set `self.RegisteredCharacters` (`self.RegisteredCharacters`)))

(fn `UnregisterCharacter`
  (params (Character :type "/Game/Core/Blueprints/Gameplay/Characters/BP_CharacterBase Object Reference (by ref)"))
  (`KismetArrayLibrary.Array_RemoveItem` (`self.RegisteredCharacters`) (`local.Character`))
  (set `self.RegisteredCharacters` (`self.RegisteredCharacters`)))