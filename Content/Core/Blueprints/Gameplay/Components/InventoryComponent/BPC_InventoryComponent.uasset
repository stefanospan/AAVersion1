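; Actor component that holds a fixed-size, replicated inventory of item-class slots with amounts, sized on the authority at begin play.
; Adding fills existing stacks, then free slots up to each class's MaxStack, returning any remainder.
; Drops from other inventories or equipment try the target slot, then free slots, before updating the source.
; Using an item constructs it, calls OnUse and optionally consumes one; OnRep broadcasts slot updates.
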(event `self.ReceiveBeginPlay`
  (`self.Init`))

(fn `AddItem`
  (params (Item :type "/Game/Core/Blueprints/Gameplay/Components/InventoryComponent/BP_ItemBase Class Reference") (Amount :type Integer))
  (returns (RemainingAmount :type Integer))
  (locals (RemainingAmountTemp :type Integer :default 0) (AmountToAdd :type Integer))
  (bind ((`CanStack_8_61F835924643783BBB3323BD9E2AB6A8` _canstack) (`MaxStack_11_D1308E624981064A24C8719DACF28EBB` _maxstack)) (break `/Game/Core/Blueprints/Gameplay/Components/InventoryComponent/Structures/ST_ItemData` (defaults `Object` (`local.Item`))))
  (if (and (`KismetSystemLibrary.IsValidClass` Item) (> Amount 0))
    (set `local.RemainingAmountTemp` (`local.Amount`))
    (bind _remainingamount (`self.TryStack` (`local.Item`) (`local.RemainingAmountTemp`)))
    (bind _output_get (set `local.RemainingAmountTemp` _remainingamount))
    (if (> _output_get 0)
      (while (> (`local.RemainingAmountTemp`) 0)
        (bind (_found _slotindex) (`self.FindFreeSlot`))
        (if _found
          (bind _output_get_2 (set `local.AmountToAdd` (`KismetMathLibrary.Min` (select `bool` _canstack :`false` 1 :`true` _maxstack) (`local.RemainingAmountTemp`))))
          (`self.SetSlotAtIndex` _slotindex (`local.Item`) _output_get_2)
          (set `local.RemainingAmountTemp` (- (`local.RemainingAmountTemp`) (`local.AmountToAdd`)))
          (else
            (return (`local.RemainingAmountTemp`)))))
      (return 0)
      (else
        (return 0)))
    (else
      (return 0))))

(fn `DropFromEquipment`
  (params (FromEquipmentComponent :type "/Game/Core/Blueprints/Gameplay/Components/EquipmentComponent/BPC_EquipmentComponent Object Reference") (FromEquipmentSlot :type "/Game/Core/Blueprints/Gameplay/Components/EquipmentComponent/Enums/E_EquipmentSlots Enum" :default "NewEnumerator0") (ToSlotIndex :type Integer))
  (returns (Success :type Boolean))
  (locals (Item :type "/Game/Core/Blueprints/Gameplay/Components/InventoryComponent/BP_ItemBase Class Reference") (RemainingAmount :type Integer) (AmountToAdd :type Integer) (BreakLoop :type Boolean) (AmountToRemove :type Integer))
  (bind ((`EquipmentItem_6_6AB0AAAF45B76011F96BD2AAF6AEDC54` _equipmentitem)) (break `/Game/Core/Blueprints/Gameplay/Components/EquipmentComponent/Structures/ST_EquipmentSlot` (`/Game/Core/Blueprints/Gameplay/Components/EquipmentComponent/BPC_EquipmentComponent.GetEquipmentSlot` FromEquipmentComponent FromEquipmentSlot)))
  (bind (_item _amount) (break `/Game/Core/Blueprints/Gameplay/Components/InventoryComponent/Structures/ST_InventorySlot` (`self.GetSlotAtIndex` (`local.ToSlotIndex`))))
  (bind ((`CanStack_8_61F835924643783BBB3323BD9E2AB6A8` _canstack) (`MaxStack_11_D1308E624981064A24C8719DACF28EBB` _maxstack)) (break `/Game/Core/Blueprints/Gameplay/Components/InventoryComponent/Structures/ST_ItemData` (defaults `Object` (`local.Item`))))
  (bind (_item_2 _amount_2) (break `/Game/Core/Blueprints/Gameplay/Components/InventoryComponent/Structures/ST_InventorySlot` (`self.GetSlotAtIndex` (`local.ToSlotIndex`))))
  (bind ((`CanStack_8_61F835924643783BBB3323BD9E2AB6A8` _canstack_2) (`MaxStack_11_D1308E624981064A24C8719DACF28EBB` _maxstack_2)) (break `/Game/Core/Blueprints/Gameplay/Components/InventoryComponent/Structures/ST_ItemData` (defaults `Object` (`local.Item`))))
  (bind ((`CanStack_8_61F835924643783BBB3323BD9E2AB6A8` _canstack_3) (`MaxStack_11_D1308E624981064A24C8719DACF28EBB` _maxstack_3)) (break `/Game/Core/Blueprints/Gameplay/Components/InventoryComponent/Structures/ST_ItemData` (defaults `Object` (`local.Item`))))
  (if (`KismetSystemLibrary.IsValidClass` _equipmentitem)
    (set `local.Item` _equipmentitem)
    (set `local.RemainingAmount` 1)
    (`|ExecutionSequence`
      (:`then_0`
        (if (and (`KismetSystemLibrary.IsValidClass` _item) (> _amount 0))
          (if (and (== _item_2 (`local.Item`)) _canstack_2 (< _amount_2 _maxstack_2))
            (set `local.AmountToAdd` (`KismetMathLibrary.Min` (- _maxstack_2 _amount_2) (`local.RemainingAmount`)))
            (`self.SetSlotAtIndex` (`local.ToSlotIndex`) (`local.Item`) (+ (`.Amount_5_E4575F814081AE76E355FCB6AECAA721` (break `/Game/Core/Blueprints/Gameplay/Components/InventoryComponent/Structures/ST_InventorySlot` (`self.GetSlotAtIndex` (`local.ToSlotIndex`)))) (`local.AmountToAdd`)))
            (set `local.RemainingAmount` (- (`local.RemainingAmount`) (`local.AmountToAdd`))))
          (else
            (set `local.AmountToAdd` (`KismetMathLibrary.Min` (select `bool` _canstack_3 :`false` 1 :`true` _maxstack_3) (`local.RemainingAmount`)))
            (set `local.RemainingAmount` (- (`local.RemainingAmount`) (`local.AmountToAdd`)))
            (`self.SetSlotAtIndex` (`local.ToSlotIndex`) (`local.Item`) (`local.AmountToAdd`)))))
      (:`then_1`
        (if (> (`local.RemainingAmount`) 0)
          (set `local.BreakLoop` false)
          (while (and (> (`local.RemainingAmount`) 0) (not (`local.BreakLoop`)))
            (bind (_found _slotindex) (`self.FindFreeSlot`))
            (if _found
              (set `local.AmountToAdd` (`KismetMathLibrary.Min` (select `bool` _canstack :`false` 1 :`true` _maxstack) (`local.RemainingAmount`)))
              (set `local.RemainingAmount` (- (`local.RemainingAmount`) (`local.AmountToAdd`)))
              (`self.SetSlotAtIndex` _slotindex (`local.Item`) (`local.AmountToAdd`))
              (else
                (set `local.BreakLoop` true))))))
      (:`then_2`
        (if (== (`local.RemainingAmount`) 0)
          (`/Game/Core/Blueprints/Gameplay/Components/EquipmentComponent/BPC_EquipmentComponent.UnequipSlot` (`local.FromEquipmentComponent`) (`local.FromEquipmentSlot`))
          (return true)
          (else
            (return false)))))
    (else
      (return false))))

(fn `DropFromInventory`
  (params (FromInventoryComponent :type "/Game/Core/Blueprints/Gameplay/Components/InventoryComponent/BPC_InventoryComponent Object Reference") (FromSlotIndex :type Integer) (ToSlotIndex :type Integer))
  (returns (Success :type Boolean))
  (locals (Item :type "/Game/Core/Blueprints/Gameplay/Components/InventoryComponent/BP_ItemBase Class Reference") (RemainingAmount :type Integer) (AmountToAdd :type Integer) (BreakLoop :type Boolean) (AmountToRemove :type Integer) (InitAmount :type Integer))
  (bind _remainingamount (`local.RemainingAmount`))
  (bind (_item _amount) (break `/Game/Core/Blueprints/Gameplay/Components/InventoryComponent/Structures/ST_InventorySlot` (`self.GetSlotAtIndex` FromInventoryComponent FromSlotIndex)))
  (bind (_item_2 _amount_2) (break `/Game/Core/Blueprints/Gameplay/Components/InventoryComponent/Structures/ST_InventorySlot` (`self.GetSlotAtIndex` (`local.ToSlotIndex`))))
  (bind ((`CanStack_8_61F835924643783BBB3323BD9E2AB6A8` _canstack) (`MaxStack_11_D1308E624981064A24C8719DACF28EBB` _maxstack)) (break `/Game/Core/Blueprints/Gameplay/Components/InventoryComponent/Structures/ST_ItemData` (defaults `Object` (`local.Item`))))
  (bind (_item_3 _amount_3) (break `/Game/Core/Blueprints/Gameplay/Components/InventoryComponent/Structures/ST_InventorySlot` (`self.GetSlotAtIndex` (`local.ToSlotIndex`))))
  (bind ((`CanStack_8_61F835924643783BBB3323BD9E2AB6A8` _canstack_2) (`MaxStack_11_D1308E624981064A24C8719DACF28EBB` _maxstack_2)) (break `/Game/Core/Blueprints/Gameplay/Components/InventoryComponent/Structures/ST_ItemData` (defaults `Object` (`local.Item`))))
  (bind ((`CanStack_8_61F835924643783BBB3323BD9E2AB6A8` _canstack_3) (`MaxStack_11_D1308E624981064A24C8719DACF28EBB` _maxstack_3)) (break `/Game/Core/Blueprints/Gameplay/Components/InventoryComponent/Structures/ST_ItemData` (defaults `Object` (`local.Item`))))
  (if (and (`KismetSystemLibrary.IsValidClass` _item) (> _amount 0))
    (set `local.Item` _item)
    (set `local.RemainingAmount` _amount)
    (set `local.InitAmount` _amount)
    (`|ExecutionSequence`
      (:`then_0`
        (if (and (`KismetSystemLibrary.IsValidClass` _item_2) (> _amount_2 0))
          (if (and (== _item_3 (`local.Item`)) _canstack_2 (< _amount_3 _maxstack_2))
            (set `local.AmountToAdd` (`KismetMathLibrary.Min` (- _maxstack_2 _amount_3) (`local.RemainingAmount`)))
            (`self.SetSlotAtIndex` (`local.ToSlotIndex`) (`local.Item`) (+ (`.Amount_5_E4575F814081AE76E355FCB6AECAA721` (break `/Game/Core/Blueprints/Gameplay/Components/InventoryComponent/Structures/ST_InventorySlot` (`self.GetSlotAtIndex` (`local.ToSlotIndex`)))) (`local.AmountToAdd`)))
            (set `local.RemainingAmount` (- (`local.RemainingAmount`) (`local.AmountToAdd`))))
          (else
            (set `local.AmountToAdd` (`KismetMathLibrary.Min` (select `bool` _canstack_3 :`false` 1 :`true` _maxstack_3) (`local.RemainingAmount`)))
            (set `local.RemainingAmount` (- (`local.RemainingAmount`) (`local.AmountToAdd`)))
            (`self.SetSlotAtIndex` (`local.ToSlotIndex`) (`local.Item`) (`local.AmountToAdd`)))))
      (:`then_1`
        (if (> (`local.RemainingAmount`) 0)
          (set `local.BreakLoop` false)
          (while (and (> (`local.RemainingAmount`) 0) (not (`local.BreakLoop`)))
            (bind (_found _slotindex) (`self.FindFreeSlot`))
            (if _found
              (set `local.AmountToAdd` (`KismetMathLibrary.Min` (select `bool` _canstack :`false` 1 :`true` _maxstack) (`local.RemainingAmount`)))
              (set `local.RemainingAmount` (- (`local.RemainingAmount`) (`local.AmountToAdd`)))
              (`self.SetSlotAtIndex` _slotindex (`local.Item`) (`local.AmountToAdd`))
              (else
                (set `local.BreakLoop` true))))))
      (:`then_2`
        (`self.SetSlotAtIndex` (`local.FromInventoryComponent`) (`local.FromSlotIndex`) (select `bool` (> _remainingamount 0) :`true` (`local.Item`)) _remainingamount)
        (return (!= (`local.RemainingAmount`) (`local.InitAmount`)))))
    (else
      (return false))))

(fn `FindFreeSlot`
  (returns (Found :type Boolean) (SlotIndex :type Integer))
  (for (_array_element _array_index) (`self.Slots`)
    (bind (_item _amount) (break `/Game/Core/Blueprints/Gameplay/Components/InventoryComponent/Structures/ST_InventorySlot` _array_element))
    (if (or (not (`KismetSystemLibrary.IsValidClass` _item)) (== _amount 0))
      (return true _array_index)))
  (return false -1))

(fn `GetAmountForItem`
  (params (Item :type "/Game/Core/Blueprints/Gameplay/Components/InventoryComponent/BP_ItemBase Class Reference"))
  (returns (Amount :type Integer))
  (locals (AmountTemp :type Integer :default 0))
  (for _array_element (`self.Slots`)
    (bind (_item _amount) (break `/Game/Core/Blueprints/Gameplay/Components/InventoryComponent/Structures/ST_InventorySlot` _array_element))
    (if (== _item (`local.Item`))
      (set `local.AmountTemp` (+ _amount (`local.AmountTemp`)))))
  (return (`local.AmountTemp`)))

(fn `GetSlotAtIndex`
  (params (Index :type Integer))
  (returns (Slot :type "/Game/Core/Blueprints/Gameplay/Components/InventoryComponent/Structures/ST_InventorySlot Structure"))
  (return (`|GetArrayItem` (`self.Slots`) (`local.Index`))))

(fn `GetSlots`
  (returns (Slots :type "Array of /Game/Core/Blueprints/Gameplay/Components/InventoryComponent/Structures/ST_InventorySlot Structure"))
  (return (`self.Slots`)))

(fn `Init`
  (`/Engine/EditorBlueprintResources/ActorComponentMacros.Switch Has Authority`
    (:`Authority`
      (`KismetArrayLibrary.Array_Resize` (`self.Slots`) (`self.TotalSlots`))
      (set `self.Slots` (`self.Slots`)))))

(fn `OnRep_Slots`
  (`self.OnUpdatedSlots` (`self.Slots`)))

(fn `RemoveAmountAtSlot`
  (params (SlotIndex :type Integer) (Amount :type Integer))
  (bind (_item _amount) (break `/Game/Core/Blueprints/Gameplay/Components/InventoryComponent/Structures/ST_InventorySlot` (`self.GetSlotAtIndex` SlotIndex)))
  (bind _returnvalue (`KismetMathLibrary.Max` (- _amount (`local.Amount`))))
  (`self.SetSlotAtIndex` (`local.SlotIndex`) (select `bool` (> _returnvalue 0) :`true` _item) _returnvalue))

(fn `RemoveItem`
  (params (Item :type "/Game/Core/Blueprints/Gameplay/Components/InventoryComponent/BP_ItemBase Class Reference") (Amount :type Integer))
  (locals (RemainingAmount :type Integer) (AmountToRemove :type Integer :default 0))
  (set `local.RemainingAmount` Amount)
  (for (_array_element _array_index) (`self.Slots`)
    (bind (_item _amount) (break `/Game/Core/Blueprints/Gameplay/Components/InventoryComponent/Structures/ST_InventorySlot` _array_element))
    (if (== _item (`local.Item`))
      (set `local.AmountToRemove` (`KismetMathLibrary.Min` _amount (`local.RemainingAmount`)))
      (`self.RemoveAmountAtSlot` _array_index (`local.AmountToRemove`))
      (bind _output_get (set `local.RemainingAmount` (- (`local.RemainingAmount`) (`local.AmountToRemove`))))
      (if (== _output_get 0)
        (return)))))

(fn `SetSlotAtIndex`
  (params (SlotIndex :type Integer) (Item :type "/Game/Core/Blueprints/Gameplay/Components/InventoryComponent/BP_ItemBase Class Reference") (Amount :type Integer))
  (setmembers `/Game/Core/Blueprints/Gameplay/Components/InventoryComponent/Structures/ST_InventorySlot` :`StructRef` (`|GetArrayItem` (`self.Slots`) (`local.SlotIndex`)) :`Item` (`local.Item`) :`Amount` (`local.Amount`))
  (set `self.Slots` (`self.Slots`)))

(fn `TryStack`
  (params (Item :type "/Game/Core/Blueprints/Gameplay/Components/InventoryComponent/BP_ItemBase Class Reference") (Amount :type Integer))
  (returns (RemainingAmount :type Integer))
  (locals (RemainingAmountTemp :type Integer :default 0) (AmountToStack :type Integer :default 0) (Index :type Integer))
  (bind ((`CanStack_8_61F835924643783BBB3323BD9E2AB6A8` _canstack) (`MaxStack_11_D1308E624981064A24C8719DACF28EBB` _maxstack)) (break `/Game/Core/Blueprints/Gameplay/Components/InventoryComponent/Structures/ST_ItemData` (defaults `Object` Item)))
  (bind _output (`|GetArrayItem` (`self.Slots`) (`local.Index`)))
  (bind ((`MaxStack_11_D1308E624981064A24C8719DACF28EBB` _maxstack_2)) (break `/Game/Core/Blueprints/Gameplay/Components/InventoryComponent/Structures/ST_ItemData` (defaults `Object` (`local.Item`))))
  (if (and _canstack (> _maxstack 1))
    (set `local.RemainingAmountTemp` (`local.Amount`))
    (for (_array_element _array_index) (`self.Slots`)
      (set `local.Index` _array_index)
      (bind (_item _amount) (break `/Game/Core/Blueprints/Gameplay/Components/InventoryComponent/Structures/ST_InventorySlot` _array_element))
      (if (== _item (`local.Item`))
        (if (< _amount _maxstack_2)
          (set `local.AmountToStack` (`KismetMathLibrary.Min` (- _maxstack_2 _amount) (`local.RemainingAmountTemp`)))
          (setmembers `/Game/Core/Blueprints/Gameplay/Components/InventoryComponent/Structures/ST_InventorySlot` :`StructRef` _output :`Amount` (+ (`.Amount_5_E4575F814081AE76E355FCB6AECAA721` (break `/Game/Core/Blueprints/Gameplay/Components/InventoryComponent/Structures/ST_InventorySlot` _output)) (`local.AmountToStack`)))
          (bind _output_get (set `local.RemainingAmountTemp` (- (`local.RemainingAmountTemp`) (`local.AmountToStack`))))
          (if (== _output_get 0)
            (set `self.Slots` (`self.Slots`))
            (return 0)))))
    (set `self.Slots` (`self.Slots`))
    (return (`local.RemainingAmountTemp`))
    (else
      (return (`local.Amount`)))))

(fn `UseItem`
  (params (SlotIndex :type Integer))
  (bind ((`Item_2_E07371884F96B38E8DE52F8CF5E06799` _item)) (break `/Game/Core/Blueprints/Gameplay/Components/InventoryComponent/Structures/ST_InventorySlot` (`|GetArrayItem` (`self.Slots`) (`local.SlotIndex`))))
  (bind (_item_2 _amount) (break `/Game/Core/Blueprints/Gameplay/Components/InventoryComponent/Structures/ST_InventorySlot` (`|GetArrayItem` (`self.Slots`) (`local.SlotIndex`))))
  (bind ((`CanUse_16_7A7A028342B7A7F8D7739CB080165FEA` _canuse) (`ConsumeOnUse_18_10367F914E3836A2E5FB12905F2FF2DA` _consumeonuse)) (break `/Game/Core/Blueprints/Gameplay/Components/InventoryComponent/Structures/ST_ItemData` (defaults `Object` _item)))
  (if (and (`KismetSystemLibrary.IsValidClass` _item_2) (> _amount 0))
    (if _canuse
      (bind _returnvalue (`|GenericCreateObject` _item))
      (`/Game/Core/Blueprints/Gameplay/Components/InventoryComponent/BP_ItemBase.OnUse` _returnvalue self)
      (if _consumeonuse
        (`self.RemoveAmountAtSlot` (`local.SlotIndex`) 1)))))