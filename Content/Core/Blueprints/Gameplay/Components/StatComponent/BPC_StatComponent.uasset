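; Actor component that holds replicated, tag-keyed stats such as health, built from stat definitions and clamped between zero and max, and handles damage and death.
; Lowering a stat starts looping timers that count down per-stat regen delays, then regenerate values until full.
; On authority it binds owner damage, scales it by an attribute multiplier, shows damage text to player attackers and triggers replicated death at zero health.
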(event `self.ReceiveBeginPlay`
  (`self.Init`))

(event `MulticastOnReceivedDamage`
  (`self.OnReceivedDamage`))

(fn `AddStat`
  (params (StatTag :type "GameplayTag Structure") (value :type "Float (double-precision)"))
  (bind ((`RegenDelay_17_5F0CD4D1426D42E0BD19C2B9C8D9EDB5` _regendelay)) (break `/Game/Core/Blueprints/Gameplay/Components/StatComponent/Structures/ST_StatDefinitionData` (`self.GetStatDefinition` (`local.StatTag`))))
  (bind ((`MaxValue_9_B98E4DE245B99F0442DD6F99ED378288` _maxvalue) (`Regenerates_11_4FBF273F44E11A69FE7A9B8ED4E88666` _regenerates)) (break `/Game/Core/Blueprints/Gameplay/Components/StatComponent/Structures/ST_StatDefinitionData` (`self.GetStatDefinition` (`local.StatTag`))))
  (for (_array_element _array_index) (`self.Stats`)
    (bind (_stattag _value) (break `/Game/Core/Blueprints/Gameplay/Components/StatComponent/Structures/ST_StatData` _array_element))
    (if (== _stattag (`local.StatTag`))
      (bind _structout (setmembers `/Game/Core/Blueprints/Gameplay/Components/StatComponent/Structures/ST_StatData` :`StructRef` (`|GetArrayItem` (`self.Stats`) _array_index) :`Value` (`KismetMathLibrary.FClamp` (+ _value (`local.value`)) 0.0 _maxvalue)))
      (set `self.Stats` (`self.Stats`))
      (`|ExecutionSequence`
        (:`then_0`
          (if (and (< (`.Value_5_A6F0143D4480E30F17FD54AE8938D50C` (break `/Game/Core/Blueprints/Gameplay/Components/StatComponent/Structures/ST_StatData` _structout)) _maxvalue) _regenerates (< (`local.value`) 0.0))
            (if (> _regendelay 0.0)
              (`BlueprintMapLibrary.Map_Add` (`self.RegenDelays`) (`local.StatTag`) _regendelay)
              (if (not (`KismetSystemLibrary.K2_IsValidTimerHandle` (`self.RegenDelaysTimer`)))
                (bind _returnvalue (`KismetSystemLibrary.K2_SetTimerDelegate` (`|CreateDelegate` :!event `HandleRegenDelays`) (`self.RefreshRate`) true))
                (set `self.RegenDelaysTimer` _returnvalue))
              (elif (not (`KismetSystemLibrary.K2_IsValidTimerHandle` (`self.RegenTimer`)))
                (bind _returnvalue_2 (`KismetSystemLibrary.K2_SetTimerDelegate` (`|CreateDelegate` :!event `HandleRegen`) (`self.RefreshRate`) true))
                (set `self.RegenTimer` _returnvalue_2)))))
        (:`then_1`
          (return))))))

(fn `Death`
  (params (KillerActor :type "Actor Object Reference"))
  (`self.ServerOnDeath` KillerActor)
  (set `self.IsDead` true))

(fn `GetIsDead`
  (returns (IsDead :type Boolean))
  (return (`self.IsDead`)))

(fn `GetReceiveDamageMultiplier`
  (returns (Value :type "Float (double-precision)"))
  (bind _attributecomponent (`self.AttributeComponent`)
    (:`then`
      (return (`.Value_5_5382FAD64776275FF614BEB1A224EFA3` (break `/Game/Core/Blueprints/Gameplay/Components/AttributeComponent/Structures/ST_AttributeData` (`/Game/Core/Blueprints/Gameplay/Components/AttributeComponent/BPC_AttributeComponent.GetAttribute` _attributecomponent (struct :`TagName` "Attribute.ReceiveDamageMultiplier"))))))
    (:`else`
      (return 1.0))))

(fn `GetStat`
  (params (StatTag :type "GameplayTag Structure"))
  (returns (Stat :type "/Game/Core/Blueprints/Gameplay/Components/StatComponent/Structures/ST_StatData Structure"))
  (for _array_element (`self.Stats`)
    (if (== (`.StatTag_2_BA3311DD46B133E7C744D4BA88606A78` (break `/Game/Core/Blueprints/Gameplay/Components/StatComponent/Structures/ST_StatData` _array_element)) (`local.StatTag`))
      (return _array_element)))
  (return))

(fn `GetStatDefinition`
  (params (StatTag :type "GameplayTag Structure"))
  (returns (StatDefinition :type "/Game/Core/Blueprints/Gameplay/Components/StatComponent/Structures/ST_StatDefinitionData Structure"))
  (for _array_element (`self.StatDefinitions`)
    (if (== (`.StatTag_2_BA3311DD46B133E7C744D4BA88606A78` (break `/Game/Core/Blueprints/Gameplay/Components/StatComponent/Structures/ST_StatDefinitionData` _array_element)) (`local.StatTag`))
      (return _array_element)))
  (return))

(fn `GetStats`
  (returns (Stats :type "Array of /Game/Core/Blueprints/Gameplay/Components/StatComponent/Structures/ST_StatData Structure"))
  (return (`self.Stats`)))

(fn `HandleRegen`
  (locals (Found :type Boolean))
  (for (_array_element _array_index) (`self.Stats`)
    (bind (_stattag _value) (break `/Game/Core/Blueprints/Gameplay/Components/StatComponent/Structures/ST_StatData` _array_element))
    (bind ((`MaxValue_9_B98E4DE245B99F0442DD6F99ED378288` _maxvalue) (`Regenerates_11_4FBF273F44E11A69FE7A9B8ED4E88666` _regenerates) (`RegenRate_14_9E1807794D9DEDEFF338A998CEB8CB00` _regenrate)) (break `/Game/Core/Blueprints/Gameplay/Components/StatComponent/Structures/ST_StatDefinitionData` (`self.GetStatDefinition` _stattag)))
    (if (and (< _value _maxvalue) _regenerates)
      (if (not (`BlueprintMapLibrary.Map_Contains` (`self.RegenDelays`) _stattag))
        (bind _structout (setmembers `/Game/Core/Blueprints/Gameplay/Components/StatComponent/Structures/ST_StatData` :`StructRef` (`|GetArrayItem` (`self.Stats`) _array_index) :`Value` (`KismetMathLibrary.FClamp` (+ _value (* _regenrate (`self.RefreshRate`))) 0.0 _maxvalue)))
        (if (< (`.Value_5_A6F0143D4480E30F17FD54AE8938D50C` (break `/Game/Core/Blueprints/Gameplay/Components/StatComponent/Structures/ST_StatData` _structout)) _maxvalue)
          (set `local.Found` true)))))
  (set `self.Stats` (`self.Stats`))
  (if (not (`local.Found`))
    (`KismetSystemLibrary.K2_ClearAndInvalidateTimerHandle` (`self.RegenTimer`))))

(fn `HandleRegenDelays`
  (bind _regendelays (`self.RegenDelays`))
  (bind _keys (`BlueprintMapLibrary.Map_Keys` _regendelays))
  (for _array_element _keys
    (bind _returnvalue (`KismetMathLibrary.FMax` (- (`BlueprintMapLibrary.Map_Find` _regendelays _array_element) (`self.RefreshRate`))))
    (if (> _returnvalue 0.0)
      (`BlueprintMapLibrary.Map_Add` (`self.RegenDelays`) _array_element _returnvalue)
      (else
        (`BlueprintMapLibrary.Map_Remove` (`self.RegenDelays`) _array_element)
        (if (not (`KismetSystemLibrary.K2_IsValidTimerHandle` (`self.RegenTimer`)))
          (bind _returnvalue_2 (`KismetSystemLibrary.K2_SetTimerDelegate` (`|CreateDelegate` :!event `HandleRegen`) (`self.RefreshRate`) true))
          (set `self.RegenTimer` _returnvalue_2)))))
  (if (== (`BlueprintMapLibrary.Map_Length` (`self.RegenDelays`)) 0)
    (`KismetSystemLibrary.K2_ClearAndInvalidateTimerHandle` (`self.RegenDelaysTimer`))))

(fn `Init`
  (`|ExecutionSequence`
    (:`then_0`
      (`/Engine/EditorBlueprintResources/ActorComponentMacros.Switch Has Authority`
        (:`Authority`
          (`self.InitStatDefinitions`)
          (add `Actor.OnTakeAnyDamage` (`self.GetOwner`) (`|CreateDelegate` :!event `OnTakeAnyDamage`)))))
    (:`then_1`
      (`self.UpdateDead`)
      (set `self.AttributeComponent` (`Actor.GetComponentByClass` (`self.GetOwner`) "/Game/Core/Blueprints/Gameplay/Components/AttributeComponent/BPC_AttributeComponent.BPC_AttributeComponent_C")))))

(fn `InitStatDefinitions`
  (`KismetArrayLibrary.Array_Clear` (`self.Stats`))
  (for _array_element (`self.StatDefinitions`)
    (bind (_stattag _startingvalue _maxvalue) (break `/Game/Core/Blueprints/Gameplay/Components/StatComponent/Structures/ST_StatDefinitionData` _array_element))
    (`KismetArrayLibrary.Array_Add` (`self.Stats`) (make `/Game/Core/Blueprints/Gameplay/Components/StatComponent/Structures/ST_StatData` _stattag (`KismetMathLibrary.FClamp` _startingvalue 0.0 _maxvalue))))
  (set `self.Stats` (`self.Stats`)))

(fn `OnRep_IsDead`
  (`self.UpdateDead`))

(fn `OnRep_StatDefinitions`
  (`self.OnUpdatedStats` (`self.Stats`)))

(fn `OnRep_Stats`
  (`self.OnUpdatedStats` (`self.Stats`)))

(fn `OnTakeAnyDamage`
  (params (DamagedActor :type "Actor Object Reference") (Damage :type "Float (single-precision)") (DamageType :type "DamageType Object Reference") (InstigatedBy :type "Controller Object Reference") (DamageCauser :type "Actor Object Reference"))
  (locals (DamageTemp :type "Float (double-precision)"))
  (if (not (`self.IsDead`))
    (bind _output_get (set `local.DamageTemp` (* (`local.Damage`) (`self.GetReceiveDamageMultiplier`))))
    (`self.RemoveStat` (struct :`TagName` "Stat.Health") _output_get)
    (`self.MulticastOnReceivedDamage`)
    (`|ExecutionSequence`
      (:`then_0`
        (bind _aspawn (cast `Pawn` (`local.DamageCauser`)))
        (bind _asbp_player_controller_base (cast `/Game/Core/Blueprints/Gameplay/GameMode/BP_PlayerControllerBase` (`Pawn.GetController` _aspawn)))
        (`/Game/Core/Blueprints/Gameplay/GameMode/BP_PlayerControllerBase.ClientShowDamageText` _asbp_player_controller_base (`local.DamageTemp`) (`self.GetOwner`)))
      (:`then_1`
        (if (== (`.Value_5_A6F0143D4480E30F17FD54AE8938D50C` (break `/Game/Core/Blueprints/Gameplay/Components/StatComponent/Structures/ST_StatData` (`self.GetStat` (struct :`TagName` "Stat.Health")))) 0.0)
          (`self.Death` (`local.DamageCauser`)))))))

(fn `RemoveStat`
  (params (StatTag :type "GameplayTag Structure") (value :type "Float (double-precision)"))
  (bind ((`RegenDelay_17_5F0CD4D1426D42E0BD19C2B9C8D9EDB5` _regendelay)) (break `/Game/Core/Blueprints/Gameplay/Components/StatComponent/Structures/ST_StatDefinitionData` (`self.GetStatDefinition` (`local.StatTag`))))
  (bind ((`MaxValue_9_B98E4DE245B99F0442DD6F99ED378288` _maxvalue) (`Regenerates_11_4FBF273F44E11A69FE7A9B8ED4E88666` _regenerates)) (break `/Game/Core/Blueprints/Gameplay/Components/StatComponent/Structures/ST_StatDefinitionData` (`self.GetStatDefinition` (`local.StatTag`))))
  (for (_array_element _array_index) (`self.Stats`)
    (bind (_stattag _value) (break `/Game/Core/Blueprints/Gameplay/Components/StatComponent/Structures/ST_StatData` _array_element))
    (if (== _stattag (`local.StatTag`))
      (bind _structout (setmembers `/Game/Core/Blueprints/Gameplay/Components/StatComponent/Structures/ST_StatData` :`StructRef` (`|GetArrayItem` (`self.Stats`) _array_index) :`Value` (`KismetMathLibrary.FClamp` (- _value (`local.value`)) 0.0 _maxvalue)))
      (set `self.Stats` (`self.Stats`))
      (`|ExecutionSequence`
        (:`then_0`
          (if (and (< (`.Value_5_A6F0143D4480E30F17FD54AE8938D50C` (break `/Game/Core/Blueprints/Gameplay/Components/StatComponent/Structures/ST_StatData` _structout)) _maxvalue) _regenerates (> (`local.value`) 0.0))
            (if (> _regendelay 0.0)
              (`BlueprintMapLibrary.Map_Add` (`self.RegenDelays`) (`local.StatTag`) _regendelay)
              (if (not (`KismetSystemLibrary.K2_IsValidTimerHandle` (`self.RegenDelaysTimer`)))
                (bind _returnvalue (`KismetSystemLibrary.K2_SetTimerDelegate` (`|CreateDelegate` :!event `HandleRegenDelays`) (`self.RefreshRate`) true))
                (set `self.RegenDelaysTimer` _returnvalue))
              (elif (not (`KismetSystemLibrary.K2_IsValidTimerHandle` (`self.RegenTimer`)))
                (bind _returnvalue_2 (`KismetSystemLibrary.K2_SetTimerDelegate` (`|CreateDelegate` :!event `HandleRegen`) (`self.RefreshRate`) true))
                (set `self.RegenTimer` _returnvalue_2)))))
        (:`then_1`
          (return))))))

(fn `SetStatDefinitions`
  (params (StatDefinitions :type "Array of /Game/Core/Blueprints/Gameplay/Components/StatComponent/Structures/ST_StatDefinitionData Structure"))
  (set `self.StatDefinitions` StatDefinitions)
  (`self.InitStatDefinitions`))

(fn `SetStatMaxValue`
  (params (StatTag :type "GameplayTag Structure") (Value :type "Float (double-precision)") (ApplyAdditiveCurrentValue :type Boolean))
  (locals (PreviousMaxValue :type "Float (double-precision)"))
  (for (_array_element _array_index) (`self.StatDefinitions`)
    (bind ((`StatTag_2_BA3311DD46B133E7C744D4BA88606A78` _stattag) (`MaxValue_9_B98E4DE245B99F0442DD6F99ED378288` _maxvalue)) (break `/Game/Core/Blueprints/Gameplay/Components/StatComponent/Structures/ST_StatDefinitionData` _array_element))
    (if (== _stattag (`local.StatTag`))
      (set `local.PreviousMaxValue` _maxvalue)
      (setmembers `/Game/Core/Blueprints/Gameplay/Components/StatComponent/Structures/ST_StatDefinitionData` :`StructRef` (`|GetArrayItem` (`self.StatDefinitions`) _array_index) :`MaxValue` (`local.Value`))
      (set `self.StatDefinitions` (`self.StatDefinitions`))
      (for (_array_element_2 _array_index_2) (`self.Stats`)
        (if (== (`.StatTag_2_BA3311DD46B133E7C744D4BA88606A78` (break `/Game/Core/Blueprints/Gameplay/Components/StatComponent/Structures/ST_StatData` _array_element_2)) (`local.StatTag`))
          (bind _output (`|GetArrayItem` (`self.Stats`) _array_index_2))
          (setmembers `/Game/Core/Blueprints/Gameplay/Components/StatComponent/Structures/ST_StatData` :`StructRef` _output :`Value` (select `bool` (`local.ApplyAdditiveCurrentValue`) :`false` (`local.Value`) :`true` (+ (`.Value_5_A6F0143D4480E30F17FD54AE8938D50C` (break `/Game/Core/Blueprints/Gameplay/Components/StatComponent/Structures/ST_StatData` _output)) (- (`local.Value`) (`local.PreviousMaxValue`)))))
          (set `self.Stats` (`self.Stats`))
          (return))))))

(fn `UpdateDead`
  (if (`self.IsDead`)
    (`self.OnDeath`)))