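; Game State wave component that spawns enemies at nightfall, using the selected island's creature list and boss.
; On the authority, a looping timer polls Ultra Dynamic Sky time for day/night changes and broadcasts them.
; Every Nth day spawns the boss at the boss spawn actor.
; Other nights spawn day-scaled numbers of random creatures at navmesh points sampled in a ring around the first player found.
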(event `self.ReceiveBeginPlay`
  (`KismetSystemLibrary.Delay` 0.1)
  (`self.Init`))

(fn `CheckNight`
  (bind _time_of_day (`/Game/UltraDynamicSky/Blueprints/Ultra_Dynamic_Sky.Time of Day` (`self.UDS`)))
  (bind _returnvalue (or (>= _time_of_day 1800.0) (< _time_of_day 600.0)))
  (if (!= (`self.IsNight`) _returnvalue)
    (bind _output_get (set `self.IsNight` _returnvalue))
    (`self.OnUpdatedIsNight` _output_get)
    (if (`self.IsNight`)
      (`self.SpawnEnemies`))))

(fn `GetAmountToSpawn`
  (returns (Amount :type Integer))
  (return (+ (`self.InitialSpawnAmount`) (* (`/Game/Core/Blueprints/Gameplay/Components/DaySystemComponent/BPC_DaySystemComponent.GetCurrentDay` (`self.DaySystemComponent`)) (`self.AdditionalDaySpawnAmount`)))))

(fn `GetIsNight`
  (returns (IsNight :type Boolean))
  (return (`self.IsNight`)))

(fn `GetRandomLocationsInRange`
  (params (CenterLocation :type "Vector Structure") (Max :type Integer) (MaxTries :type Integer) (Radius :type "Vector2D Structure"))
  (returns (Locations :type "Array of Vector Structure"))
  (locals (LocationsTemp :type "Array of Vector Structure") (FinalLocations :type "Array of Vector Structure") (Found :type Boolean))
  (bind (_radius_x _radius_y) (`KismetMathLibrary.BreakVector2D` (`local.Radius`)))
  (bind (_radius_x_2 _radius_y_2) (`KismetMathLibrary.BreakVector2D` (`local.Radius`)))
  (for _ (range Max)
    (`KismetArrayLibrary.Array_Clear` (`local.LocationsTemp`))
    (for _ (range (`local.MaxTries`))
      (bind _randomlocation (`NavigationSystemV1.K2_GetRandomLocationInNavigableRadius` (`local.CenterLocation`) _radius_y_2 null null))
      (`KismetArrayLibrary.Array_Add` (`local.LocationsTemp`) _randomlocation)
      (if (`KismetMathLibrary.InRange_FloatFloat` (`KismetMathLibrary.Vector_Distance` _randomlocation (`local.CenterLocation`)) _radius_x _radius_y)
        (`KismetArrayLibrary.Array_Add` (`local.FinalLocations`) _randomlocation)
        (set `local.Found` true)
        (break)))
    (if (not (`local.Found`))
      (`KismetArrayLibrary.Array_Add` (`local.FinalLocations`) (`KismetArrayLibrary.Array_Random` (`local.LocationsTemp`)))))
  (return (`local.FinalLocations`)))

(fn `Init`
  (`/Engine/EditorBlueprintResources/ActorComponentMacros.Switch Has Authority`
    (:`Authority`
      (`|ExecutionSequence`
        (:`then_0`
          (set `self.DaySystemComponent` (`Actor.GetComponentByClass` (`self.GetOwner`) "/Game/Core/Blueprints/Gameplay/Components/DaySystemComponent/BPC_DaySystemComponent.BPC_DaySystemComponent_C")))
        (:`then_1`
          (bind _uds (`/Game/UltraDynamicSky/Blueprints/Functions/UltraDynamicSky_Functions.Get Ultra Dynamic Sky`))
          (set `self.UDS` _uds))
        (:`then_2`
          (bind _asbp_game_state_base (cast `/Game/Core/Blueprints/Gameplay/GameMode/BP_GameStateBase` (`self.GetOwner`)))
          (bind ((`BossCharacter_11_776DCEC740F1DD9803F3488A7D5148E4` _bosscharacter) (`SpawnableCreatures_16_C1EB94724D826F5F249EFFA611CFA69C` _spawnablecreatures)) (break `/Game/Core/Blueprints/Gameplay/Islands/Structures/ST_IslandData` (`/Game/Core/Blueprints/Gameplay/Islands/PDA_IslandBase.IslandData` (`/Game/Core/Blueprints/Gameplay/GameMode/BP_GameStateBase.GetSelectedIsland` _asbp_game_state_base))))
          (set `self.SpawnableCreatures` _spawnablecreatures)
          (set `self.BossCharacter` _bosscharacter))
        (:`then_3`
          (bind _returnvalue (`GameplayStatics.GetActorOfClass` "/Game/Core/Blueprints/Gameplay/Components/WaveSystemComponent/BP_BossSpawn.BP_BossSpawn_C"))
          (set `self.BossSpawnActor` _returnvalue))
        (:`then_4`
          (bind _returnvalue_2 (`KismetSystemLibrary.K2_SetTimerDelegate` (`|CreateDelegate` :!event `CheckNight`) 1.0 true))
          (set `self.Timer` _returnvalue_2))))))

(fn `IsBossRound`
  (returns (Success :type Boolean))
  (return (== (mod (+ (`/Game/Core/Blueprints/Gameplay/Components/DaySystemComponent/BPC_DaySystemComponent.GetCurrentDay` (`self.DaySystemComponent`)) 1) (`self.BossSpawnRound`)) 0)))

(fn `SpawnEnemies`
  (if (`self.IsBossRound`)
    (bind _returnvalue (`KismetSystemLibrary.LoadClassAsset_Blocking` (`self.BossCharacter`)))
    (bind _asbp_enemy_character_base (castclass `/Game/Core/Blueprints/Gameplay/Characters/EnemyCharacters/BP_EnemyCharacterBase` _returnvalue))
    (`|SpawnActorFromClass` _asbp_enemy_character_base (`Actor.GetTransform` (`self.BossSpawnActor`)) "Undefined" "MultiplyWithRoot" null null)
    (`self.OnBossSpawned`)
    (else
      (bind _returnvalue_2 (`GameplayStatics.GetActorOfClass` "/Game/Core/Blueprints/Gameplay/Characters/PlayerCharacters/BP_PlayerCharacterBase.BP_PlayerCharacterBase_C"))
      (bind _locations (`self.GetRandomLocationsInRange` (`Actor.K2_GetActorLocation` _returnvalue_2) 50 50 (1000.0 3000.0)))
      (for _ (range (`self.GetAmountToSpawn`))
        (`|SpawnActorFromClass` (`KismetArrayLibrary.Array_Random` (`self.SpawnableCreatures`)) (`KismetMathLibrary.MakeTransform` (`KismetArrayLibrary.Array_Random` _locations)) "AdjustIfPossibleButAlwaysSpawn" "MultiplyWithRoot" null null)))))