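; Base ability Blueprint for a custom ability system component, with overridable activation, CanActivate and montage event hooks.
; Commit and end calls fire dispatchers, and OnRep functions broadcast changes to remaining cooldown and current charges.
; Montages replicate through a server RPC to a multicast that plays on the owner character's mesh and forwards end and notify events.
; Helpers expose the owner character, local-control check and attributes via the AbilitySystemComponent.
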(event `OnAbilityActivated`)

(event `ServerPlayAnimMontage`
  (params (AnimMontage :type "AnimMontage Object Reference") (PlayRate :type "Float (single-precision)"))
  (`self.MulticastPlayAnimMontage` AnimMontage PlayRate))

(event `MulticastPlayAnimMontage`
  (params (AnimMontage :type "AnimMontage Object Reference") (PlayRate :type "Float (single-precision)" :default 1.0))
  (bind _notifyname (`|PlayMontage` (`Character.Mesh` (`self.GetOwnerCharacter`)) AnimMontage PlayRate)
    (:`OnCompleted`
      (`self.OnAnimMontageEnded` :!label _label))
    (:`OnInterrupted`
      (goto _label))
    (:`OnNotifyBegin`
      (`self.OnNotifyBegin` _notifyname))
    (:`OnNotifyEnd`
      (`self.OnNotifyEnd` _notifyname))))

(event `OnAnimMontageEnded`)

(event `OnNotifyBegin`
  (params (NotifyName :type Name)))

(event `OnNotifyEnd`
  (params (NotifyName :type Name)))

(fn `CanActivate`
  (returns (Success :type Boolean))
  (return true))

(fn `CommitAbility`
  (`self.OnAbilityCommit` self))

(fn `EndAbility`
  (`self.OnEndAbility` self))

(fn `GetAbilitySystemComponent`
  (returns (AbilitySystemComponent :type "/Game/Core/Blueprints/Gameplay/Components/AbilitySystemComponent/BPC_AbilitySystemComponent Object Reference"))
  (return (`self.AbilitySystemComponent`)))

(fn `GetAttribute`
  (params (AttributeTag :type "GameplayTag Structure"))
  (returns (Attribute :type "/Game/Core/Blueprints/Gameplay/Components/AttributeComponent/Structures/ST_AttributeData Structure"))
  (return (`/Game/Core/Blueprints/Gameplay/Components/AttributeComponent/BPC_AttributeComponent.GetAttribute` (`/Game/Core/Blueprints/Gameplay/Components/AbilitySystemComponent/BPC_AbilitySystemComponent.GetAttributeComponent` (`self.AbilitySystemComponent`)) (`local.AttributeTag`))))

(fn `GetCurrentCharges`
  (returns (CurrentCharges :type Integer))
  (return (`self.CurrentCharges`)))

(fn `GetOwnerCharacter`
  (returns (OwnerCharacter :type "/Game/Core/Blueprints/Gameplay/Characters/BP_CharacterBase Object Reference"))
  (return (`/Game/Core/Blueprints/Gameplay/Components/AbilitySystemComponent/BPC_AbilitySystemComponent.GetOwnerCharacter` (`self.AbilitySystemComponent`))))

(fn `GetRemainingCooldown`
  (returns (RemainingCooldown :type "Float (double-precision)"))
  (return (`self.RemainingCooldown`)))

(fn `IsLocal`
  (returns (Success :type Boolean))
  (return (`Pawn.IsLocallyControlled` (`self.GetOwnerCharacter`))))

(fn `OnRep_CurrentCharges`
  (`self.OnUpdatedCurrentCharges` (`self.CurrentCharges`)))

(fn `OnRep_RemainingCooldown`
  (`self.OnUpdatedRemainingCooldown` (`self.RemainingCooldown`)))

(fn `PlayAnimMontage`
  (params (AnimMontage :type "AnimMontage Object Reference") (PlayRate :type "Float (single-precision)" :default 1.0))
  (`/Engine/EditorBlueprintResources/ActorMacros.Switch Has Authority`
    (:`Authority`
      (`self.MulticastPlayAnimMontage` AnimMontage PlayRate))
    (:`Remote`
      (`self.ServerPlayAnimMontage` AnimMontage PlayRate))))

(fn `SetCurrentCharges`
  (params (CurrentCharges :type Integer))
  (set `self.CurrentCharges` CurrentCharges))

(fn `SetRemainingCooldown`
  (params (RemainingCooldown :type "Float (double-precision)"))
  (set `self.RemainingCooldown` RemainingCooldown))

(fn `UserConstructionScript`)