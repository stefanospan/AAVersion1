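; Character component that manages slot-based abilities, spawning DefaultAbilities as actors on the authority and notifying listeners when the replicated list updates.
; Activation by slot allows one active ability at a time, checks charges and CanActivate, and also calls the client event when not locally controlled.
; Ability commit spends a charge if it has a cooldown, and one shared looping timer restores charges sequentially; ending clears the active state.
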(event `self.ReceiveBeginPlay`
  (`self.Init`))

(event `ClientActivateAbility`
  (params (Ability :type "/Game/Core/Blueprints/Gameplay/Components/AbilitySystemComponent/BP_AbilityBase Object Reference"))
  (`/Game/Core/Blueprints/Gameplay/Components/AbilitySystemComponent/BP_AbilityBase.OnAbilityActivated` Ability))

(event `ServerActivateAbilityBySlot`
  (params (SlotTag :type "GameplayTag Structure"))
  (`self.ActivateAbilityBySlot` SlotTag))

(fn `ActivateAbilityBySlot`
  (params (SlotTag :type "GameplayTag Structure"))
  (if (`self.CanActivateAnyAbility`)
    (bind _ability (`self.GetAbilityBySlot` (`local.SlotTag`)))
    (bind _success (`self.CanActivateAbility` _ability))
    (if _success
      (set `self.IsAbilityActive` true)
      (set `self.ActiveAbility` _ability)
      (add `/Game/Core/Blueprints/Gameplay/Components/AbilitySystemComponent/BP_AbilityBase.OnAbilityCommit` (`self.ActiveAbility`) (`|CreateDelegate` :!event `OnAbilityCommit`))
      (add `/Game/Core/Blueprints/Gameplay/Components/AbilitySystemComponent/BP_AbilityBase.OnEndAbility` (`self.ActiveAbility`) (`|CreateDelegate` :!event `OnEndAbility`))
      (if (not (`self.IsLocallyControlled`))
        (`self.ClientActivateAbility` (`self.ActiveAbility`)))
      (`/Game/Core/Blueprints/Gameplay/Components/AbilitySystemComponent/BP_AbilityBase.OnAbilityActivated` (`self.ActiveAbility`)))))

(fn `CanActivateAbility`
  (params (Ability :type "/Game/Core/Blueprints/Gameplay/Components/AbilitySystemComponent/BP_AbilityBase Object Reference"))
  (returns (Success :type Boolean))
  (if (== (`/Game/Core/Blueprints/Gameplay/Components/AbilitySystemComponent/BP_AbilityBase.GetCurrentCharges` Ability) 0)
    (return false)
    (else
      (bind _success (`/Game/Core/Blueprints/Gameplay/Components/AbilitySystemComponent/BP_AbilityBase.CanActivate` (`local.Ability`)))
      (return _success))))

(fn `CanActivateAnyAbility`
  (returns (Success :type Boolean))
  (return (not (`self.IsAbilityActive`))))

(fn `EquipAbility`
  (params (Ability :type "/Game/Core/Blueprints/Gameplay/Components/AbilitySystemComponent/Structures/ST_AbilityEquipData Structure"))
  (`|ExecutionSequence`
    (:`then_0`
      (`self.UnequipAbility` (`.AbilitySlot_2_DDEB49C646145711E2A0BE940DD2A385` (break `/Game/Core/Blueprints/Gameplay/Components/AbilitySystemComponent/Structures/ST_AbilityEquipData` (`local.Ability`)))))
    (:`then_1`
      (bind _returnvalue (`|SpawnActorFromClass` (`.Ability_5_D058F5D84E451EB8B8186480F09DFC3F` (break `/Game/Core/Blueprints/Gameplay/Components/AbilitySystemComponent/Structures/ST_AbilityEquipData` (`local.Ability`))) (`KismetMathLibrary.MakeTransform` (0.0 0.0 0.0)) "AlwaysSpawn" "MultiplyWithRoot" (`self.GetOwner`) self null))
      (`KismetArrayLibrary.Array_Add` (`self.InstancedAbilities`) (make `/Game/Core/Blueprints/Gameplay/Components/AbilitySystemComponent/Structures/ST_AbilitySlotData` (`.AbilitySlot_2_DDEB49C646145711E2A0BE940DD2A385` (break `/Game/Core/Blueprints/Gameplay/Components/AbilitySystemComponent/Structures/ST_AbilityEquipData` (`local.Ability`))) _returnvalue))
      (set `self.InstancedAbilities` (`self.InstancedAbilities`))
      (`/Game/Core/Blueprints/Gameplay/Components/AbilitySystemComponent/BP_AbilityBase.SetCurrentCharges` _returnvalue (`.MaxCharges_11_1CC1C6C64FF6D41F8A00A7876D8A04CF` (break `/Game/Core/Blueprints/Gameplay/Components/AbilitySystemComponent/Structures/ST_AbilityData` (`/Game/Core/Blueprints/Gameplay/Components/AbilitySystemComponent/BP_AbilityBase.AbilityData` _returnvalue)))))))

(fn `GetAbilityBySlot`
  (params (SlotTag :type "GameplayTag Structure"))
  (returns (Ability :type "/Game/Core/Blueprints/Gameplay/Components/AbilitySystemComponent/BP_AbilityBase Object Reference"))
  (for _array_element (`self.InstancedAbilities`)
    (bind (_abilityslot _ability) (break `/Game/Core/Blueprints/Gameplay/Components/AbilitySystemComponent/Structures/ST_AbilitySlotData` _array_element))
    (if (== _abilityslot (`local.SlotTag`))
      (return _ability)))
  (return null))

(fn `GetAttributeComponent`
  (returns (AttributeComponent :type "/Game/Core/Blueprints/Gameplay/Components/AttributeComponent/BPC_AttributeComponent Object Reference"))
  (return (`self.AttributeComponent`)))

(fn `GetInstancedAbilities`
  (returns (InstancedAbilities :type "Array of /Game/Core/Blueprints/Gameplay/Components/AbilitySystemComponent/Structures/ST_AbilitySlotData Structure"))
  (return (`self.InstancedAbilities`)))

(fn `GetOwnerCharacter`
  (returns (OwnerCharacter :type "/Game/Core/Blueprints/Gameplay/Characters/BP_CharacterBase Object Reference"))
  (return (`self.OwnerCharacter`)))

(fn `HandleCooldown`
  (locals (Found :type Boolean) (AbilityTemp :type "/Game/Core/Blueprints/Gameplay/Components/AbilitySystemComponent/BP_AbilityBase Object Reference"))
  (bind _abilitytemp (`local.AbilityTemp`))
  (for _array_element (`self.InstancedAbilities`)
    (bind ((`Ability_6_D058F5D84E451EB8B8186480F09DFC3F` _ability)) (break `/Game/Core/Blueprints/Gameplay/Components/AbilitySystemComponent/Structures/ST_AbilitySlotData` _array_element))
    (set `local.AbilityTemp` _ability)
    (bind _remainingcooldown (`/Game/Core/Blueprints/Gameplay/Components/AbilitySystemComponent/BP_AbilityBase.GetRemainingCooldown` _ability))
    (if (> _remainingcooldown 0.0)
      (`/Game/Core/Blueprints/Gameplay/Components/AbilitySystemComponent/BP_AbilityBase.SetRemainingCooldown` _ability (`KismetMathLibrary.FMax` (- _remainingcooldown (`self.RefreshRate`))))
      (if (> _remainingcooldown 0.0)
        (set `local.Found` true)
        (else
          (`/Game/Core/Blueprints/Gameplay/Components/AbilitySystemComponent/BP_AbilityBase.SetCurrentCharges` (`local.AbilityTemp`) (+ (`/Game/Core/Blueprints/Gameplay/Components/AbilitySystemComponent/BP_AbilityBase.GetCurrentCharges` (`local.AbilityTemp`)) 1))
          (if (< (`/Game/Core/Blueprints/Gameplay/Components/AbilitySystemComponent/BP_AbilityBase.GetCurrentCharges` _abilitytemp) (`.MaxCharges_11_1CC1C6C64FF6D41F8A00A7876D8A04CF` (break `/Game/Core/Blueprints/Gameplay/Components/AbilitySystemComponent/Structures/ST_AbilityData` (`/Game/Core/Blueprints/Gameplay/Components/AbilitySystemComponent/BP_AbilityBase.AbilityData` _abilitytemp))))
            (`/Game/Core/Blueprints/Gameplay/Components/AbilitySystemComponent/BP_AbilityBase.SetRemainingCooldown` (`local.AbilityTemp`) (`.Cooldown_8_B32567E94CD6F3DFB8410AAB63AEA5D3` (break `/Game/Core/Blueprints/Gameplay/Components/AbilitySystemComponent/Structures/ST_AbilityData` (`/Game/Core/Blueprints/Gameplay/Components/AbilitySystemComponent/BP_AbilityBase.AbilityData` (`local.AbilityTemp`)))))
            (set `local.Found` true))))))
  (if (not (`local.Found`))
    (`KismetSystemLibrary.K2_ClearAndInvalidateTimerHandle` (`self.CooldownTimer`))))

(fn `Init`
  (`|ExecutionSequence`
    (:`then_0`
      (bind _asbp_character_base (cast `/Game/Core/Blueprints/Gameplay/Characters/BP_CharacterBase` (`self.GetOwner`)))
      (set `self.OwnerCharacter` _asbp_character_base)
      (set `self.AttributeComponent` (`Actor.GetComponentByClass` (`self.GetOwner`) "/Game/Core/Blueprints/Gameplay/Components/AttributeComponent/BPC_AttributeComponent.BPC_AttributeComponent_C")))
    (:`then_1`
      (`/Engine/EditorBlueprintResources/ActorComponentMacros.Switch Has Authority`
        (:`Authority`
          (for _array_element (`self.DefaultAbilities`)
            (`self.EquipAbility` _array_element)))))))

(fn `IsLocallyControlled`
  (returns (ReturnValue :type Boolean))
  (return (`Pawn.IsLocallyControlled` (`self.OwnerCharacter`))))

(fn `OnAbilityCommit`
  (params (Ability :type "/Game/Core/Blueprints/Gameplay/Components/AbilitySystemComponent/BP_AbilityBase Object Reference"))
  (remove `/Game/Core/Blueprints/Gameplay/Components/AbilitySystemComponent/BP_AbilityBase.OnAbilityCommit` Ability (`|CreateDelegate` :!event `OnAbilityCommit`))
  (if (> (`.Cooldown_8_B32567E94CD6F3DFB8410AAB63AEA5D3` (break `/Game/Core/Blueprints/Gameplay/Components/AbilitySystemComponent/Structures/ST_AbilityData` (`/Game/Core/Blueprints/Gameplay/Components/AbilitySystemComponent/BP_AbilityBase.AbilityData` (`local.Ability`)))) 0.0)
    (`/Game/Core/Blueprints/Gameplay/Components/AbilitySystemComponent/BP_AbilityBase.SetRemainingCooldown` (`local.Ability`) (`.Cooldown_8_B32567E94CD6F3DFB8410AAB63AEA5D3` (break `/Game/Core/Blueprints/Gameplay/Components/AbilitySystemComponent/Structures/ST_AbilityData` (`/Game/Core/Blueprints/Gameplay/Components/AbilitySystemComponent/BP_AbilityBase.AbilityData` (`local.Ability`)))))
    (`/Game/Core/Blueprints/Gameplay/Components/AbilitySystemComponent/BP_AbilityBase.SetCurrentCharges` (`local.Ability`) (- (`/Game/Core/Blueprints/Gameplay/Components/AbilitySystemComponent/BP_AbilityBase.GetCurrentCharges` (`local.Ability`)) 1))
    (if (not (`KismetSystemLibrary.K2_IsValidTimerHandle` (`self.CooldownTimer`)))
      (bind _returnvalue (`KismetSystemLibrary.K2_SetTimerDelegate` (`|CreateDelegate` :!event `HandleCooldown`) (`self.RefreshRate`) true))
      (set `self.CooldownTimer` _returnvalue))))

(fn `OnEndAbility`
  (params (Ability :type "/Game/Core/Blueprints/Gameplay/Components/AbilitySystemComponent/BP_AbilityBase Object Reference"))
  (`|ExecutionSequence`
    (:`then_0`
      (`local.Ability`
        (:`then`
          (remove `/Game/Core/Blueprints/Gameplay/Components/AbilitySystemComponent/BP_AbilityBase.OnEndAbility` (`local.Ability`) (`|CreateDelegate` :!event `OnEndAbility`))
          (remove `/Game/Core/Blueprints/Gameplay/Components/AbilitySystemComponent/BP_AbilityBase.OnAbilityCommit` (`local.Ability`) (`|CreateDelegate` :!event `OnAbilityCommit`)))
        (:`else`)))
    (:`then_1`
      (set `self.IsAbilityActive` false)
      (set `self.ActiveAbility` null)
      (`self.OnAbilityCompleted`))))

(fn `OnRep_InstancedAbilities`
  (`self.OnUpdatedInstancedAbilities` (`self.InstancedAbilities`)))

(fn `UnequipAbility`
  (params (AbilitySlot :type "GameplayTag Structure"))
  (locals (AbilityTemp :type "/Game/Core/Blueprints/Gameplay/Components/AbilitySystemComponent/BP_AbilityBase Object Reference"))
  (for (_array_element _array_index) (`self.InstancedAbilities`)
    (bind (_abilityslot _ability) (break `/Game/Core/Blueprints/Gameplay/Components/AbilitySystemComponent/Structures/ST_AbilitySlotData` _array_element))
    (if (== _abilityslot (`local.AbilitySlot`))
      (`|ExecutionSequence`
        (:`then_0`
          (`/Engine/EditorBlueprintResources/StandardMacros.IsValid` _ability
            (:`Is Valid`
              (set `local.AbilityTemp` _ability)
              (`|ExecutionSequence`
                (:`then_0`
                  (if (and (`self.IsAbilityActive`) (== (`self.ActiveAbility`) (`local.AbilityTemp`)))
                    (set `self.IsAbilityActive` false)
                    (set `self.ActiveAbility` null)
                    (`self.OnAbilityCompleted`)))
                (:`then_1`
                  (`Actor.K2_DestroyActor` (`local.AbilityTemp`))
                  (set `local.AbilityTemp` null))))))
        (:`then_1`
          (`KismetArrayLibrary.Array_Remove` (`self.InstancedAbilities`) _array_index)
          (set `self.InstancedAbilities` (`self.InstancedAbilities`)))
        (:`then_2`
          (return))))))