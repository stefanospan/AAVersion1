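; Tank role effect that grants a damage reduction aura to nearby teammates, excluding the tank itself.
; On activation it spawns an area actor attached to the owner, binds its overlap events and processes characters already inside.
; Same-team characters receive the aura effect through their effect component and are tracked in AffectedActors.
; Leaving the area removes the effect; deactivation destroys the area and runs end-overlap handling on tracked actors.
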(event `self.OnEffectActivated`
  (bind _returnvalue (`|SpawnActorFromClass` "/Game/Core/Blueprints/Gameplay/Roles/Roles/Tank/BP_TankDamageReductionAuraArea.BP_TankDamageReductionAuraArea_C" (`KismetMathLibrary.MakeTransform` (`self.K2_GetActorLocation` (`ActorComponent.GetOwner` (`self.GetRoleComponent`)))) "AlwaysSpawn" "MultiplyWithRoot" null null))
  (bind _output_get (set `self.AreaActor` _returnvalue))
  (`self.K2_AttachToActor` _output_get (`ActorComponent.GetOwner` (`self.GetRoleComponent`)) "None" "SnapToTarget" "KeepWorld" "KeepWorld" true)
  (add `self.OnActorBeginOverlap` (`self.AreaActor`) (`|CreateDelegate` :!event `OnAreaBeginOverlap`))
  (add `self.OnActorEndOverlap` (`self.AreaActor`) (`|CreateDelegate` :!event `OnAreaEndOverlap`))
  (`self.HandleInitOverlaps`))

(event `OnAreaBeginOverlap` :!signature `self.OnActorBeginOverlap`
  (params (OverlappedActor :type "Actor Object Reference") (OtherActor :type "Actor Object Reference"))
  (bind _ascharacter (cast `Character` OtherActor))
  (bind _team (message `/Game/Core/Blueprints/Gameplay/Components/TeamComponent/BPI_Teams.GetTeam` _ascharacter))
  (bind _team_2 (message `/Game/Core/Blueprints/Gameplay/Components/TeamComponent/BPI_Teams.GetTeam` (`ActorComponent.GetOwner` (`self.GetRoleComponent`))))
  (if (== _team_2 _team)
    (if (!= (`ActorComponent.GetOwner` (`self.GetRoleComponent`)) _ascharacter)
      (if (not (`KismetArrayLibrary.Array_Contains` (`self.AffectedActors`) _ascharacter))
        (bind _effectcomponent (message `/Game/Core/Blueprints/Gameplay/Components/EffectComponent/BPI_Effects.GetEffectComponent` _ascharacter))
        (`/Engine/EditorBlueprintResources/StandardMacros.IsValid` _effectcomponent
          (:`Is Valid`
            (bind _success (`/Game/Core/Blueprints/Gameplay/Components/EffectComponent/BPC_EffectComponent.ApplyEffect` _effectcomponent "/Game/Core/Blueprints/Gameplay/Roles/Roles/Tank/BP_Effect_Tank_DamageReductionAura.BP_Effect_Tank_DamageReductionAura_C" null))
            (if _success
              (`KismetArrayLibrary.Array_Add` (`self.AffectedActors`) _ascharacter))))))))

(event `OnAreaEndOverlap` :!signature `self.OnActorEndOverlap`
  (params (OverlappedActor :type "Actor Object Reference") (OtherActor :type "Actor Object Reference"))
  (bind _returnvalue (`KismetArrayLibrary.Array_RemoveItem` (`self.AffectedActors`) OtherActor))
  (if _returnvalue
    (bind _effectcomponent (message `/Game/Core/Blueprints/Gameplay/Components/EffectComponent/BPI_Effects.GetEffectComponent` OtherActor))
    (`/Engine/EditorBlueprintResources/StandardMacros.IsValid` _effectcomponent
      (:`Is Valid`
        (`/Game/Core/Blueprints/Gameplay/Components/EffectComponent/BPC_EffectComponent.RemoveEffectByClass` _effectcomponent "/Game/Core/Blueprints/Gameplay/Roles/Roles/Tank/BP_Effect_Tank_DamageReductionAura.BP_Effect_Tank_DamageReductionAura_C")))))

(event `self.OnEffectDeactivated`
  (`|ExecutionSequence`
    (:`then_0`
      (bind _areaactor (`self.AreaActor`)
        (:`then`
          (`self.K2_DestroyActor` _areaactor)
          (set `self.AreaActor` null))
        (:`else`)))
    (:`then_1`
      (for _array_element (`self.AffectedActors`)
        (`self.OnAreaEndOverlap` (`ActorComponent.GetOwner` (`self.GetRoleComponent`)) _array_element))
      (`KismetArrayLibrary.Array_Clear` (`self.AffectedActors`)))))

(fn `HandleInitOverlaps`
  (locals (OverlappingActors :type "Array of Character Object Reference"))
  (bind _output_get (set `local.OverlappingActors` (`self.GetOverlappingActors` (`self.AreaActor`) "/Script/Engine.Character")))
  (for _array_element _output_get
    (`self.OnAreaBeginOverlap` (`ActorComponent.GetOwner` (`self.GetRoleComponent`)) _array_element)))

(fn `UserConstructionScript`
  (`parent.UserConstructionScript`))