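; Healer role effect that gives the owner's teammates the HealerHeal effect.
; On activation it binds to the CharacterManager component on the GameState and processes the registered characters, repeating whenever that list updates.
; Each pass skips the owner, matches characters by team and applies BP_Effect_HealerHeal through their effect component, with no check for an existing application in this graph.
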(event `self.OnEffectActivated`
  (bind _output_get (set `self.CharacterManagerComponent` (`self.GetComponentByClass` (`GameplayStatics.GetGameState`) "/Game/Core/Blueprints/Gameplay/Components/CharacterManagerComponent/BPC_CharacterManagerComponent.BPC_CharacterManagerComponent_C")))
  (add `/Game/Core/Blueprints/Gameplay/Components/CharacterManagerComponent/BPC_CharacterManagerComponent.OnUpdatedRegisteredCharacters` _output_get (`|CreateDelegate` :!event `OnUpdatedRegisteredCharacters`))
  (`self.OnUpdatedRegisteredCharacters` (`/Game/Core/Blueprints/Gameplay/Components/CharacterManagerComponent/BPC_CharacterManagerComponent.GetRegisteredCharacters` _output_get)))

(event `OnUpdatedRegisteredCharacters`
  (params (RegisteredCharacters :type "Array of /Game/Core/Blueprints/Gameplay/Characters/BP_CharacterBase Object Reference (by ref)"))
  (bind _team (message `/Game/Core/Blueprints/Gameplay/Components/TeamComponent/BPI_Teams.GetTeam` (`ActorComponent.GetOwner` (`self.GetRoleComponent`))))
  (for _array_element RegisteredCharacters
    (if (!= _array_element (`ActorComponent.GetOwner` (`self.GetRoleComponent`)))
      (bind _team_2 (message `/Game/Core/Blueprints/Gameplay/Components/TeamComponent/BPI_Teams.GetTeam` _array_element))
      (if (== _team_2 _team)
        (bind _effectcomponent (message `/Game/Core/Blueprints/Gameplay/Components/EffectComponent/BPI_Effects.GetEffectComponent` _array_element))
        (`/Engine/EditorBlueprintResources/StandardMacros.IsValid` _effectcomponent
          (:`Is Valid`
            (`/Game/Core/Blueprints/Gameplay/Components/EffectComponent/BPC_EffectComponent.ApplyEffect` _effectcomponent "/Game/Core/Blueprints/Gameplay/Roles/Roles/Healer/BP_Effect_HealerHeal.BP_Effect_HealerHeal_C" null)))))))

(fn `UserConstructionScript`
  (`parent.UserConstructionScript`))