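; Healer role effect that gradually restores Health on the owner of its effect component.
; On application, a looping timer adds HealRate scaled by RefreshRate to the Health stat through the owner's stats component.
; The effect also binds to the owner's any-damage event, where taking damage replaces the heal timer with a short delay, apparently before healing restarts.
; Removing the effect clears the timer.
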(event `self.OnEffectApplied`
  (add `Actor.OnTakeAnyDamage` (`ActorComponent.GetOwner` (`self.GetEffectComponent`)) (`|CreateDelegate` :!event `OnReceiveDamage`))
  (`self.StartHeal`))

(event `StartHeal`
  (bind _returnvalue (`KismetSystemLibrary.K2_SetTimerDelegate` (`|CreateDelegate` :!event `Heal`) (`self.RefreshRate`) true))
  (set `self.HealTimer` _returnvalue))

(event `OnReceiveDamage`
  (params (DamagedActor :type "Actor Object Reference") (Damage :type "Float (single-precision)") (DamageType :type "DamageType Object Reference") (InstigatedBy :type "Controller Object Reference") (DamageCauser :type "Actor Object Reference"))
  (`KismetSystemLibrary.K2_ClearAndInvalidateTimerHandle` (`self.HealTimer`))
  (bind _returnvalue (`KismetSystemLibrary.K2_SetTimerDelegate` (`|CreateDelegate` :!event `StartHeal`) 3.0))
  (set `self.HealTimer` _returnvalue))

(event `Heal`
  (bind _statcomponent (message `/Game/Core/Blueprints/Gameplay/Components/StatComponent/BPI_Stats.GetStatsComponent` (`ActorComponent.GetOwner` (`self.GetEffectComponent`))))
  (`/Game/Core/Blueprints/Gameplay/Components/StatComponent/BPC_StatComponent.AddStat` _statcomponent (struct :`TagName` "Stat.Health") (* (`self.RefreshRate`) (`self.HealRate`))))

(event `self.OnEffectRemoved`
  (`KismetSystemLibrary.K2_ClearAndInvalidateTimerHandle` (`self.HealTimer`)))

(fn `UserConstructionScript`
  (`parent.UserConstructionScript`))