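; Actor component that gives its owner a gameplay role, defining its stats, attributes, abilities and persistent effects.
; On BeginPlay it caches the owner's stat, attribute and ability system components, then assigns the starting role with authority only.
; AssignRole pushes the role's data into those components and spawns each role effect as an owned actor, then activates it.
; EndPlay deactivates and destroys those effect actors on authority.
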(event `self.ReceiveBeginPlay`
  (`self.Init`))

(event `self.ReceiveEndPlay`
  (params (EndPlayReason :type "EEndPlayReason Enum" :default "Destroyed"))
  (`/Engine/EditorBlueprintResources/ActorComponentMacros.Switch Has Authority`
    (:`Authority`
      (for _array_element (`self.RoleEffects`)
        (`/Game/Core/Blueprints/Gameplay/Roles/BP_RoleEffectBase.OnEffectDeactivated` _array_element)
        (`Actor.K2_DestroyActor` _array_element))
      (`KismetArrayLibrary.Array_Clear` (`self.RoleEffects`)))))

(fn `AssignRole`
  (params (Role :type "/Game/Core/Blueprints/Gameplay/Roles/PDA_Role Object Reference"))
  (set `self.AssignedRole` Role)
  (`|ExecutionSequence`
    (:`then_0`
      (`/Game/Core/Blueprints/Gameplay/Components/StatComponent/BPC_StatComponent.SetStatDefinitions` (`self.StatComponent`) (`.Stats_14_9839A97F4E25F7441EB2B6AAC115ABE5` (break `/Game/Core/Blueprints/Gameplay/Roles/Structures/ST_RoleData` (`/Game/Core/Blueprints/Gameplay/Roles/PDA_Role.RoleData` (`self.AssignedRole`))))))
    (:`then_1`
      (`/Game/Core/Blueprints/Gameplay/Components/AttributeComponent/BPC_AttributeComponent.SetDefaultAttributes` (`self.AttributeComponent`) (`.Attributes_13_1506198043321B704392609BD86C05C8` (break `/Game/Core/Blueprints/Gameplay/Roles/Structures/ST_RoleData` (`/Game/Core/Blueprints/Gameplay/Roles/PDA_Role.RoleData` (`self.AssignedRole`))))))
    (:`then_2`
      (for _array_element (`.RoleAbilities_24_ECD01AEB4EC3B9C6891617B16105CB3E` (break `/Game/Core/Blueprints/Gameplay/Roles/Structures/ST_RoleData` (`/Game/Core/Blueprints/Gameplay/Roles/PDA_Role.RoleData` (`self.AssignedRole`))))
        (`/Game/Core/Blueprints/Gameplay/Components/AbilitySystemComponent/BPC_AbilitySystemComponent.EquipAbility` (`self.AbilitySystemComponent`) _array_element)))
    (:`then_3`
      (for _array_element_2 (`.RoleEffects_21_BF5C67F04D0C2669FC308EA4AEB2B905` (break `/Game/Core/Blueprints/Gameplay/Roles/Structures/ST_RoleData` (`/Game/Core/Blueprints/Gameplay/Roles/PDA_Role.RoleData` (`self.AssignedRole`))))
        (bind _returnvalue (`|SpawnActorFromClass` _array_element_2 (`KismetMathLibrary.MakeTransform` (0.0 0.0 0.0)) "AlwaysSpawn" "MultiplyWithRoot" (`self.GetOwner`) self null))
        (`KismetArrayLibrary.Array_Add` (`self.RoleEffects`) _returnvalue)
        (`/Game/Core/Blueprints/Gameplay/Roles/BP_RoleEffectBase.OnEffectActivated` _returnvalue)))))

(fn `GetAssignedRole`
  (returns (AssignedRole :type "/Game/Core/Blueprints/Gameplay/Roles/PDA_Role Object Reference"))
  (return (`self.AssignedRole`)))

(fn `Init`
  (`|ExecutionSequence`
    (:`then_0`
      (set `self.StatComponent` (`Actor.GetComponentByClass` (`self.GetOwner`) "/Game/Core/Blueprints/Gameplay/Components/StatComponent/BPC_StatComponent.BPC_StatComponent_C"))
      (set `self.AttributeComponent` (`Actor.GetComponentByClass` (`self.GetOwner`) "/Game/Core/Blueprints/Gameplay/Components/AttributeComponent/BPC_AttributeComponent.BPC_AttributeComponent_C"))
      (set `self.AbilitySystemComponent` (`Actor.GetComponentByClass` (`self.GetOwner`) "/Game/Core/Blueprints/Gameplay/Components/AbilitySystemComponent/BPC_AbilitySystemComponent.BPC_AbilitySystemComponent_C")))
    (:`then_1`
      (`/Engine/EditorBlueprintResources/ActorComponentMacros.Switch Has Authority`
        (:`Authority`
          (bind _startingrole (`self.StartingRole`)
            (:`then`
              (`self.AssignRole` _startingrole))
            (:`else`)))))))