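; BP_ResourceBase is a base resource actor that drops an item pickup when it dies.
; On the stat component's server death event, it spawns a BP_PickupBase carrying its resource item and amount, then destroys itself.
; The spawn point is randomly offset horizontally, then dropped to the surface by a vertical Visibility trace and raised slightly, falling back to the trace end on a miss.
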(event `self.BPC_StatComponent.ServerOnDeath`
  (params (KillerActor :type "Actor Object Reference"))
  (`|SpawnActorFromClass` "/Game/Core/Blueprints/Gameplay/Pickups/BP_PickupBase.BP_PickupBase_C" (`KismetMathLibrary.MakeTransform` (`self.GetPickupSpawnLocation`)) "AlwaysSpawn" "MultiplyWithRoot" null (`self.ResourceItem`) (`self.Amount`) null)
  (`self.K2_DestroyActor`))

(fn `GetPickupSpawnLocation`
  (returns (Location :type "Vector Structure"))
  (locals (LocationTemp :type "Vector Structure"))
  (bind _returnvalue (`KismetMathLibrary.RandomFloatInRange` -50.0 50.0))
  (bind _output_get (set `local.LocationTemp` (+ (`self.K2_GetActorLocation`) (`KismetMathLibrary.MakeVector` _returnvalue _returnvalue))))
  (bind _outhit (`KismetSystemLibrary.LineTraceSingle` (+ _output_get (0.0 0.0 250.0)) (- _output_get (0.0 0.0 500.0)) "TraceTypeQuery1"))
  (bind (_bblockinghit _binitialoverlap _time _distance _location _impactpoint _normal _impactnormal _physmat _hitactor _hitcomponent _hitbonename _bonename _hititem _elementindex _faceindex _tracestart _traceend) (`GameplayStatics.BreakHitResult` _outhit))
  (return (+ (select `bool` _bblockinghit :`false` _traceend :`true` _location) (0.0 0.0 50.0))))

(fn `UserConstructionScript`)