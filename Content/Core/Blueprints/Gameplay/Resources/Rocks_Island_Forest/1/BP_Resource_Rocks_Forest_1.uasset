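; Blueprint for a forest-island rock resource that gives audio feedback when hit and when destroyed.
; Damage received through its stat component plays a quiet, higher-pitched stone impact sound at the resource mesh location.
; Destruction plays a stone-breaking sound at the same location.
; The construction script only calls the parent, and the BeginPlay, overlap and Tick events are disabled stubs.
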(event `self.BPC_StatComponent.OnReceivedDamage`
  (`GameplayStatics.PlaySoundAtLocation` "/Game/Game_Item/Destruction/Cue/Impact_Stone_04.Impact_Stone_04" (`SceneComponent.K2_GetComponentLocation` (`self.ResourceMesh`)) (struct) 0.3 1.5 0.0 null null null null))

(event `self.ReceiveDestroyed`
  (`GameplayStatics.PlaySoundAtLocation` "/Game/Magic_Spell_SFX_Pack_Vol1/Additional_and_Loops/cue/Destroyed_stone_01.Destroyed_stone_01" (`SceneComponent.K2_GetComponentLocation` (`self.ResourceMesh`)) (struct) 1.0 1.0 0.0 null null null null))

(fn `UserConstructionScript`
  (`parent.UserConstructionScript`))