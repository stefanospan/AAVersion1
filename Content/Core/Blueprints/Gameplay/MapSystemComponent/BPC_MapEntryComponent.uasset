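; Actor component that registers itself as an entry with the map system.
; On BeginPlay it retries on a short delay until the GameState is valid, then registers with the GameState's BPC_MapSystemComponent.
; On EndPlay it unregisters from that same component.
; UpdatePosition broadcasts the OnUpdatePosition dispatcher with itself as payload so listeners can react to position changes.
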(event `self.ReceiveBeginPlay`
  (bind _returnvalue (`GameplayStatics.GetGameState`))
  (`/Engine/EditorBlueprintResources/StandardMacros.IsValid` _returnvalue :!label _label
    (:`Is Valid`
      (`/Game/Core/Blueprints/Gameplay/MapSystemComponent/BPC_MapSystemComponent.RegisterMapEntryComponent` (`Actor.GetComponentByClass` _returnvalue "/Game/Core/Blueprints/Gameplay/MapSystemComponent/BPC_MapSystemComponent.BPC_MapSystemComponent_C") self))
    (:`Is Not Valid`
      (`KismetSystemLibrary.Delay` 0.1)
      (goto _label))))

(event `self.ReceiveEndPlay`
  (params (EndPlayReason :type "EEndPlayReason Enum" :default "Destroyed"))
  (`/Game/Core/Blueprints/Gameplay/MapSystemComponent/BPC_MapSystemComponent.UnregisterMapEntryComponent` (`Actor.GetComponentByClass` (`GameplayStatics.GetGameState`) "/Game/Core/Blueprints/Gameplay/MapSystemComponent/BPC_MapSystemComponent.BPC_MapSystemComponent_C") self))

(fn `UpdatePosition`
  (`self.OnUpdatePosition` self))