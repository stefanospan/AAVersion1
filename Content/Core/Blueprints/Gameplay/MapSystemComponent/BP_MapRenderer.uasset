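; BP_MapRenderer is an actor that captures a map image of the area between two marker actors, MapPoint1 and MapPoint2.
; Its construction script centers it between the markers at a fixed high altitude and sets the scene capture's ortho width to their X distance.
; AlignPoints moves MapPoint2 along Y so its Y offset from MapPoint1 equals the X offset, squaring the area.
; CaptureScene triggers the capture on demand.
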(fn `AlignPoints`
  (bind _x (.x (`self.K2_GetActorLocation` (`self.MapPoint2`))))
  (`self.K2_SetActorLocation` (`self.MapPoint2`) (`KismetMathLibrary.MakeVector` _x (+ (- _x (.x (`self.K2_GetActorLocation` (`self.MapPoint1`)))) (.y (`self.K2_GetActorLocation` (`self.MapPoint1`)))) (.z (`self.K2_GetActorLocation` (`self.MapPoint2`)))) false false))

(fn `CaptureScene`
  (`SceneCaptureComponent2D.CaptureScene` (`self.SceneCaptureComponent2D`)))

(fn `UserConstructionScript`
  (bind _mappoint1 (`self.MapPoint1`)
    (:`then`
      (bind _mappoint2 (`self.MapPoint2`)
        (:`then`
          (bind _returnvalue (`self.K2_GetActorLocation` _mappoint1))
          (bind _returnvalue_2 (- (`self.K2_GetActorLocation` _mappoint2) _returnvalue))
          (`self.K2_SetActorLocation` (`KismetMathLibrary.MakeVector` (.x (+ (/ _returnvalue_2 2.0) _returnvalue)) (.y (+ (/ _returnvalue_2 2.0) _returnvalue)) 50000.0))
          (set `SceneCaptureComponent2D.OrthoWidth` (`KismetMathLibrary.Abs` (.x _returnvalue_2)) (`self.SceneCaptureComponent2D`)))
        (:`else`)))
    (:`else`)))