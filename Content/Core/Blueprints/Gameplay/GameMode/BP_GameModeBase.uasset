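; Base game mode for team elimination matches, running from player join to the return to the lobby.
; On login it applies team and character from GameInstance transition data, with a default fallback, then spawns pawns at unused team starts, or as spectators.
; A GameState timer component holds input until countdown ends.
; Deaths spawn team-restricted spectators; one surviving team triggers win/lose screens and server travel, while empty dedicated servers shut down.
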(event `self.ReceiveBeginPlay`
  (`KismetSystemLibrary.Delay` 0.0)
  (`self.Init`))

(event `self.K2_PostLogin`
  (params (NewPlayer :type "PlayerController Object Reference"))
  (`self.Init`)
  (bind _asbp_player_controller_base (cast `/Game/Core/Blueprints/Gameplay/GameMode/BP_PlayerControllerBase` NewPlayer))
  (bind (_success _transitiondata) (`self.ValidatePC` _asbp_player_controller_base))
  (if _success
    (`KismetArrayLibrary.Array_Add` (`self.PCs`) _asbp_player_controller_base)
    (bind _asbp_player_state_base (cast `/Game/Core/Blueprints/Gameplay/GameMode/BP_PlayerStateBase` (`Controller.PlayerState` _asbp_player_controller_base)))
    (bind ((`Character_5_4E528BF240C93B0D374764B5370A201F` _character) (`Team_8_C4244EDF4A3C7CC7854FFA95488B1996` _team)) (break `/Game/Core/Blueprints/Lobby/GameMode/Structures/ST_PlayerTransitionData` _transitiondata))
    (`/Game/Core/Blueprints/Gameplay/Components/TeamComponent/BPC_TeamComponent.SetTeam` (`/Game/Core/Blueprints/Gameplay/GameMode/BP_PlayerStateBase.BPC_TeamComponent` _asbp_player_state_base) _team)
    (`/Game/Core/Blueprints/Gameplay/GameMode/BP_PlayerControllerBase.SetSelectedCharacter` _asbp_player_controller_base _character)
    (`self.SpawnPC` _asbp_player_controller_base)
    (bind _asbp_player_state_base_2 (cast `/Game/Core/Blueprints/Gameplay/GameMode/BP_PlayerStateBase` (`Controller.PlayerState` _asbp_player_controller_base)))
    (`/Game/Core/Blueprints/Gameplay/GameMode/BP_GameStateBase.RegisterPlayerState` (`self.GetGameState`) _asbp_player_state_base_2)))

(event `self.K2_OnLogout`
  (params (ExitingController :type "Controller Object Reference"))
  (bind _asbp_player_controller_base (cast `/Game/Core/Blueprints/Gameplay/GameMode/BP_PlayerControllerBase` ExitingController))
  (`KismetArrayLibrary.Array_RemoveItem` (`self.PCs`) _asbp_player_controller_base)
  (bind _asbp_player_state_base (cast `/Game/Core/Blueprints/Gameplay/GameMode/BP_PlayerStateBase` (`Controller.PlayerState` _asbp_player_controller_base)))
  (`/Game/Core/Blueprints/Gameplay/GameMode/BP_GameStateBase.UnregisterPlayerState` (`self.GetGameState`) _asbp_player_state_base)
  (if (and (== (`KismetArrayLibrary.Array_Length` (`self.PCs`)) 0) (`KismetSystemLibrary.IsDedicatedServer`) (not (`self.IsServerTravel`)))
    (`self.ShutdownServer`)))

(event `SpawnPC`
  (params (PC :type "/Game/Core/Blueprints/Gameplay/GameMode/BP_PlayerControllerBase Object Reference"))
  (bind _team (message `/Game/Core/Blueprints/Gameplay/Components/TeamComponent/BPI_Teams.GetTeam` PC))
  (bind _playerstart (`self.GetRandomPlayerStart` _team))
  (`KismetArrayLibrary.Array_Add` (`self.UsedPlayerStarts`) _playerstart)
  (bind _returnvalue (`|SpawnActorFromClass` (`self.GetPawnClassForPC` PC) (`self.GetTransform` _playerstart) "AdjustIfPossibleButAlwaysSpawn" "MultiplyWithRoot" null null))
  (`Controller.Possess` PC _returnvalue)
  (bind _asbp_player_character_base (cast `/Game/Core/Blueprints/Gameplay/Characters/PlayerCharacters/BP_PlayerCharacterBase` _returnvalue))
  (add `/Game/Core/Blueprints/Gameplay/Characters/PlayerCharacters/BP_PlayerCharacterBase.OnDeath` _asbp_player_character_base (`|CreateDelegate` :!event `OnPlayerDeath`))
  (if (not (`self.IsInCountdown`))
    (`/Game/Core/Blueprints/Gameplay/Characters/PlayerCharacters/BP_PlayerCharacterBase.SetIsInputSuspended` _asbp_player_character_base false)))

(event `StartCountdown`
  (bind _bpc_timercomponent (`/Game/Core/Blueprints/Gameplay/GameMode/BP_GameStateBase.BPC_TimerComponent` (`self.GetGameState`)))
  (set `self.IsInCountdown` true)
  (add `/Game/Core/Blueprints/Gameplay/Components/TimerComponent/BPC_TimerComponent.OnTimerCompleted` _bpc_timercomponent (`|CreateDelegate` :!event `OnCountdownTimerCompleted`))
  (`/Game/Core/Blueprints/Gameplay/Components/TimerComponent/BPC_TimerComponent.StartTimer` _bpc_timercomponent (`self.CountdownTime`)))

(event `OnCountdownTimerCompleted`
  (remove `/Game/Core/Blueprints/Gameplay/Components/TimerComponent/BPC_TimerComponent.OnTimerCompleted` (`/Game/Core/Blueprints/Gameplay/GameMode/BP_GameStateBase.BPC_TimerComponent` (`self.GetGameState`)) (`|CreateDelegate` :!event `OnCountdownTimerCompleted`))
  (set `self.IsInCountdown` false)
  (for _array_element (`self.PCs`)
    (bind _asbp_player_character_base (cast `/Game/Core/Blueprints/Gameplay/Characters/PlayerCharacters/BP_PlayerCharacterBase` (`Controller.K2_GetPawn` _array_element)))
    (`/Game/Core/Blueprints/Gameplay/Characters/PlayerCharacters/BP_PlayerCharacterBase.SetIsInputSuspended` _asbp_player_character_base false)))

(event `OnPlayerDeath`
  (params (PlayerCharacter :type "/Game/Core/Blueprints/Gameplay/Characters/PlayerCharacters/BP_PlayerCharacterBase Object Reference"))
  (remove `/Game/Core/Blueprints/Gameplay/Characters/PlayerCharacters/BP_PlayerCharacterBase.OnDeath` PlayerCharacter (`|CreateDelegate` :!event `OnPlayerDeath`))
  (bind _asbp_player_controller_base (cast `/Game/Core/Blueprints/Gameplay/GameMode/BP_PlayerControllerBase` (`Pawn.GetController` PlayerCharacter)))
  (`self.K2_DestroyActor` PlayerCharacter)
  (`self.SpawnSpectator` _asbp_player_controller_base)
  (bind (_success _team) (`self.CheckGameEnded`))
  (if _success
    (`self.EndGame` _team)
    (else
      (`/Game/Core/Blueprints/Gameplay/GameMode/BP_PlayerControllerBase.ClientShowLoseScreen` _asbp_player_controller_base))))

(event `EndGame`
  (params (TeamWon :type Integer))
  (for _array_element (`self.PCs`)
    (bind _team (message `/Game/Core/Blueprints/Gameplay/Components/TeamComponent/BPI_Teams.GetTeam` _array_element))
    (if (== _team TeamWon)
      (`/Game/Core/Blueprints/Gameplay/GameMode/BP_PlayerControllerBase.ClientShowWinScreen` _array_element)
      (else
        (`/Game/Core/Blueprints/Gameplay/GameMode/BP_PlayerControllerBase.ClientShowLoseScreen` _array_element))))
  (`KismetSystemLibrary.Delay` 8.0)
  (set `self.IsServerTravel` true)
  (`KismetSystemLibrary.ExecuteConsoleCommand` "servertravel LobbyMap_P" null))

(event `SpawnSpectator`
  (params (PC :type "/Game/Core/Blueprints/Gameplay/GameMode/BP_PlayerControllerBase Object Reference"))
  (bind _team (message `/Game/Core/Blueprints/Gameplay/Components/TeamComponent/BPI_Teams.GetTeam` PC))
  (bind _returnvalue (`|SpawnActorFromClass` "/Game/Core/Blueprints/Gameplay/GameMode/BP_SpectatorPawn.BP_SpectatorPawn_C" (`KismetMathLibrary.MakeTransform` (0.0 0.0 0.0)) "AlwaysSpawn" "MultiplyWithRoot" null _team null))
  (`Controller.Possess` PC _returnvalue))

(fn `CheckGameEnded`
  (returns (Success :type Boolean) (Team :type Integer))
  (locals (TeamFound :type Integer :default -1))
  (for _array_element (`self.PCs`)
    (bind _returnvalue (`Controller.K2_GetPawn` _array_element))
    (`/Engine/EditorBlueprintResources/StandardMacros.IsValid` _returnvalue
      (:`Is Valid`
        (bind _success (message `/Game/Core/Blueprints/Gameplay/Components/StatComponent/BPI_Stats.IsAlive` _returnvalue))
        (if _success
          (bind _team (message `/Game/Core/Blueprints/Gameplay/Components/TeamComponent/BPI_Teams.GetTeam` _returnvalue))
          (if (== (`local.TeamFound`) -1)
            (set `local.TeamFound` _team)
            (elif (not (== _team (`local.TeamFound`)))
              (return false -1)))))))
  (return true (`local.TeamFound`)))

(fn `GetGameState`
  (returns (GameState :type "/Game/Core/Blueprints/Gameplay/GameMode/BP_GameStateBase Object Reference"))
  (bind _gamestateref (`self.GameStateRef`)
    (:`then`
      (return _gamestateref))
    (:`else`
      (bind _asbp_game_state_base (cast `/Game/Core/Blueprints/Gameplay/GameMode/BP_GameStateBase` (`GameplayStatics.GetGameState`)))
      (bind _output_get (set `self.GameStateRef` _asbp_game_state_base))
      (return _output_get))))

(fn `GetPawnClassForPC`
  (params (PC :type "/Game/Core/Blueprints/Gameplay/GameMode/BP_PlayerControllerBase Object Reference"))
  (returns (PawnClass :type "Pawn Class Reference"))
  (bind _team (message `/Game/Core/Blueprints/Gameplay/Components/TeamComponent/BPI_Teams.GetTeam` PC))
  (if (== _team 2)
    (return "/Game/Core/Blueprints/Gameplay/GameMode/BP_SpectatorPawn.BP_SpectatorPawn_C")
    (else
      (return (`/Game/Core/Blueprints/Gameplay/GameMode/BP_PlayerControllerBase.GetSelectedCharacter` PC)))))

(fn `GetPCs`
  (returns (PCs :type "Array of /Game/Core/Blueprints/Gameplay/GameMode/BP_PlayerControllerBase Object Reference"))
  (return (`self.PCs`)))

(fn `GetRandomPlayerStart`
  (params (Team :type Integer))
  (returns (PlayerStart :type "/Game/Core/Blueprints/Gameplay/GameMode/BP_PlayerStart Object Reference (by ref)"))
  (locals (AvailablePlayerStarts :type "Array of /Game/Core/Blueprints/Gameplay/GameMode/BP_PlayerStart Object Reference"))
  (for _array_element (`self.PlayerStart`)
    (if (== (`/Game/Core/Blueprints/Gameplay/GameMode/BP_PlayerStart.Team` _array_element) (`local.Team`))
      (if (not (`KismetArrayLibrary.Array_Contains` (`self.UsedPlayerStarts`) _array_element))
        (`KismetArrayLibrary.Array_Add` (`local.AvailablePlayerStarts`) _array_element))))
  (return (`KismetArrayLibrary.Array_Random` (`local.AvailablePlayerStarts`))))

(fn `Init`
  (`|ExecutionSequence`
    (:`then_0`
      (bind _asbp_game_instance (cast `/Game/Core/Blueprints/GameInstance/BP_GameInstance` (`GameplayStatics.GetGameInstance`)))
      (set `self.PlayerTransitionData` (`/Game/Core/Blueprints/GameInstance/BP_GameInstance.PlayerTransitionData` _asbp_game_instance))
      (`/Game/Core/Blueprints/Gameplay/GameMode/BP_GameStateBase.SetSelectedIsland` (`self.GetGameState`) (`/Game/Core/Blueprints/GameInstance/BP_GameInstance.SelectedIsland` _asbp_game_instance)))
    (:`then_1`
      (bind _outactors (`GameplayStatics.GetAllActorsOfClass` "/Game/Core/Blueprints/Gameplay/GameMode/BP_PlayerStart.BP_PlayerStart_C"))
      (set `self.PlayerStart` _outactors))
    (:`then_2`
      (`self.StartCountdown`))))

(fn `UserConstructionScript`)

(fn `ValidatePC`
  (params (PlayerController :type "/Game/Core/Blueprints/Gameplay/GameMode/BP_PlayerControllerBase Object Reference"))
  (returns (Success :type Boolean) (TransitionData :type "/Game/Core/Blueprints/Lobby/GameMode/Structures/ST_PlayerTransitionData Structure"))
  (for _array_element (`self.PlayerTransitionData`)
    (if (== (`GameplayStatics.GetPlayerStateFromUniqueNetId` (`.UniqueNetId_2_59F1991C4AB4F27A75158BB51FC68F7A` (break `/Game/Core/Blueprints/Lobby/GameMode/Structures/ST_PlayerTransitionData` _array_element))) (`Controller.PlayerState` (`local.PlayerController`)))
      (return true _array_element)))
  (return true (make `/Game/Core/Blueprints/Lobby/GameMode/Structures/ST_PlayerTransitionData` "INVALID" "/Game/Core/Blueprints/Gameplay/Characters/PlayerCharacters/Sigrun/BP_PlayerCharacter_Sigrun.BP_PlayerCharacter_Sigrun_C")))