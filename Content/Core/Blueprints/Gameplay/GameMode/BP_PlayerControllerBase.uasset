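; Base player controller that sets up local game input and acts as the network entry point for player actions.
; Server events forward inventory, equipment and item-use requests to their components.
; Shop purchases and teleports check and deduct Rune Fragments from the PlayerState before granting the item or moving the pawn.
; It also relays damage text to the HUD, broadcasts selected-character changes through a RepNotify and reads team from the PlayerState.
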(event `self.ReceiveBeginPlay`
  (`self.Init`))

(event `ClientShowDamageText`
  (params (Damage :type "Float (double-precision)") (Actor :type "Actor Object Reference"))
  (bind _asbp_hudbase (cast `/Game/Core/Blueprints/Gameplay/GameMode/BP_HUDBase` (`self.GetHUD`)))
  (`/Game/Core/Blueprints/Gameplay/GameMode/BP_HUDBase.ShowDamageText` _asbp_hudbase Damage Actor))

(event `ServerInventoryDropFromInventory`
  (params (FromInventoryComponent :type "/Game/Core/Blueprints/Gameplay/Components/InventoryComponent/BPC_InventoryComponent Object Reference") (FromSlotIndex :type Integer) (ToInventoryComponent :type "/Game/Core/Blueprints/Gameplay/Components/InventoryComponent/BPC_InventoryComponent Object Reference") (ToSlotIndex :type Integer))
  (`/Game/Core/Blueprints/Gameplay/Components/InventoryComponent/BPC_InventoryComponent.DropFromInventory` ToInventoryComponent FromInventoryComponent FromSlotIndex ToSlotIndex))

(event `ServerEquipmentEquipFromInventory`
  (params (FromInventoryComponent :type "/Game/Core/Blueprints/Gameplay/Components/InventoryComponent/BPC_InventoryComponent Object Reference") (FromSlotIndex :type Integer) (ToEquipmentComponent :type "/Game/Core/Blueprints/Gameplay/Components/EquipmentComponent/BPC_EquipmentComponent Object Reference") (ToEquipmentSlot :type "/Game/Core/Blueprints/Gameplay/Components/EquipmentComponent/Enums/E_EquipmentSlots Enum" :default "NewEnumerator0"))
  (`/Game/Core/Blueprints/Gameplay/Components/EquipmentComponent/BPC_EquipmentComponent.EquipFromInventory` ToEquipmentComponent FromInventoryComponent FromSlotIndex ToEquipmentSlot))

(event `ServerInventoryDropFromEquipment`
  (params (FromEquipmentComponent :type "/Game/Core/Blueprints/Gameplay/Components/EquipmentComponent/BPC_EquipmentComponent Object Reference") (FromEquipmentSlot :type "/Game/Core/Blueprints/Gameplay/Components/EquipmentComponent/Enums/E_EquipmentSlots Enum" :default "NewEnumerator0") (ToInventoryComponent :type "/Game/Core/Blueprints/Gameplay/Components/InventoryComponent/BPC_InventoryComponent Object Reference") (ToSlotIndex :type Integer))
  (`/Game/Core/Blueprints/Gameplay/Components/InventoryComponent/BPC_InventoryComponent.DropFromEquipment` ToInventoryComponent FromEquipmentComponent FromEquipmentSlot ToSlotIndex))

(event `ServerBuyShopkeeper`
  (params (Shopkeeper :type "/Game/Core/Blueprints/Gameplay/Characters/Shopkeeper/BP_Shopkeeper Object Reference") (ItemIndex :type Integer))
  (bind (_item _price) (break `/Game/Core/Blueprints/Gameplay/Characters/Shopkeeper/Structures/ST_ShopkeeperItemData` (`|GetArrayItem` (`/Game/Core/Blueprints/Gameplay/Characters/Shopkeeper/BP_Shopkeeper.GetShopkeeperItems` Shopkeeper) ItemIndex)))
  (if (>= (`/Game/Core/Blueprints/Gameplay/Components/RuneFragmentsComponent/BPC_RuneFragmentsComponent.GetCurrentRuneFragments` (`self.GetComponentByClass` (`self.PlayerState`) "/Game/Core/Blueprints/Gameplay/Components/RuneFragmentsComponent/BPC_RuneFragmentsComponent.BPC_RuneFragmentsComponent_C")) _price)
    (`/Game/Core/Blueprints/Gameplay/Components/RuneFragmentsComponent/BPC_RuneFragmentsComponent.RemoveRuneFragments` (`self.GetComponentByClass` (`self.PlayerState`) "/Game/Core/Blueprints/Gameplay/Components/RuneFragmentsComponent/BPC_RuneFragmentsComponent.BPC_RuneFragmentsComponent_C") _price)
    (`/Game/Core/Blueprints/Gameplay/Components/InventoryComponent/BPC_InventoryComponent.AddItem` (`self.GetComponentByClass` (`self.K2_GetPawn`) "/Game/Core/Blueprints/Gameplay/Components/InventoryComponent/BPC_InventoryComponent.BPC_InventoryComponent_C") _item 1)))

(event `ServerUseItem`
  (params (InventoryComponent :type "/Game/Core/Blueprints/Gameplay/Components/InventoryComponent/BPC_InventoryComponent Object Reference") (SlotIndex :type Integer))
  (`/Game/Core/Blueprints/Gameplay/Components/InventoryComponent/BPC_InventoryComponent.UseItem` InventoryComponent SlotIndex))

(event `ServerTeleport`
  (params (TeleportPoint :type "/Game/Core/Blueprints/Gameplay/Components/WeaponSystemComponent/Weapons/Portal/BP_TeleportPoint Object Reference"))
  (bind (_returnvalue_location _returnvalue_rotation) (`KismetMathLibrary.BreakTransform` (`self.GetTransform` TeleportPoint)))
  (bind _runefragmentscomponent (message `/Game/Core/Blueprints/Gameplay/Components/RuneFragmentsComponent/BPI_RuneFragments.GetRuneFragmentsComponent` (`self.PlayerState`)))
  (if (>= (`/Game/Core/Blueprints/Gameplay/Components/RuneFragmentsComponent/BPC_RuneFragmentsComponent.GetCurrentRuneFragments` _runefragmentscomponent) 25)
    (`/Game/Core/Blueprints/Gameplay/Components/RuneFragmentsComponent/BPC_RuneFragmentsComponent.RemoveRuneFragments` _runefragmentscomponent 25)
    (`self.K2_TeleportTo` (`self.K2_GetPawn`) _returnvalue_location _returnvalue_rotation)))

(fn `GetSelectedCharacter`
  (returns (SelectedCharacter :type "/Game/Core/Blueprints/Gameplay/Characters/PlayerCharacters/BP_PlayerCharacterBase Class Reference"))
  (return (`self.SelectedCharacter`)))

(fn `GetTeam`
  (returns (Team :type Integer))
  (bind _team (message `/Game/Core/Blueprints/Gameplay/Components/TeamComponent/BPI_Teams.GetTeam` (`self.PlayerState`)))
  (return _team))

(fn `Init`
  (`|ExecutionSequence`
    (:`then_0`
      (if (`self.IsLocalPlayerController`)
        (`WidgetBlueprintLibrary.SetInputMode_GameOnly` self)
        (set `self.bShowMouseCursor` false)
        (`EnhancedInputSubsystemInterface.AddMappingContext` (subsystem `EnhancedInputLocalPlayerSubsystem`) "/Game/Core/Inputs/IMC_DefaultInputs.IMC_DefaultInputs" 0 (struct))
        (`WidgetBlueprintLibrary.SetFocusToGameViewport`)))))

(fn `OnRep_SelectedCharacter`
  (`self.OnUpdatedSelectedCharacter` (`self.SelectedCharacter`)))

(fn `SetSelectedCharacter`
  (params (SelectedCharacter :type "/Game/Core/Blueprints/Gameplay/Characters/PlayerCharacters/BP_PlayerCharacterBase Class Reference"))
  (set `self.SelectedCharacter` SelectedCharacter))

(fn `UserConstructionScript`)