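; Base game state that holds the selected island and registered player states, and announces wave-system boss spawns.
; RepNotify handlers pass island and player-state changes on through update calls.
; Register and unregister functions reassign the array after editing it so its notify fires.
; When the wave component spawns a boss, the server has every player controller from the game mode play a client boss message.
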(event `self.BPC_WaveSystemComponent.OnBossSpawned`
  (`/Engine/EditorBlueprintResources/ActorMacros.Switch Has Authority`
    (:`Authority`
      (bind _asbp_game_mode_base (cast `/Game/Core/Blueprints/Gameplay/GameMode/BP_GameModeBase` (`GameplayStatics.GetGameMode`)))
      (for _array_element (`/Game/Core/Blueprints/Gameplay/GameMode/BP_GameModeBase.GetPCs` _asbp_game_mode_base)
        (`/Game/Core/Blueprints/Gameplay/GameMode/BP_PlayerControllerBase.ClientPlayBossMessage` _array_element)))))

(fn `GetPlayerStates`
  (returns (PlayerStates :type "Array of /Game/Core/Blueprints/Gameplay/GameMode/BP_PlayerStateBase Object Reference"))
  (return (`self.PlayerStates`)))

(fn `GetSelectedIsland`
  (returns (SelectedIsland :type "/Game/Core/Blueprints/Gameplay/Islands/PDA_IslandBase Object Reference"))
  (return (`self.SelectedIsland`)))

(fn `OnRep_PlayerStates`
  (`self.OnUpdatedPlayerStates` (`self.PlayerStates`)))

(fn `OnRep_SelectedIsland`
  (`self.OnUpdatedSelectedIsland` (`self.SelectedIsland`)))

(fn `RegisterPlayerState`
  (params (PlayerState :type "/Game/Core/Blueprints/Gameplay/GameMode/BP_PlayerStateBase Object Reference"))
  (`KismetArrayLibrary.Array_Add` (`self.PlayerStates`) (`local.PlayerState`))
  (set `self.PlayerStates` (`self.PlayerStates`)))

(fn `SetSelectedIsland`
  (params (SelectedIsland :type "/Game/Core/Blueprints/Gameplay/Islands/PDA_IslandBase Object Reference"))
  (set `self.SelectedIsland` SelectedIsland))

(fn `UnregisterPlayerState`
  (params (PlayerState :type "/Game/Core/Blueprints/Gameplay/GameMode/BP_PlayerStateBase Object Reference"))
  (`KismetArrayLibrary.Array_RemoveItem` (`self.PlayerStates`) (`local.PlayerState`))
  (set `self.PlayerStates` (`self.PlayerStates`)))

(fn `UserConstructionScript`)