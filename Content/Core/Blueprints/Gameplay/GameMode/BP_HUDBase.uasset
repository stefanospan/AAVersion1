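; Base HUD that creates the in-game HUD widget for the player character and controls its inventory, shopkeeper, full map and portal map panels.
; Set and toggle events drive panel visibility, with inventory, shop and portal changes switching input mode and cursor, and shopkeeper changes playing voice lines.
; Tick closes the shop or portal panel when the player walks out of range.
; It also spawns screen-projected damage text above actors.
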(event `InitPlayerCharacter`
  (params (PlayerCharacter :type "/Game/Core/Blueprints/Gameplay/Characters/PlayerCharacters/BP_PlayerCharacterBase Object Reference"))
  (set `self.PlayerCharacter` PlayerCharacter)
  (bind _returnvalue (`|CreateWidget` "/Game/Core/Widgets/Gameplay/WBP_InGameHUD.WBP_InGameHUD_C"))
  (bind _output_get (set `self.HUDWidget` _returnvalue))
  (`UserWidget.AddToViewport` _output_get 0)
  (`/Game/Core/Widgets/Gameplay/WBP_InGameHUD.InitPlayerCharacter` (`self.HUDWidget`) (`self.PlayerCharacter`)))

(event `ShowDamageText`
  (params (Damage :type "Float (double-precision)") (Actor :type "Actor Object Reference"))
  (bind _returnvalue (`|CreateWidget` "/Game/Core/Widgets/Gameplay/DamageText/WBP_DamageText.WBP_DamageText_C" null Damage))
  (`UserWidget.AddToViewport` _returnvalue 0)
  (`UserWidget.SetPositionInViewport` _returnvalue (`PlayerController.ProjectWorldLocationToScreen` (`GameplayStatics.GetPlayerController` 0) (+ (`self.K2_GetActorLocation` Actor) (0.0 0.0 45.0)) false) true))

(event `SetInventoryVisibility`
  (params (Show :type Boolean))
  (bind _output_get (set `self.IsInventoryVisible` Show))
  (`Widget.SetVisibility` (`/Game/Core/Widgets/Gameplay/WBP_InGameHUD.WBP_Inventory` (`self.HUDWidget`)) (select `bool` _output_get :`false` "Hidden" :`true` "Visible" :!type "ESlateVisibility Enum"))
  (`Widget.SetVisibility` (`/Game/Core/Widgets/Gameplay/WBP_InGameHUD.WBP_Equipment` (`self.HUDWidget`)) (select `bool` _output_get :`false` "Hidden" :`true` "Visible" :!type "ESlateVisibility Enum"))
  (`self.HandleInput`))

(event `ToggleInventory`
  (`self.SetInventoryVisibility` (not (`self.IsInventoryVisible`))))

(event `SetShopkeeper`
  (params (Show :type Boolean) (Shopkeeper :type "/Game/Core/Blueprints/Gameplay/Characters/Shopkeeper/BP_Shopkeeper Object Reference"))
  (bind _wbp_shopkeeper (`/Game/Core/Widgets/Gameplay/WBP_InGameHUD.WBP_Shopkeeper` (`self.HUDWidget`)))
  (bind _wbp_shopkeeper_2 (`/Game/Core/Widgets/Gameplay/WBP_InGameHUD.WBP_Shopkeeper` (`self.HUDWidget`)))
  (bind _output_get (set `self.IsShopkeeperVisible` Show))
  (if _output_get
    (set `self.CurrentShopkeeper` Shopkeeper)
    (`Widget.SetVisibility` _wbp_shopkeeper "Visible")
    (`/Game/Core/Widgets/Gameplay/Shopkeeper/WBP_Shopkeeper.SetShopkeeper` _wbp_shopkeeper (`self.CurrentShopkeeper`))
    (bind _shopkeepersound (`self.ShopkeeperSound`)
      (:`then`
        (`AudioComponent.Stop` _shopkeepersound))
      (:`else`
        _))
    (bind _returnvalue (`GameplayStatics.SpawnSound2D` "/Game/Placeholder-Assets/SFX/SelectedSFX/VoiceSFX/ShopkeeprSFX/12_BARTOLEMEU_How_Can_I_Assist_You_Cue.12_BARTOLEMEU_How_Can_I_Assist_You_Cue" 1.0 1.0 0.0 null))
    (bind _output_get_2 (set `self.ShopkeeperSound` _returnvalue))
    (`AudioComponent.Play` _output_get_2 0.0)
    (`self.HandleInput`)
    (else
      (set `self.CurrentShopkeeper` null)
      (`Widget.SetVisibility` _wbp_shopkeeper_2 "Hidden")
      (`/Game/Core/Widgets/Gameplay/Shopkeeper/WBP_Shopkeeper.SetShopkeeper` _wbp_shopkeeper_2 null)
      (bind _shopkeepersound_2 (`self.ShopkeeperSound`)
        (:`then`
          (`AudioComponent.Stop` _shopkeepersound_2))
        (:`else`
          _))
      (bind _returnvalue_2 (`GameplayStatics.SpawnSound2D` "/Game/Placeholder-Assets/SFX/SelectedSFX/VoiceSFX/ShopkeeprSFX/20_BARTOLEMEU_Off_You_Go_Cue.20_BARTOLEMEU_Off_You_Go_Cue" 1.0 1.0 0.0 null))
      (bind _output_get_3 (set `self.ShopkeeperSound` _returnvalue_2))
      (`AudioComponent.Play` _output_get_3 0.0)
      (`self.HandleInput`))))

(event `ToggleShopkeeper`
  (params (Shopkeeper :type "/Game/Core/Blueprints/Gameplay/Characters/Shopkeeper/BP_Shopkeeper Object Reference"))
  (if (!= (`self.CurrentShopkeeper`) Shopkeeper)
    (`self.SetShopkeeper` true Shopkeeper)
    (else
      (`self.SetShopkeeper` false))))

(event `self.ReceiveTick`
  (params (DeltaSeconds :type "Float (single-precision)"))
  (`self.HandleShopkeeperDistance`)
  (`self.HandlePortalDistance`))

(event `SetFullMapVisibility`
  (params (Show :type Boolean))
  (bind _output_get (set `self.IsFullMapVisible` Show))
  (`Widget.SetVisibility` (`/Game/Core/Widgets/Gameplay/WBP_InGameHUD.WBP_FullMap` (`self.HUDWidget`)) (select `bool` _output_get :`false` "Hidden" :`true` "Visible" :!type "ESlateVisibility Enum")))

(event `ToggleFullMap`
  (`self.SetFullMapVisibility` (not (`self.IsFullMapVisible`))))

(event `SetPortal`
  (params (Show :type Boolean) (Portal :type "/Game/Core/Blueprints/Gameplay/Components/WeaponSystemComponent/Weapons/Portal/BP_Portal Object Reference"))
  (bind _output_get (set `self.IsPortalVisible` Show))
  (if _output_get
    (set `self.CurrentPortal` Portal)
    (`Widget.SetVisibility` (`/Game/Core/Widgets/Gameplay/WBP_InGameHUD.WBP_PortalMap` (`self.HUDWidget`)) "Visible")
    (`self.HandleInput`)
    (else
      (set `self.CurrentPortal` null)
      (`Widget.SetVisibility` (`/Game/Core/Widgets/Gameplay/WBP_InGameHUD.WBP_PortalMap` (`self.HUDWidget`)) "Hidden")
      (`self.HandleInput`))))

(event `TogglePortal`
  (params (Portal :type "/Game/Core/Blueprints/Gameplay/Components/WeaponSystemComponent/Weapons/Portal/BP_Portal Object Reference"))
  (if (!= (`self.CurrentPortal`) Portal)
    (`self.SetPortal` true Portal)
    (else
      (`self.SetPortal` false))))

(fn `HandlePortalDistance`
  (if (`self.IsPortalVisible`)
    (bind _currentportal (`self.CurrentPortal`)
      (:`then`
        (if (> (`KismetMathLibrary.Vector_Distance` (`self.K2_GetActorLocation` _currentportal) (`self.K2_GetActorLocation` (`GameplayStatics.GetPlayerCharacter` 0))) 450.0)
          (`self.SetPortal` false)))
      (:`else`
        (`self.SetPortal` false)))))

(fn `HandleShopkeeperDistance`
  (if (`self.IsShopkeeperVisible`)
    (bind _currentshopkeeper (`self.CurrentShopkeeper`)
      (:`then`
        (if (> (`KismetMathLibrary.Vector_Distance` (`self.K2_GetActorLocation` _currentshopkeeper) (`self.K2_GetActorLocation` (`GameplayStatics.GetPlayerCharacter` 0))) 450.0)
          (`self.SetShopkeeper` false)))
      (:`else`))))

(fn `UserConstructionScript`)