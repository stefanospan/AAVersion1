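; Shopkeeper character that offers randomly stocked, randomly priced items through a HUD shop screen toggled when a player interacts with it.
; On BeginPlay the server rolls each item definition's spawn chance and price range into a replicated item list, whose OnRep broadcasts updates.
; The server also starts a looping timer, and a day check against Ultra Dynamic Sky sets replicated IsActive, which toggles visibility, collision and movement.
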(event `self.ReceiveBeginPlay`
  ; Init
  (`parent.ReceiveBeginPlay`)
  (`self.UpdateState`)
  (`/Engine/EditorBlueprintResources/ActorMacros.Switch Has Authority`
    (:`Authority`
      (`|ExecutionSequence`
        (:`then_0`
          (for _array_element (`self.ShopkeeperItemDefinitions`)
            (bind (_item _spawnchance _pricerange) (break `/Game/Core/Blueprints/Gameplay/Characters/Shopkeeper/Structures/ST_ShopkeeperItemDefinitionData` _array_element))
            (if (`KismetMathLibrary.RandomBoolWithWeight` _spawnchance)
              (bind (_x _y) (break `IntPoint` _pricerange))
              (`KismetArrayLibrary.Array_Add` (`self.ShopkeeperItems`) (make `/Game/Core/Blueprints/Gameplay/Characters/Shopkeeper/Structures/ST_ShopkeeperItemData` _item (`KismetMathLibrary.RandomIntegerInRange` _x _y)))))
          (set `self.ShopkeeperItems` (`self.ShopkeeperItems`)))
        (:`then_1`
          (bind _uds (`/Game/UltraDynamicSky/Blueprints/Functions/UltraDynamicSky_Functions.Get Ultra Dynamic Sky`))
          (set `self.UDS` _uds)
          (`KismetSystemLibrary.K2_SetTimerDelegate` (`|CreateDelegate` :!event `CheckTime`) 1.0 true))))))

(event `self.BPC_Interactable.ClientOnInteract`
  (params (InteractionSystemComponent :type "/Game/Core/Blueprints/Gameplay/Components/InteractionSystemComponent/BPC_InteractionSystemComponent Object Reference"))
  ; Calls to toggle shopkeeper UI
  (bind _ascharacter (cast `Character` (`ActorComponent.GetOwner` InteractionSystemComponent)))
  (bind _asplayer_controller (cast `PlayerController` (`self.GetController` _ascharacter)))
  (bind _asbp_hudbase (cast `/Game/Core/Blueprints/Gameplay/GameMode/BP_HUDBase` (`PlayerController.GetHUD` _asplayer_controller)))
  (`/Game/Core/Blueprints/Gameplay/GameMode/BP_HUDBase.ToggleShopkeeper` _asbp_hudbase self))

(fn `CheckTime`
  (if (!= (`/Game/UltraDynamicSky/Blueprints/Ultra_Dynamic_Sky.Is it Daytime?` (`self.UDS`)) (`self.IsActive`))
    (set `self.IsActive` (`/Game/UltraDynamicSky/Blueprints/Ultra_Dynamic_Sky.Is it Daytime?` (`self.UDS`)))))

(fn `GetInteractable`
  (returns (Interactable :type "/Game/Core/Blueprints/Gameplay/Components/InteractionSystemComponent/BPC_Interactable Object Reference"))
  (return (`self.BPC_Interactable`)))

(fn `GetShopkeeperItems`
  (returns (ShopkeeperItems :type "Array of /Game/Core/Blueprints/Gameplay/Characters/Shopkeeper/Structures/ST_ShopkeeperItemData Structure"))
  (return (`self.ShopkeeperItems`)))

(fn `OnRep_IsActive`
  (`self.UpdateState`))

(fn `OnRep_ShopkeeperItems`
  (`self.OnUpdatedShopkeeperItems` (`self.ShopkeeperItems`)))

(fn `UpdateState`
  (if (`self.IsActive`)
    (`CharacterMovementComponent.SetMovementMode` (`self.CharacterMovement`) "MOVE_Walking" 0)
    (`self.SetActorEnableCollision` true)
    (`self.SetActorHiddenInGame` false)
    (else
      (`CharacterMovementComponent.SetMovementMode` (`self.CharacterMovement`) "MOVE_None" 0)
      (`self.SetActorEnableCollision` false)
      (`self.SetActorHiddenInGame` true))))

(fn `UserConstructionScript`)