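; Sigrun's first ability, which sends a BP_SigrunSpirit from the owner to a chosen teammate.
; While left mouse is held, the local player gets a cursor with look input locked, and a sphere trace under it places a marker above the hovered teammate.
; Release passes the target to ServerTarget, which commits and spawns the spirit if valid, then ends.
; Activation requires fewer than two characters carrying the owner's Spirit Embrace effect.
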(event `self.OnAbilityActivated`
  (if (`self.IsLocal`)
    (bind _returnvalue (`|SpawnActorFromClass` "/Game/Core/Blueprints/Gameplay/Characters/PlayerCharacters/Sigrun/Ability1/BP_SigrunTarget.BP_SigrunTarget_C" (`KismetMathLibrary.MakeTransform` (0.0 0.0 0.0)) "AlwaysSpawn" "MultiplyWithRoot" null null))
    (set `self.SigrunTargetActor` _returnvalue)
    (`self.SetActorTickEnabled` true)
    (`Controller.SetIgnoreLookInput` (`GameplayStatics.GetPlayerController` 0) true)
    (set `PlayerController.bShowMouseCursor` true (`GameplayStatics.GetPlayerController` 0))
    (bind _asbp_player_character_base (cast `/Game/Core/Blueprints/Gameplay/Characters/BP_PlayerCharacterBase` (`self.GetOwnerCharacter`)))
    (if (`/Game/Core/Blueprints/Gameplay/Characters/BP_PlayerCharacterBase.GetIsLeftMousePressed` _asbp_player_character_base)
      (add `/Game/Core/Blueprints/Gameplay/Characters/BP_PlayerCharacterBase.OnUpdatedIsLeftMousePressed` _asbp_player_character_base (`|CreateDelegate` :!event `OnUpdatedIsLeftMousePressed`))
      (else
        (`self.ReleaseButton`)))))

(event `self.ReceiveTick`
  (params (DeltaSeconds :type "Float (single-precision)"))
  (if (`self.IsLocal`)
    (`self.SigrunTargetActor`
      (:`then`
        (bind (_found _character) (`self.GetHoveredTeammate`))
        (if _found
          (set `self.HoveredCharacter` _character)
          (`self.SetActorHiddenInGame` (`self.SigrunTargetActor`) false)
          (`self.K2_SetActorLocation` (`self.SigrunTargetActor`) (+ (`self.K2_GetActorLocation` (`self.HoveredCharacter`)) (0.0 0.0 120.0)) false false)
          (else
            (`self.SetActorHiddenInGame` (`self.SigrunTargetActor`) true)
            (set `self.HoveredCharacter` null))))
      (:`else`))))

(event `ReleaseButton`
  (`self.ServerTarget` (`self.HoveredCharacter`))
  (set `self.HoveredCharacter` null)
  (`Controller.SetIgnoreLookInput` (`GameplayStatics.GetPlayerController` 0) false)
  (set `PlayerController.bShowMouseCursor` false (`GameplayStatics.GetPlayerController` 0))
  (bind _sigruntargetactor (`self.SigrunTargetActor`)
    (:`then`
      (`self.K2_DestroyActor` _sigruntargetactor)
      (set `self.SigrunTargetActor` null))
    (:`else`)))

(event `OnUpdatedIsLeftMousePressed`
  (params (IsLeftMousePressed :type Boolean))
  (if (not IsLeftMousePressed)
    (bind _asbp_player_character_base (cast `/Game/Core/Blueprints/Gameplay/Characters/BP_PlayerCharacterBase` (`self.GetOwnerCharacter`)))
    (remove `/Game/Core/Blueprints/Gameplay/Characters/BP_PlayerCharacterBase.OnUpdatedIsLeftMousePressed` _asbp_player_character_base (`|CreateDelegate` :!event `OnUpdatedIsLeftMousePressed`))
    (`self.ReleaseButton`)))

(event `ServerTarget`
  (params (Target :type "Character Object Reference"))
  (bind (_returnvalue_roll _returnvalue_pitch _returnvalue_yaw) (`KismetMathLibrary.BreakRotator` (`KismetMathLibrary.FindLookAtRotation` (`self.K2_GetActorLocation` (`self.GetOwnerCharacter`)) (`self.K2_GetActorLocation` Target))))
  (`/Engine/EditorBlueprintResources/StandardMacros.IsValid` Target
    (:`Is Valid`
      (`self.CommitAbility`)
      (`|SpawnActorFromClass` "/Game/Core/Blueprints/Gameplay/Characters/PlayerCharacters/Sigrun/Ability1/BP_SigrunSpirit.BP_SigrunSpirit_C" (`KismetMathLibrary.MakeTransform` (`self.K2_GetActorLocation` (`self.GetOwnerCharacter`)) (`KismetMathLibrary.MakeRotator` 0.0 0.0 _returnvalue_yaw)) "AlwaysSpawn" "MultiplyWithRoot" (`self.GetOwnerCharacter`) Target null)
      (`self.EndAbility`))
    (:`Is Not Valid`
      (`self.EndAbility`))))

(fn `CanActivate`
  (returns (Success :type Boolean))
  (locals (Chars :type "Array of /Game/Core/Blueprints/Gameplay/Characters/BP_CharacterBase Object Reference") (Counter :type Integer))
  (bind _output_get (set `local.Chars` (`/Game/Core/Blueprints/Gameplay/Components/CharacterManagerComponent/BPC_CharacterManagerComponent.GetRegisteredCharacters` (`self.GetComponentByClass` (`GameplayStatics.GetGameState`) "/Game/Core/Blueprints/Gameplay/Components/CharacterManagerComponent/BPC_CharacterManagerComponent.BPC_CharacterManagerComponent_C"))))
  (for _array_element _output_get
    (bind _effectcomponent (message `/Game/Core/Blueprints/Gameplay/Components/EffectComponent/BPI_Effects.GetEffectComponent` _array_element))
    (for _array_element_2 (`/Game/Core/Blueprints/Gameplay/Components/EffectComponent/BPC_EffectComponent.GetActiveEffects` _effectcomponent)
      (if (and (== (`GameplayStatics.GetObjectClass` _array_element_2) "/Game/Core/Blueprints/Gameplay/Characters/PlayerCharacters/Sigrun/Ability1/BP_Effect_SpiritEmbrace.BP_Effect_SpiritEmbrace_C") (== (`/Game/Core/Blueprints/Gameplay/Components/EffectComponent/BP_EffectBase.GetInstigatorActor` _array_element_2) (`self.GetOwnerCharacter`)))
        (`/Engine/EditorBlueprintResources/StandardMacros.IncrementInt` (`local.Counter`)
          (:`  `
            (break))))))
  (return (< (`local.Counter`) 2)))

(fn `GetHoveredTeammate`
  (returns (Found :type Boolean) (Character :type "Character Object Reference"))
  (bind (_worldlocation _worlddirection) (`PlayerController.DeprojectMousePositionToWorld` (`GameplayStatics.GetPlayerController` 0)))
  (bind _outhit (`KismetSystemLibrary.SphereTraceSingle` _worldlocation (+ _worldlocation (* _worlddirection 10000.0)) 10.0 "TraceTypeQuery1"))
  (bind (_bblockinghit _binitialoverlap _time _distance _location _impactpoint _normal _impactnormal _physmat _hitactor) (`GameplayStatics.BreakHitResult` _outhit))
  (if _bblockinghit
    (bind _ascharacter (cast `Character` _hitactor)
      (:`then`
        (bind _team (message `/Game/Core/Blueprints/Gameplay/Components/TeamComponent/BPI_Teams.GetTeam` _ascharacter))
        (bind _team_2 (message `/Game/Core/Blueprints/Gameplay/Components/TeamComponent/BPI_Teams.GetTeam` (`self.GetOwnerCharacter`)))
        (if (== _team_2 _team)
          (return true _ascharacter)
          (else
            _)))
      (:`CastFailed`
        _)))
  (return false null))

(fn `UserConstructionScript`
  (`parent.UserConstructionScript`))