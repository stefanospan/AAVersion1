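; BP_SigrunSpirit is the spirit actor for Sigrun's Ability1, which flies to a target actor and applies the Spirit Embrace effect.
; On BeginPlay, only the authority plays a timeline that lerps from the spawn location to the target's current location, so it follows a moving target without sweeping.
; When the timeline finishes, it applies the effect through the target's effect component with its owner as instigator, then destroys itself.
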(event `self.ReceiveBeginPlay`
  (`/Engine/EditorBlueprintResources/ActorMacros.Switch Has Authority`
    (:`Authority`
      (set `self.InitLocation` (`self.K2_GetActorLocation`))
      (bind (_direction _alpha) (`Timeline|MoveTimeline`)
        (:`Update`
          (`self.K2_SetActorLocation` (`KismetMathLibrary.VLerp` (`self.InitLocation`) (`self.K2_GetActorLocation` (`self.TargetActor`)) _alpha)))
        (:`Finished`
          (bind _effectcomponent (message `/Game/Core/Blueprints/Gameplay/Components/EffectComponent/BPI_Effects.GetEffectComponent` (`self.TargetActor`)))
          (`/Game/Core/Blueprints/Gameplay/Components/EffectComponent/BPC_EffectComponent.ApplyEffect` _effectcomponent "/Game/Core/Blueprints/Gameplay/Characters/PlayerCharacters/Sigrun/Ability1/BP_Effect_SpiritEmbrace.BP_Effect_SpiritEmbrace_C" (`self.GetOwner`))
          (`self.K2_DestroyActor`))))))

(fn `UserConstructionScript`)