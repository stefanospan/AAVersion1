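; Sigrun's second ability, which applies the Spirit Surge effect to her own character.
; On activation it plays a looping slide sound in 2D, then on authority asks the owner's effect component to apply the effect with the owner as instigator.
; The ability commits only if the effect applies, and ends on authority either way.
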(event `self.OnAbilityActivated`
  (`GameplayStatics.PlaySound2D` "/Game/UI_SFX_Free_Pack/Wavs/Sliders/slide_loop_1.slide_loop_1" 1.0 1.0 0.0 null null)
  (`/Engine/EditorBlueprintResources/ActorMacros.Switch Has Authority`
    (:`Authority`
      (bind _effectcomponent (message `/Game/Core/Blueprints/Gameplay/Components/EffectComponent/BPI_Effects.GetEffectComponent` (`self.GetOwnerCharacter`)))
      (bind _success (`/Game/Core/Blueprints/Gameplay/Components/EffectComponent/BPC_EffectComponent.ApplyEffect` _effectcomponent "/Game/Core/Blueprints/Gameplay/Characters/PlayerCharacters/Sigrun/Ability2/BP_Effect_SpiritSurge.BP_Effect_SpiritSurge_C" (`self.GetOwnerCharacter`)))
      (if _success
        (`self.CommitAbility`)
        (`self.EndAbility`)
        (else
          (`self.EndAbility`))))))

(fn `UserConstructionScript`
  (`parent.UserConstructionScript`))