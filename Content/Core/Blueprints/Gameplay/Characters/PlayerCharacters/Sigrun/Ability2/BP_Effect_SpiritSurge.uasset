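; BP_Effect_SpiritSurge is the effect for Sigrun's second ability, Spirit Surge, that turns her spirit on while active.
; When applied or removed, it casts the effect component's owner to BP_PlayerCharacter_Sigrun and calls ToggleSpirit on or off to match.
; It does nothing if the owner is not Sigrun, and all spirit behavior lives in the character Blueprint.
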(event `self.OnEffectApplied`
  (bind _asbp_player_character_sigrun (cast `/Game/Core/Blueprints/Gameplay/Characters/PlayerCharacters/Sigrun/BP_PlayerCharacter_Sigrun` (`ActorComponent.GetOwner` (`self.GetEffectComponent`))))
  (`/Game/Core/Blueprints/Gameplay/Characters/PlayerCharacters/Sigrun/BP_PlayerCharacter_Sigrun.ToggleSpirit` _asbp_player_character_sigrun true))

(event `self.OnEffectRemoved`
  (bind _asbp_player_character_sigrun (cast `/Game/Core/Blueprints/Gameplay/Characters/PlayerCharacters/Sigrun/BP_PlayerCharacter_Sigrun` (`ActorComponent.GetOwner` (`self.GetEffectComponent`))))
  (`/Game/Core/Blueprints/Gameplay/Characters/PlayerCharacters/Sigrun/BP_PlayerCharacter_Sigrun.ToggleSpirit` _asbp_player_character_sigrun false))

(fn `UserConstructionScript`
  (`parent.UserConstructionScript`))