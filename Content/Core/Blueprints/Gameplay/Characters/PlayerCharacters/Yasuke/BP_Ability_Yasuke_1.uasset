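; Yasuke's first ability: a forward dodge lunge that passes through pawns and damages characters on other teams.
; On activation the server commits, plays the root dodge montage, launches the character forward and up, and multicasts the capsule to ignore Pawn.
; Montage notifies toggle a Tick sphere trace that hits each target once per window, scaling damage by the DamageMultiplier attribute.
; Montage end stops tracing, restores collision and ends the ability.
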(event `self.OnAbilityActivated`
  (`/Engine/EditorBlueprintResources/ActorMacros.Switch Has Authority`
    (:`Authority`
      (`self.CommitAbility`)
      (`self.MulticastTogglePawnCollision` true)
      (`self.PlayAnimMontage` "/Game/Core/Animations/DodgesRolls/DodgeForward_Root_Montage.DodgeForward_Root_Montage")
      (`Character.LaunchCharacter` (`self.GetOwnerCharacter`) (+ (* (`self.GetActorForwardVector` (`self.GetOwnerCharacter`)) (`self.ForwardForce`)) (`KismetMathLibrary.MakeVector` 0.0 0.0 (`self.UpForce`))) false false))))

(event `self.OnAnimMontageEnded`
  (`/Engine/EditorBlueprintResources/ActorMacros.Switch Has Authority`
    (:`Authority`
      (`self.ToggleTrace` false)
      (`self.MulticastTogglePawnCollision` false)
      (`self.EndAbility`))))

(event `MulticastTogglePawnCollision`
  (params (IgnorePawn :type Boolean))
  (`PrimitiveComponent.SetCollisionResponseToChannel` (`Character.CapsuleComponent` (`self.GetOwnerCharacter`)) "ECC_Pawn" (select `bool` IgnorePawn :`false` "ECR_Block" :`true` "ECR_Ignore" :!type "ECollisionResponse Enum")))

(event `self.OnNotifyBegin`
  (params (NotifyName :type Name))
  (`/Engine/EditorBlueprintResources/ActorMacros.Switch Has Authority`
    (:`Authority`
      (switch `name` NotifyName
        (:`Trace`
          (`self.ToggleTrace` true))))))

(event `self.OnNotifyEnd`
  (params (NotifyName :type Name))
  (`/Engine/EditorBlueprintResources/ActorMacros.Switch Has Authority`
    (:`Authority`
      (switch `name` NotifyName
        (:`Trace`
          (`self.ToggleTrace` false))))))

(event `ToggleTrace`
  (params (IsTrace :type Boolean))
  (set `self.IsTrace` IsTrace)
  (`KismetArrayLibrary.Array_Clear` (`self.AttackedActors`))
  (`self.SetActorTickEnabled` (`self.IsTrace`)))

(event `self.ReceiveTick`
  (params (DeltaSeconds :type "Float (single-precision)"))
  (bind _ownercharacter (`self.GetOwnerCharacter`))
  (bind _returnvalue (`self.K2_GetActorLocation` _ownercharacter))
  (`/Engine/EditorBlueprintResources/ActorMacros.Switch Has Authority`
    (:`Authority`
      (bind _team (message `/Game/Core/Blueprints/Gameplay/Components/TeamComponent/BPI_Teams.GetTeam` (`self.GetOwnerCharacter`)))
      (bind _outhits (`KismetSystemLibrary.SphereTraceMulti` _returnvalue (+ _returnvalue (* (`self.GetActorForwardVector` _ownercharacter) 50.0)) 50.0 "TraceTypeQuery1" false (`|MakeArray` (`self.GetOwnerCharacter`) :!type "Actor Object Reference")))
      (for _array_element _outhits
        (bind (_bblockinghit _binitialoverlap _time _distance _location _impactpoint _normal _impactnormal _physmat _hitactor) (`GameplayStatics.BreakHitResult` _array_element))
        (bind _team_2 (message `/Game/Core/Blueprints/Gameplay/Components/TeamComponent/BPI_Teams.GetTeam` _hitactor))
        (if (!= _team_2 _team)
          (bind _returnvalue_2 (`KismetArrayLibrary.Array_AddUnique` (`self.AttackedActors`) _hitactor))
          (if (>= _returnvalue_2 0)
            (`GameplayStatics.ApplyDamage` _hitactor (* (`self.Damage`) (`.Value_5_5382FAD64776275FF614BEB1A224EFA3` (break `/Game/Core/Blueprints/Gameplay/Components/AttributeComponent/Structures/ST_AttributeData` (`self.GetAttribute` (struct :`TagName` "Attribute.DamageMultiplier"))))) null (`self.GetOwnerCharacter`))))))))

(fn `UserConstructionScript`
  (`parent.UserConstructionScript`))