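; Yasuke's second ability, a 360-degree melee sword attack that plays a montage and damages characters on other teams.
; Montage notifies switch actor tick on and off to open and close the hit window.
; Each tick sphere-traces between the sword mesh's start and end sockets, damaging each enemy once per window, scaled by the DamageMultiplier attribute.
; Commit, tracing, damage and ability end run only on the server.
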(event `self.OnAbilityActivated`
  (`/Engine/EditorBlueprintResources/ActorMacros.Switch Has Authority`
    (:`Authority`
      (`self.CommitAbility`)
      (bind _asbp_player_character_yasuke (cast `/Game/Core/Blueprints/Gameplay/Characters/PlayerCharacters/Yasuke/BP_PlayerCharacter_Yasuke` (`self.GetOwnerCharacter`)))
      (set `self.YasukeCharacter` _asbp_player_character_yasuke)
      (`self.PlayAnimMontage` "/Game/Core/Animations/Sword/StandingMeleeAttack360Low_UE_Montage.StandingMeleeAttack360Low_UE_Montage"))))

(event `self.OnAnimMontageEnded`
  (`/Engine/EditorBlueprintResources/ActorMacros.Switch Has Authority`
    (:`Authority`
      (`self.ToggleTrace` false)
      (`self.EndAbility`))))

(event `self.OnNotifyBegin`
  (params (NotifyName :type Name))
  (`/Engine/EditorBlueprintResources/ActorMacros.Switch Has Authority`
    (:`Authority`
      (switch `name` NotifyName
        (:`Trace`
          (`self.ToggleTrace` true))))))

(event `self.OnNotifyEnd`
  (params (NotifyName :type Name))
  (`/Engine/EditorBlueprintResources/ActorMacros.Switch Has Authority`
    (:`Authority`
      (switch `name` NotifyName
        (:`Trace`
          (`self.ToggleTrace` false))))))

(event `ToggleTrace`
  (params (IsTrace :type Boolean))
  (set `self.IsTrace` IsTrace)
  (`KismetArrayLibrary.Array_Clear` (`self.AttackedActors`))
  (`self.SetActorTickEnabled` (`self.IsTrace`)))

(event `self.ReceiveTick`
  (params (DeltaSeconds :type "Float (single-precision)"))
  (bind _swordmesh (`/Game/Core/Blueprints/Gameplay/Characters/PlayerCharacters/Yasuke/BP_PlayerCharacter_Yasuke.SwordMesh` (`self.YasukeCharacter`)))
  (`/Engine/EditorBlueprintResources/ActorMacros.Switch Has Authority`
    (:`Authority`
      (bind _team (message `/Game/Core/Blueprints/Gameplay/Components/TeamComponent/BPI_Teams.GetTeam` (`self.GetOwnerCharacter`)))
      (bind _outhits (`KismetSystemLibrary.SphereTraceMulti` (`SceneComponent.GetSocketLocation` _swordmesh "TraceStart") (`SceneComponent.GetSocketLocation` _swordmesh "TraceEnd") 22.5 "TraceTypeQuery1" false (`|MakeArray` (`self.GetOwnerCharacter`) :!type "Actor Object Reference")))
      (for _array_element _outhits
        (bind (_bblockinghit _binitialoverlap _time _distance _location _impactpoint _normal _impactnormal _physmat _hitactor) (`GameplayStatics.BreakHitResult` _array_element))
        (bind _team_2 (message `/Game/Core/Blueprints/Gameplay/Components/TeamComponent/BPI_Teams.GetTeam` _hitactor))
        (if (!= _team_2 _team)
          (bind _returnvalue (`KismetArrayLibrary.Array_AddUnique` (`self.AttackedActors`) _hitactor))
          (if (>= _returnvalue 0)
            (`GameplayStatics.ApplyDamage` _hitactor (* (`self.Damage`) (`.Value_5_5382FAD64776275FF614BEB1A224EFA3` (break `/Game/Core/Blueprints/Gameplay/Components/AttributeComponent/Structures/ST_AttributeData` (`self.GetAttribute` (struct :`TagName` "Attribute.DamageMultiplier"))))) null (`self.GetOwnerCharacter`))))))))

(fn `UserConstructionScript`
  (`parent.UserConstructionScript`))