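; Rapid Retreat ability for the Dash player character that launches the owner backward and upward in a dodge.
; On activation, only the authority commits the ability, plays the backward dodge montage and calls LaunchCharacter.
; The launch adds the reversed actor forward vector, scaled by a forward force, to an upward force without overriding existing velocity.
; The ability ends immediately after the launch, without waiting for the montage.
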(event `self.OnAbilityActivated`
  (`/Engine/EditorBlueprintResources/ActorMacros.Switch Has Authority`
    (:`Authority`
      (`self.CommitAbility`)
      (`self.PlayAnimMontage` "/Game/Core/Animations/DodgesRolls/DodgeBackward_Root_Montage.DodgeBackward_Root_Montage")
      (`Character.LaunchCharacter` (`self.GetOwnerCharacter`) (+ (* (`self.GetActorForwardVector` (`self.GetOwnerCharacter`)) (`self.ForwardForce`) -1.0) (`KismetMathLibrary.MakeVector` 0.0 0.0 (`self.UpForce`))) false false)
      (`self.EndAbility`))))

(fn `UserConstructionScript`
  (`parent.UserConstructionScript`))