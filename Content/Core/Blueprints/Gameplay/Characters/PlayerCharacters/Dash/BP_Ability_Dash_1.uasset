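; Dash ability for player characters that launches the owner forward and hits enemies ahead.
; On activation the server plays a dodge montage, commits, and launches the owner, at reduced forward force when airborne.
; A montage notify multicasts a short-lived water particle effect, then sphere-traces forward for opposing-team characters, applying multiplier-scaled damage and knockback.
; Gameplay is authority-only, and montage end ends the ability.
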(event `self.OnAbilityActivated`
  (bind _ownercharacter (`self.GetOwnerCharacter`))
  (bind _forwardforce (`self.ForwardForce`))
  (`GameplayStatics.PlaySound2D` "/Game/Placeholder-Assets/SFX/FabSFX_Packs/Sci-Fi_Shots_Pack2_Game_Of_Weapons/Wave/SciFi_Shot_P2__20_.SciFi_Shot_P2__20_" 1.0 1.0 0.0 null null)
  (`/Engine/EditorBlueprintResources/ActorMacros.Switch Has Authority`
    (:`Authority`
      (`self.PlayAnimMontage` "/Game/Core/Animations/DodgesRolls/DodgeForward_Root_Montage1.DodgeForward_Root_Montage1")
      (`self.CommitAbility`)
      (`Character.LaunchCharacter` (`self.GetOwnerCharacter`) (+ (* (`self.GetActorForwardVector` _ownercharacter) (select `bool` (`NavMovementComponent.IsFalling` (`Character.CharacterMovement` _ownercharacter)) :`false` _forwardforce :`true` (* _forwardforce 0.5) :!type "Float (single-precision)")) (`KismetMathLibrary.MakeVector` 0.0 0.0 (`self.UpForce`))) false false))))

(event `self.OnNotifyBegin`
  (params (NotifyName :type Name))
  (`/Engine/EditorBlueprintResources/ActorMacros.Switch Has Authority`
    (:`Authority`
      (switch `name` NotifyName
        (:`Shockwave`
          (`self.MulticastVisuals`)
          (bind _characters (`self.GetTargetCharacters`))
          (for _array_element _characters
            (`GameplayStatics.ApplyDamage` _array_element (* (`self.Damage`) (`.Value_5_5382FAD64776275FF614BEB1A224EFA3` (break `/Game/Core/Blueprints/Gameplay/Components/AttributeComponent/Structures/ST_AttributeData` (`self.GetAttribute` (struct :`TagName` "Attribute.DamageMultiplier"))))))
            (`Character.LaunchCharacter` _array_element (+ (* (`self.GetActorForwardVector` (`self.GetOwnerCharacter`)) 650.0) (0.0 0.0 75.0)) true true)))))))

(event `MulticastVisuals`
  (`/Engine/EditorBlueprintResources/StandardMacros.Can Execute Cosmetic Events`
    (:`True`
      (bind _returnvalue (`GameplayStatics.SpawnEmitterAttached` "/Game/AdvancedMagicFX12/particles/P_ky_shot_water.P_ky_shot_water" (`Actor.RootComponent` (`self.GetOwnerCharacter`)) "None" (40.0 0.0 0.0) (struct :`Yaw` 180.0) (1.0 1.0 1.0) "SnapToTarget"))
      (`KismetSystemLibrary.Delay` 0.5)
      (`ActorComponent.K2_DestroyComponent` _returnvalue))))

(event `self.OnAnimMontageEnded`
  (`/Engine/EditorBlueprintResources/ActorMacros.Switch Has Authority`
    (:`Authority`
      (`self.EndAbility`))))

(fn `GetTargetCharacters`
  (returns (Characters :type "Array of /Game/Core/Blueprints/Gameplay/Characters/BP_CharacterBase Object Reference"))
  (locals (CharactersTemp :type "Array of /Game/Core/Blueprints/Gameplay/Characters/BP_CharacterBase Object Reference"))
  (bind _ownercharacter (`self.GetOwnerCharacter`))
  (bind _returnvalue (`self.K2_GetActorLocation` _ownercharacter))
  (bind _team (message `/Game/Core/Blueprints/Gameplay/Components/TeamComponent/BPI_Teams.GetTeam` _ownercharacter))
  (bind _outhits (`KismetSystemLibrary.SphereTraceMultiForObjects` _returnvalue (+ _returnvalue (* (`self.GetActorForwardVector` _ownercharacter) 1000.0)) 50.0 (`|MakeArray` "ObjectTypeQuery3" :!type "EObjectTypeQuery Enum") false (`|MakeArray` (`self.GetOwnerCharacter`) :!type "Actor Object Reference")))
  (for _array_element _outhits
    (bind _asbp_character_base (cast `/Game/Core/Blueprints/Gameplay/Characters/BP_CharacterBase` (`.HitActor` (`GameplayStatics.BreakHitResult` _array_element))))
    (bind _team_2 (message `/Game/Core/Blueprints/Gameplay/Components/TeamComponent/BPI_Teams.GetTeam` _asbp_character_base))
    (if (!= _team_2 _team)
      (`KismetArrayLibrary.Array_AddUnique` (`local.CharactersTemp`) _asbp_character_base)))
  (return (`local.CharactersTemp`)))

(fn `UserConstructionScript`
  (`parent.UserConstructionScript`))