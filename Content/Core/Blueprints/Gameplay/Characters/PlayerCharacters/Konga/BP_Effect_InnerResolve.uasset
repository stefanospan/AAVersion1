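; Konga's Inner Resolve gameplay effect, which raises the owner's maximum health while it is active.
; On apply and on removal, it gets the stats component from the effect component's owner and sets the max value of the Stat.Health tag.
; Both values are hard-coded, so removal resets to a fixed baseline (half the boosted amount) instead of restoring the previous maximum.
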(event `self.OnEffectApplied`
  (bind _statcomponent (message `/Game/Core/Blueprints/Gameplay/Components/StatComponent/BPI_Stats.GetStatsComponent` (`ActorComponent.GetOwner` (`self.GetEffectComponent`))))
  (`/Game/Core/Blueprints/Gameplay/Components/StatComponent/BPC_StatComponent.SetStatMaxValue` _statcomponent (struct :`TagName` "Stat.Health") 2000.0))

(event `self.OnEffectRemoved`
  (bind _statcomponent (message `/Game/Core/Blueprints/Gameplay/Components/StatComponent/BPI_Stats.GetStatsComponent` (`ActorComponent.GetOwner` (`self.GetEffectComponent`))))
  (`/Game/Core/Blueprints/Gameplay/Components/StatComponent/BPC_StatComponent.SetStatMaxValue` _statcomponent (struct :`TagName` "Stat.Health") 1000.0))

(fn `UserConstructionScript`
  (`parent.UserConstructionScript`))