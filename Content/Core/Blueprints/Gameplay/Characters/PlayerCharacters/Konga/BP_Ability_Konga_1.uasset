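; Konga's leap-and-slam ability, moving the character forward and damaging nearby enemy-team characters.
; The server commits, fits montage speed to the move duration and sphere-traces a destination, stopping short of obstacles.
; A multicast timeline disables movement and sets location along a triangular height arc without sweeping, then restores walking.
; A montage notify spawns impact particles and applies multiplier-scaled sphere-overlap damage on the server; montage end ends the ability.
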(event `self.OnAbilityActivated`
  (`GameplayStatics.PlaySound2D` "/Game/Placeholder-Assets/SFX/FabSFX_Packs/Sci-Fi_Shots_Pack2_Game_Of_Weapons/Wave/SciFi_Shot_P2__20_.SciFi_Shot_P2__20_" 1.0 1.0 0.0 null null)
  (`/Engine/EditorBlueprintResources/ActorMacros.Switch Has Authority`
    (:`Authority`
      (`self.CommitAbility`)
      (`self.PlayAnimMontage` (`self.AnimMontage`) (/ (- (`AnimationAsset.GetPlayLength` (`self.AnimMontage`)) (`self.AnimEndOffset`)) (`self.MoveDuration`)))
      (bind _location (`self.FindTargetLocation`))
      (`self.MulticastMove` (`self.K2_GetActorLocation` (`self.GetOwnerCharacter`)) _location))))

(event `MulticastMove`
  (params (StartLocation :type "Vector Structure") (EndLocation :type "Vector Structure"))
  (`CharacterMovementComponent.SetMovementMode` (`Character.CharacterMovement` (`self.GetOwnerCharacter`)) "MOVE_None" 0)
  (`TimelineComponent.SetPlayRate` (`self.MoveTimeline`) (/ 1.0 (`self.MoveDuration`)))
  (bind (_direction _lerp) (`Timeline|MoveTimeline` :!via `PlayFromStart`)
    (:`Update`
      (`self.K2_SetActorLocation` (`self.GetOwnerCharacter`) (`KismetMathLibrary.MakeVector` (.x (`KismetMathLibrary.VLerp` StartLocation EndLocation _lerp)) (.y (`KismetMathLibrary.VLerp` StartLocation EndLocation _lerp)) (+ (.z StartLocation) (* (- 1.0 (`KismetMathLibrary.Abs` (- (* _lerp 2.0) 1.0))) (`self.MoveHeight`)))) false false))
    (:`Finished`
      (`CharacterMovementComponent.SetMovementMode` (`Character.CharacterMovement` (`self.GetOwnerCharacter`)) "MOVE_Walking" 0))))

(event `self.OnNotifyBegin`
  (params (NotifyName :type Name))
  (bind _ownercharacter (`self.GetOwnerCharacter`))
  (switch `name` NotifyName
    (:`Attack`
      (`|ExecutionSequence`
        (:`then_0`
          (`/Engine/EditorBlueprintResources/StandardMacros.Can Execute Cosmetic Events`
            (:`True`
              (`GameplayStatics.SpawnEmitterAtLocation` "/Game/AdvancedMagicFX13/Particles/P_ky_gaither.P_ky_gaither" (+ (- (`self.K2_GetActorLocation` _ownercharacter) (0.0 0.0 88.0)) (* (`self.GetActorForwardVector` _ownercharacter) 40.0))))))
        (:`then_1`
          (`/Engine/EditorBlueprintResources/ActorMacros.Switch Has Authority`
            (:`Authority`
              (bind _actors (`self.GetAttackActors`))
              (for _array_element _actors
                (`GameplayStatics.ApplyDamage` _array_element (* (`self.Damage`) (`.Value_5_5382FAD64776275FF614BEB1A224EFA3` (break `/Game/Core/Blueprints/Gameplay/Components/AttributeComponent/Structures/ST_AttributeData` (`self.GetAttribute` (struct :`TagName` "Attribute.DamageMultiplier"))))) null (`self.GetOwnerCharacter`))))))))))

(event `self.OnAnimMontageEnded`
  (`/Engine/EditorBlueprintResources/ActorMacros.Switch Has Authority`
    (:`Authority`
      (`self.EndAbility`))))

(fn `FindTargetLocation`
  (returns (Location :type "Vector Structure"))
  (bind _ownercharacter (`self.GetOwnerCharacter`))
  (bind _returnvalue (`self.GetActorForwardVector` _ownercharacter))
  (bind _returnvalue_2 (`self.K2_GetActorLocation` _ownercharacter))
  (bind _returnvalue_3 (+ _returnvalue_2 (* _returnvalue (`self.MoveDistance`))))
  (bind _outhit (`KismetSystemLibrary.SphereTraceSingle` _returnvalue_2 _returnvalue_3 30.0 "TraceTypeQuery1" false (`|MakeArray` (`self.GetOwnerCharacter`) :!type "Actor Object Reference") "ForDuration"))
  (bind (_bblockinghit _binitialoverlap _time _distance _location) (`GameplayStatics.BreakHitResult` _outhit))
  (return (select `bool` _bblockinghit :`false` _returnvalue_3 :`true` (+ _location (* _returnvalue -100.0)))))

(fn `GetAttackActors`
  (returns (Actors :type "Array of Actor Object Reference"))
  (locals (ActorsTemp :type "Array of Actor Object Reference"))
  (bind _ownercharacter (`self.GetOwnerCharacter`))
  (bind _team (message `/Game/Core/Blueprints/Gameplay/Components/TeamComponent/BPI_Teams.GetTeam` _ownercharacter))
  (bind _outactors (`KismetSystemLibrary.SphereOverlapActors` (`self.K2_GetActorLocation` _ownercharacter) 500.0 (`|MakeArray` "ObjectTypeQuery3" :!type "EObjectTypeQuery Enum") "/Game/Core/Blueprints/Gameplay/Characters/BP_CharacterBase.BP_CharacterBase_C" (`|MakeArray` (`self.GetOwnerCharacter`) :!type "Actor Object Reference")))
  (for _array_element _outactors
    (bind _team_2 (message `/Game/Core/Blueprints/Gameplay/Components/TeamComponent/BPI_Teams.GetTeam` _array_element))
    (if (!= _team_2 _team)
      (`KismetArrayLibrary.Array_Add` (`local.ActorsTemp`) _array_element)))
  (return (`local.ActorsTemp`)))

(fn `UserConstructionScript`
  (`parent.UserConstructionScript`))