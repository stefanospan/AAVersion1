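; Konga's second ability, which applies the Inner Resolve effect to its own character.
; Activation plays a 2D sound, then the authority commits the ability and plays a magic area attack montage.
; A montage notify triggers the server-side effect application through the owner's effect component, with the owner as instigator.
; The authority ends the ability when the montage finishes.
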(event `self.OnAbilityActivated`
  (`GameplayStatics.PlaySound2D` "/Game/Placeholder-Assets/SFX/FabSFX_Packs/Sci-Fi_Shots_Pack2_Game_Of_Weapons/Wave/SciFi_Shot_P2__20_.SciFi_Shot_P2__20_" 1.0 1.0 0.0 null null)
  (`/Engine/EditorBlueprintResources/ActorMacros.Switch Has Authority`
    (:`Authority`
      (`self.CommitAbility`)
      (`self.PlayAnimMontage` "/Game/Core/Animations/Cast/Standing2HMagicAreaAttack01_UE_Montage.Standing2HMagicAreaAttack01_UE_Montage"))))

(event `self.OnNotifyBegin`
  (params (NotifyName :type Name))
  (switch `name` NotifyName
    (:`Effect`
      (`/Engine/EditorBlueprintResources/ActorMacros.Switch Has Authority`
        (:`Authority`
          (bind _effectcomponent (message `/Game/Core/Blueprints/Gameplay/Components/EffectComponent/BPI_Effects.GetEffectComponent` (`self.GetOwnerCharacter`)))
          (`/Game/Core/Blueprints/Gameplay/Components/EffectComponent/BPC_EffectComponent.ApplyEffect` _effectcomponent "/Game/Core/Blueprints/Gameplay/Characters/PlayerCharacters/Konga/BP_Effect_InnerResolve.BP_Effect_InnerResolve_C" (`self.GetOwnerCharacter`)))))))

(event `self.OnAnimMontageEnded`
  (`/Engine/EditorBlueprintResources/ActorMacros.Switch Has Authority`
    (:`Authority`
      (`self.EndAbility`))))

(fn `UserConstructionScript`
  (`parent.UserConstructionScript`))