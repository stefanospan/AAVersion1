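; Base character Blueprint that tracks itself with the game's character manager and exposes common gameplay queries.
; On the server, it registers with BPC_CharacterManagerComponent on the GameState at BeginPlay and unregisters at EndPlay.
; Getters expose its effect and stat components, read team from PlayerState, and derive alive status from the stat component's dead flag.
; GetMapEntryComponent is an empty stub here.
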(event `self.ReceiveBeginPlay`
  ; Init
  (`self.Init`))

(event `self.ReceiveEndPlay`
  (params (EndPlayReason :type "EEndPlayReason Enum" :default "Destroyed"))
  ; End Play
  (`/Engine/EditorBlueprintResources/ActorMacros.Switch Has Authority`
    (:`Authority`
      (`/Game/Core/Blueprints/Gameplay/Components/CharacterManagerComponent/BPC_CharacterManagerComponent.UnregisterCharacter` (`self.GetComponentByClass` (`GameplayStatics.GetGameState`) "/Game/Core/Blueprints/Gameplay/Components/CharacterManagerComponent/BPC_CharacterManagerComponent.BPC_CharacterManagerComponent_C") self))))

(fn `GetEffectComponent`
  (returns (EffectComponent :type "/Game/Core/Blueprints/Gameplay/Components/EffectComponent/BPC_EffectComponent Object Reference"))
  (return (`self.BPC_EffectComponent`)))

(fn `GetMapEntryComponent`
  (returns (MapEntryComponent :type "/Game/Core/Blueprints/Gameplay/MapSystemComponent/BPC_MapEntryComponent Object Reference"))
  (return null))

(fn `GetStatsComponent`
  (returns (StatComponent :type "/Game/Core/Blueprints/Gameplay/Components/StatComponent/BPC_StatComponent Object Reference"))
  (return (`self.BPC_StatComponent`)))

(fn `GetTeam`
  (returns (Team :type Integer))
  (bind _team (message `/Game/Core/Blueprints/Gameplay/Components/TeamComponent/BPI_Teams.GetTeam` (`self.PlayerState`)))
  (return _team))

(fn `Init`
  (`/Engine/EditorBlueprintResources/ActorMacros.Switch Has Authority`
    (:`Authority`
      (`/Game/Core/Blueprints/Gameplay/Components/CharacterManagerComponent/BPC_CharacterManagerComponent.RegisterCharacter` (`self.GetComponentByClass` (`GameplayStatics.GetGameState`) "/Game/Core/Blueprints/Gameplay/Components/CharacterManagerComponent/BPC_CharacterManagerComponent.BPC_CharacterManagerComponent_C") self))))

(fn `IsAlive`
  (returns (Success :type Boolean))
  (return (not (`/Game/Core/Blueprints/Gameplay/Components/StatComponent/BPC_StatComponent.GetIsDead` (`self.BPC_StatComponent`)))))

(fn `UserConstructionScript`)