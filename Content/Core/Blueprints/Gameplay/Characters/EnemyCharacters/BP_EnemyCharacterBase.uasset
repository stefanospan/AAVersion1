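; Base enemy character that targets players through its AI Blackboard, shows a health widget and handles death.
; A looping server timer drives target updates, picking the nearest living player pawn from the game mode when the target is invalid or dead.
; Server death stops AI logic, drops rune fragments and sets replicated IsDead, whose OnRep triggers ragdoll and hides the widget.
; Cosmetic-only logic binds the widget to stats and turns it toward the camera.
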(event `self.ReceiveBeginPlay`
  (`parent.ReceiveBeginPlay`)
  (set `self.OriginLocation` (`self.K2_GetActorLocation`))
  (`self.UpdateDead`)
  (`|ExecutionSequence`
    (:`then_0`
      (`/Engine/EditorBlueprintResources/StandardMacros.Can Execute Cosmetic Events`
        (:`True`
          (bind _aswbp_health (cast `/Game/Core/Widgets/Gameplay/Health/WBP_Health` (`WidgetComponent.GetUserWidgetObject` (`self.Widget`))))
          (`/Game/Core/Widgets/Gameplay/Health/WBP_Health.InitStatComponent` _aswbp_health (`self.BPC_StatComponent`)))))
    (:`then_1`
      (`/Engine/EditorBlueprintResources/ActorMacros.Switch Has Authority`
        (:`Authority`
          (bind _returnvalue (`KismetSystemLibrary.K2_SetTimerDelegate` (`|CreateDelegate` :!event `UpdateTarget`) 0.1 true))
          (set `self.UpdateTargetTimer` _returnvalue))))))

(event `UpdateTarget`
  (bind _actor (`self.GetTargetActor`))
  (`/Engine/EditorBlueprintResources/StandardMacros.IsValid` _actor
    (:`Is Valid`
      (bind _success (message `/Game/Core/Blueprints/Gameplay/Components/StatComponent/BPI_Stats.IsAlive` _actor))
      (if (not _success)
        (bind (_found _attacktarget) (`self.FindAttackTarget` :!label _label))
        (if _found
          (`BlackboardComponent.SetValueAsEnum` (`AIBlueprintHelperLibrary.GetBlackboard` null) "State" (enumliteral `/Game/Core/Blueprints/Gameplay/Characters/EnemyCharacters/Enums/E_EnemyStates` "NewEnumerator1"))
          (`BlackboardComponent.SetValueAsObject` (`AIBlueprintHelperLibrary.GetBlackboard` null) "TargetActor" _attacktarget))))
    (:`Is Not Valid`
      (goto _label))))

(event `self.BPC_StatComponent.ServerOnDeath`
  (params (KillerActor :type "Actor Object Reference"))
  (`BrainComponent.StopLogic` (`AIController.BrainComponent` (`AIBlueprintHelperLibrary.GetAIController` self)) "Death")
  (set `self.IsDead` true)
  (`self.SetLifeSpan` 8.0)
  (if (> (`self.DeathRuneFragments`) 0)
    (`|SpawnActorFromClass` "/Game/Core/Blueprints/Gameplay/Components/RuneFragmentsComponent/BP_RuneFragmentsPickup.BP_RuneFragmentsPickup_C" (`KismetMathLibrary.MakeTransform` (- (`self.K2_GetActorLocation`) (`KismetMathLibrary.MakeVector` 0.0 0.0 (`CapsuleComponent.GetScaledCapsuleHalfHeight` (`self.CapsuleComponent`))))) "AlwaysSpawn" "MultiplyWithRoot" null (`self.DeathRuneFragments`) null)))

(event `self.ReceiveTick`
  (params (DeltaSeconds :type "Float (single-precision)"))
  (`parent.ReceiveTick` DeltaSeconds)
  (`/Engine/EditorBlueprintResources/StandardMacros.Can Execute Cosmetic Events`
    (:`True`
      (`SceneComponent.K2_SetWorldRotation` (`self.Widget`) (`KismetMathLibrary.FindLookAtRotation` (`SceneComponent.K2_GetComponentLocation` (`self.Widget`)) (`self.K2_GetActorLocation` (`GameplayStatics.GetPlayerCameraManager` 0))) false false))))

(fn `FindAttackTarget`
  (returns (Found :type Boolean) (AttackTarget :type "Actor Object Reference"))
  (locals (IsFirst :type Boolean :default true) (ClosestActor :type "Actor Object Reference") (ClosestDistance :type "Float (double-precision)") (ActorTemp :type "Actor Object Reference"))
  (bind _closestactor (`local.ClosestActor`))
  (bind _asbp_game_mode_base (cast `/Game/Core/Blueprints/Gameplay/GameMode/BP_GameModeBase` (`GameplayStatics.GetGameMode`)))
  (for _array_element (`/Game/Core/Blueprints/Gameplay/GameMode/BP_GameModeBase.GetPCs` _asbp_game_mode_base)
    (bind _output_get (set `local.ActorTemp` (`Controller.K2_GetPawn` _array_element)))
    (bind _ascharacter (cast `Character` _output_get))
    (bind _success (message `/Game/Core/Blueprints/Gameplay/Components/StatComponent/BPI_Stats.IsAlive` _ascharacter))
    (if _success
      (bind _returnvalue (`KismetMathLibrary.Vector_Distance` (`self.K2_GetActorLocation` _output_get) (`self.K2_GetActorLocation`)))
      (if (or (`local.IsFirst`) (< _returnvalue (`local.ClosestDistance`)))
        (set `local.IsFirst` false)
        (set `local.ClosestActor` (`local.ActorTemp`))
        (set `local.ClosestDistance` _returnvalue))))
  (return (`KismetSystemLibrary.IsValid` _closestactor) _closestactor))

(fn `GetOriginLocation`
  (returns (OriginLocation :type "Vector Structure"))
  (return (`self.OriginLocation`)))

(fn `GetState`
  (returns (State :type "/Game/Core/Blueprints/Gameplay/Characters/EnemyCharacters/Enums/E_EnemyStates Enum"))
  (return (cast `/Game/Core/Blueprints/Gameplay/Characters/EnemyCharacters/Enums/E_EnemyStates` (`BlackboardComponent.GetValueAsEnum` (`AIBlueprintHelperLibrary.GetBlackboard` null) "State"))))

(fn `GetTargetActor`
  (returns (Actor :type "Actor Object Reference"))
  (bind _asactor (cast `Actor` (`BlackboardComponent.GetValueAsObject` (`AIBlueprintHelperLibrary.GetBlackboard` null) "State"))
    (:`then`
      (return _asactor))
    (:`CastFailed`
      (return null))))

(fn `GetTeam`
  (returns (Team :type Integer))
  (return (`/Game/Core/Blueprints/Gameplay/Components/TeamComponent/BPC_TeamComponent.GetTeam` (`self.BPC_TeamComponent`))))

(fn `OnRep_IsDead`
  (`self.UpdateDead`))

(fn `UpdateDead`
  (if (`self.IsDead`)
    (`ActorComponent.Deactivate` (`self.CharacterMovement`))
    (`PrimitiveComponent.SetSimulatePhysics` (`self.Mesh`) true)
    (`PrimitiveComponent.SetCollisionEnabled` (`self.CapsuleComponent`) "NoCollision")
    (`SceneComponent.SetVisibility` (`self.Widget`) false false)))

(fn `UserConstructionScript`
  (`parent.UserConstructionScript`))