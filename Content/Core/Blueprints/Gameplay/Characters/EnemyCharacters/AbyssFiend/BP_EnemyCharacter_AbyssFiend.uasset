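; Abyss Fiend enemy character that gets stronger as days pass and exists only at night.
; On server BeginPlay, HandleDay reads elapsed days from Ultra Dynamic Sky and scales max health, move speed and damage multiplier, capping at day ten.
; It then binds to the GameState wave system's night update, retrying until the GameState is valid, and destroys itself whenever it is not night.
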(event `self.ReceiveBeginPlay`
  (bind _returnvalue (`GameplayStatics.GetGameState`))
  (bind _returnvalue_2 (`self.GetComponentByClass` _returnvalue "/Game/Core/Blueprints/Gameplay/Components/WaveSystemComponent/BPC_WaveSystemComponent.BPC_WaveSystemComponent_C"))
  (`parent.ReceiveBeginPlay`)
  (`/Engine/EditorBlueprintResources/ActorMacros.Switch Has Authority`
    (:`Authority`
      (`self.HandleDay`)
      (`/Engine/EditorBlueprintResources/StandardMacros.IsValid` _returnvalue :!label _label
        (:`Is Valid`
          (add `/Game/Core/Blueprints/Gameplay/Components/WaveSystemComponent/BPC_WaveSystemComponent.OnUpdatedIsNight` _returnvalue_2 (`|CreateDelegate` :!event `OnUpdatedIsNight`))
          (`self.OnUpdatedIsNight` (`/Game/Core/Blueprints/Gameplay/Components/WaveSystemComponent/BPC_WaveSystemComponent.GetIsNight` _returnvalue_2)))
        (:`Is Not Valid`
          (`KismetSystemLibrary.Delay` 0.1)
          (goto _label))))))

(event `OnUpdatedIsNight`
  (params (IsNight :type Boolean))
  (if (not IsNight)
    (`self.K2_DestroyActor`)))

(fn `HandleDay`
  (locals (CurrentDay :type Integer :default 0))
  (bind _uds (`/Game/UltraDynamicSky/Blueprints/Functions/UltraDynamicSky_Functions.Get Ultra Dynamic Sky`))
  (set `local.CurrentDay` (`/Game/UltraDynamicSky/Blueprints/Ultra_Dynamic_Sky.Total Days Elapsed` _uds))
  (`|ExecutionSequence`
    (:`then_0`
      (`/Game/Core/Blueprints/Gameplay/Components/StatComponent/BPC_StatComponent.SetStatMaxValue` (`self.BPC_StatComponent`) (struct :`TagName` "Stat.Health") (`KismetMathLibrary.MapRangeClamped` (/ (`KismetMathLibrary.Conv_IntToDouble` (`local.CurrentDay`)) 10.0) 0.0 1.0 300.0 500.0) false))
    (:`then_1`
      (`/Game/Core/Blueprints/Gameplay/Components/AttributeComponent/BPC_AttributeComponent.AddAdditiveAttribute` (`self.BPC_AttributeComponent`) (make `/Game/Core/Blueprints/Gameplay/Components/AttributeComponent/Structures/ST_AdditiveAttributeData` (struct :`TagName` "Attribute.MoveSpeed") "NewEnumerator1" (`KismetMathLibrary.MapRangeClamped` (/ (`KismetMathLibrary.Conv_IntToDouble` (`local.CurrentDay`)) 10.0) 0.0 1.0 1.0 1.33)))
      (`/Game/Core/Blueprints/Gameplay/Components/AttributeComponent/BPC_AttributeComponent.AddAdditiveAttribute` (`self.BPC_AttributeComponent`) (make `/Game/Core/Blueprints/Gameplay/Components/AttributeComponent/Structures/ST_AdditiveAttributeData` (struct :`TagName` "Attribute.DamageMultiplier") "NewEnumerator1" (`KismetMathLibrary.MapRangeClamped` (/ (`KismetMathLibrary.Conv_IntToDouble` (`local.CurrentDay`)) 10.0) 0.0 1.0 1.0 2.0))))))

(fn `UserConstructionScript`
  (`parent.UserConstructionScript`))