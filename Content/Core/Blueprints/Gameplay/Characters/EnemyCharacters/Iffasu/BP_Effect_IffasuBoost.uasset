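; Status effect for the Iffasu enemy that boosts the attributes of the character it is applied to.
; On application it gets the effect component's owner and adds modifiers to its BPC_AttributeComponent.
; The modifiers cover attack speed, move speed, damage, building health and building time, all using the same modifier type, with only building time set below one.
; The graph contains no removal logic.
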(event `self.OnEffectApplied`
  (bind _returnvalue (`self.GetComponentByClass` (`ActorComponent.GetOwner` (`self.GetEffectComponent`)) "/Game/Core/Blueprints/Gameplay/Components/AttributeComponent/BPC_AttributeComponent.BPC_AttributeComponent_C"))
  (`|ExecutionSequence`
    (:`then_0`
      (`/Game/Core/Blueprints/Gameplay/Components/AttributeComponent/BPC_AttributeComponent.AddAdditiveAttribute` _returnvalue (make `/Game/Core/Blueprints/Gameplay/Components/AttributeComponent/Structures/ST_AdditiveAttributeData` (struct :`TagName` "Attribute.AttackSpeed") "NewEnumerator1" 1.3)))
    (:`then_1`
      (`/Game/Core/Blueprints/Gameplay/Components/AttributeComponent/BPC_AttributeComponent.AddAdditiveAttribute` _returnvalue (make `/Game/Core/Blueprints/Gameplay/Components/AttributeComponent/Structures/ST_AdditiveAttributeData` (struct :`TagName` "Attribute.BuildingHealthMultiplier") "NewEnumerator1" 1.3)))
    (:`then_2`
      (`/Game/Core/Blueprints/Gameplay/Components/AttributeComponent/BPC_AttributeComponent.AddAdditiveAttribute` _returnvalue (make `/Game/Core/Blueprints/Gameplay/Components/AttributeComponent/Structures/ST_AdditiveAttributeData` (struct :`TagName` "Attribute.BuildingTimeMultiplier") "NewEnumerator1" 0.7)))
    (:`then_3`
      (`/Game/Core/Blueprints/Gameplay/Components/AttributeComponent/BPC_AttributeComponent.AddAdditiveAttribute` _returnvalue (make `/Game/Core/Blueprints/Gameplay/Components/AttributeComponent/Structures/ST_AdditiveAttributeData` (struct :`TagName` "Attribute.DamageMultiplier") "NewEnumerator1" 1.3)))
    (:`then_4`
      (`/Game/Core/Blueprints/Gameplay/Components/AttributeComponent/BPC_AttributeComponent.AddAdditiveAttribute` _returnvalue (make `/Game/Core/Blueprints/Gameplay/Components/AttributeComponent/Structures/ST_AdditiveAttributeData` (struct :`TagName` "Attribute.MoveSpeed") "NewEnumerator1" 1.3)))))

(fn `UserConstructionScript`
  (`parent.UserConstructionScript`))