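; Iffasu enemy melee attack ability that damages opposing-team characters in front of it.
; On activation the server commits the ability, plays a random attack montage and multicasts a yaw turn toward the blackboard TargetActor.
; Montage notifies trigger a forward sphere overlap, with a debug sphere drawn, that filters out teammates and applies damage scaled by the DamageMultiplier attribute.
; The server ends the ability when the montage ends.
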(event `self.OnAbilityActivated`
  (bind (_returnvalue_roll _returnvalue_pitch _returnvalue_yaw) (`KismetMathLibrary.BreakRotator` (`KismetMathLibrary.FindLookAtRotation` (`self.K2_GetActorLocation` (`self.GetOwner`)) (`self.K2_GetActorLocation` (`self.GetTargetActor`)))))
  (`/Engine/EditorBlueprintResources/ActorMacros.Switch Has Authority`
    (:`Authority`
      (`self.CommitAbility`)
      (`self.PlayAnimMontage` (`KismetArrayLibrary.Array_Random` (`self.AttackAnimMontages`)))
      (`self.MulticastSetActorRotation` (`KismetMathLibrary.MakeRotator` 0.0 0.0 _returnvalue_yaw)))))

(event `self.OnNotifyBegin`
  (params (NotifyName :type Name))
  (switch `name` NotifyName
    (:`Attack`
      (`/Engine/EditorBlueprintResources/ActorMacros.Switch Has Authority`
        (:`Authority`
          (bind _actors (`self.GetAttackActors`))
          (for _array_element _actors
            (`GameplayStatics.ApplyDamage` _array_element (* (`self.Damage`) (`.Value_5_5382FAD64776275FF614BEB1A224EFA3` (break `/Game/Core/Blueprints/Gameplay/Components/AttributeComponent/Structures/ST_AttributeData` (`self.GetAttribute` (struct :`TagName` "Attribute.DamageMultiplier"))))) null (`self.GetOwnerCharacter`))))))))

(event `self.OnAnimMontageEnded`
  (`/Engine/EditorBlueprintResources/ActorMacros.Switch Has Authority`
    (:`Authority`
      (`self.EndAbility`))))

(event `MulticastSetActorRotation`
  (params (NewRotation :type "Rotator Structure"))
  (`self.K2_SetActorRotation` (`self.GetOwnerCharacter`) NewRotation false))

(fn `GetAttackActors`
  (returns (Actors :type "Array of Actor Object Reference"))
  (locals (ActorsTemp :type "Array of Actor Object Reference"))
  (bind _ownercharacter (`self.GetOwnerCharacter`))
  (bind _returnvalue (+ (`self.K2_GetActorLocation` _ownercharacter) (* (`self.GetActorForwardVector` _ownercharacter) 100.0)))
  (bind _team (message `/Game/Core/Blueprints/Gameplay/Components/TeamComponent/BPI_Teams.GetTeam` _ownercharacter))
  (`KismetSystemLibrary.DrawDebugSphere` _returnvalue 100.0 12 (struct :`R` 1.0 :`G` 0.036852 :`A` 1.0) 3.0 1.0)
  (bind _outactors (`KismetSystemLibrary.SphereOverlapActors` _returnvalue 100.0 (`|MakeArray` "ObjectTypeQuery3" :!type "EObjectTypeQuery Enum") "/Game/Core/Blueprints/Gameplay/Characters/BP_CharacterBase.BP_CharacterBase_C" (`|MakeArray` (`self.GetOwnerCharacter`) :!type "Actor Object Reference")))
  (for _array_element _outactors
    (bind _team_2 (message `/Game/Core/Blueprints/Gameplay/Components/TeamComponent/BPI_Teams.GetTeam` _array_element))
    (if (!= _team_2 _team)
      (`KismetArrayLibrary.Array_Add` (`local.ActorsTemp`) _array_element)))
  (return (`local.ActorsTemp`)))

(fn `GetTargetActor`
  (returns (TargetActor :type "Actor Object Reference"))
  (bind _asactor (cast `Actor` (`BlackboardComponent.GetValueAsObject` (`AIBlueprintHelperLibrary.GetBlackboard` (`self.GetOwnerCharacter`)) "TargetActor")))
  (return _asactor))

(fn `UserConstructionScript`
  (`parent.UserConstructionScript`))