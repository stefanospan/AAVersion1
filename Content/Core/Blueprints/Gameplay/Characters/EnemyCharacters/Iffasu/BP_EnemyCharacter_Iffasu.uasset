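; Iffasu enemy character that periodically spawns minions and teleports around the level, dropping a boost pickup on death.
; On BeginPlay, the server starts looping timers for both behaviors and caches all enemy spawn areas as teleport destinations.
; Minions are random picks from a configurable class list, placed at reachable points around Iffasu.
; Death spawns an IffasuBoost effect pickup at a reachable point nearby.
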(event `self.ReceiveBeginPlay`
  (`parent.ReceiveBeginPlay`)
  (`/Engine/EditorBlueprintResources/ActorMacros.Switch Has Authority`
    (:`Authority`
      (`|ExecutionSequence`
        (:`then_0`
          (bind _returnvalue (`KismetSystemLibrary.K2_SetTimerDelegate` (`|CreateDelegate` :!event `SpawnCreatures`) (`self.SpawnCreaturesRate`) true))
          (set `self.SpawnCreaturesTimer` _returnvalue))
        (:`then_1`
          (bind _outactors (`GameplayStatics.GetAllActorsOfClass` "/Game/Core/Blueprints/Gameplay/Characters/EnemyCharacters/BP_EnemySpawnArea.BP_EnemySpawnArea_C"))
          (set `self.SpawnAreas` _outactors)
          (bind _returnvalue_2 (`KismetSystemLibrary.K2_SetTimerDelegate` (`|CreateDelegate` :!event `Teleport`) (`self.TeleportRate`) true))
          (set `self.TeleportTimer` _returnvalue_2))))))

(event `self.BPC_StatComponent.ServerOnDeath`
  (params (KillerActor :type "Actor Object Reference"))
  (`|SpawnActorFromClass` "/Game/Core/Blueprints/Gameplay/Components/EffectComponent/BP_EffectPickup.BP_EffectPickup_C" (`KismetMathLibrary.MakeTransform` (`NavigationSystemV1.K2_GetRandomReachablePointInRadius` (`self.K2_GetActorLocation`) 200.0 null null)) "AlwaysSpawn" "MultiplyWithRoot" null "/Game/Core/Blueprints/Gameplay/Characters/EnemyCharacters/Iffasu/BP_Effect_IffasuBoost.BP_Effect_IffasuBoost_C" null))

(fn `SpawnCreatures`
  (if (> (`KismetArrayLibrary.Array_Length` (`self.SpawnableCreatures`)) 0)
    (for _ (range (`self.SpawnCreaturesAmount`))
      (`|SpawnActorFromClass` (`KismetArrayLibrary.Array_Random` (`self.SpawnableCreatures`)) (`KismetMathLibrary.MakeTransform` (`NavigationSystemV1.K2_GetRandomReachablePointInRadius` (`self.K2_GetActorLocation`) (`self.SpawnCreaturesRadius`) null null)) "Undefined" "MultiplyWithRoot" null null))))

(fn `Teleport`
  (bind _spawnareas (`self.SpawnAreas`))
  (if (> (`KismetArrayLibrary.Array_Length` _spawnareas) 0)
    (`self.K2_TeleportTo` (.location (`self.GetTransform` (`KismetArrayLibrary.Array_Random` _spawnareas))) (.rotation (`self.GetTransform` (`KismetArrayLibrary.Array_Random` _spawnareas))))))

(fn `UserConstructionScript`
  (`parent.UserConstructionScript`))