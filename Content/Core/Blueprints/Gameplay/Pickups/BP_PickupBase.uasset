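; Base pickup actor that grants an amount of an item class to actors with a BPC_InventoryComponent that overlap it.
; Its mesh comes from the item class defaults, set on BeginPlay and refreshed through OnRep when the class replicates.
; The server enables sphere query collision after a short delay and handles overlaps.
; AddItem's return value is kept as the remaining Amount, and the pickup destroys itself when that is zero.
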(event `self.ReceiveBeginPlay`
  (`self.UpdateVisuals`)
  (`/Engine/EditorBlueprintResources/ActorMacros.Switch Has Authority`
    (:`Authority`
      (`KismetSystemLibrary.Delay` 0.65)
      (`PrimitiveComponent.SetCollisionEnabled` (`self.Sphere`) "QueryOnly"))))

(event `self.ReceiveActorBeginOverlap`
  (params (OtherActor :type "Actor Object Reference"))
  (bind _returnvalue (`self.GetComponentByClass` OtherActor "/Game/Core/Blueprints/Gameplay/Components/InventoryComponent/BPC_InventoryComponent.BPC_InventoryComponent_C"))
  (`/Engine/EditorBlueprintResources/ActorMacros.Switch Has Authority`
    (:`Authority`
      (`/Engine/EditorBlueprintResources/StandardMacros.IsValid` _returnvalue
        (:`Is Valid`
          (bind _remainingamount (`/Game/Core/Blueprints/Gameplay/Components/InventoryComponent/BPC_InventoryComponent.AddItem` _returnvalue (`self.ItemClass`) (`self.Amount`)))
          (if (== _remainingamount 0)
            (`self.K2_DestroyActor`)
            (else
              (set `self.Amount` _remainingamount))))))))

(fn `OnRep_ItemClass`
  (`self.UpdateVisuals`))

(fn `UpdateVisuals`
  (`self.ItemClass`
    (:`then`
      (`StaticMeshComponent.SetStaticMesh` (`self.StaticMesh`) (`.ItemMesh_14_FE008AFC4E8A84E40564718AEDF885CD` (break `/Game/Core/Blueprints/Gameplay/Components/InventoryComponent/Structures/ST_ItemData` (defaults `Object` (`self.ItemClass`))))))
    (:`else`)))

(fn `UserConstructionScript`)