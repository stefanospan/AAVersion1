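; BP_PlayerStateLobby is the lobby player state, holding each player's selected character and exposing their team.
; SelectedCharacter has a getter and setter, and its OnRep handler calls the OnUpdatedSelectedCharacter dispatcher with the new value.
; GetTeam delegates to the BPC team component, while the event graph and construction script are empty.
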(fn `GetSelectedCharacter`
  (returns (SelectedCharacter :type "Object Soft Class Reference"))
  (return (`self.SelectedCharacter`)))

(fn `GetTeam`
  (returns (Team :type Integer))
  (return (`/Game/Core/Blueprints/Gameplay/Components/TeamComponent/BPC_TeamComponent.GetTeam` (`self.BPC_TeamComponent`))))

(fn `OnRep_SelectedCharacter`
  (`self.OnUpdatedSelectedCharacter` (`self.SelectedCharacter`)))

(fn `SetSelectedCharacter`
  (params (SelectedCharacter :type "Object Soft Class Reference"))
  (set `self.SelectedCharacter` SelectedCharacter))

(fn `UserConstructionScript`)