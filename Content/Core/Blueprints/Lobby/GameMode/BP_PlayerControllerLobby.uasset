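; Lobby player controller that handles character selection before a match.
; On BeginPlay it switches to Game and UI input and shows the mouse cursor for the first local player.
; A server select event validates the soft class reference and accepts only the first pick, storing it on the lobby player state.
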(event `self.ReceiveBeginPlay`
  ; Init
  (`self.Init`))

(event `ServerSelectCharacter`
  (params (Character :type "Object Soft Class Reference"))
  ; Sets selected character on server
  (if (`KismetSystemLibrary.IsValidSoftClassReference` Character)
    (if (not (`self.HasSelectedCharacter`))
      (set `self.HasSelectedCharacter` true)
      (bind _asbp_player_state_lobby (cast `/Game/Core/Blueprints/Lobby/GameMode/BP_PlayerStateLobby` (`self.PlayerState`)))
      (`/Game/Core/Blueprints/Lobby/GameMode/BP_PlayerStateLobby.SetSelectedCharacter` _asbp_player_state_lobby Character))))

(fn `Init`
  (`WidgetBlueprintLibrary.SetInputMode_GameAndUIEx` (`GameplayStatics.GetPlayerController` 0) null "DoNotLock" false)
  (set `PlayerController.bShowMouseCursor` true (`GameplayStatics.GetPlayerController` 0)))

(fn `UserConstructionScript`)