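; Lobby game state Blueprint that holds the selected island and the list of registered player states.
; Both variables use RepNotify functions that fire event dispatchers, so listeners learn when either one updates.
; Register and unregister functions edit the player array, then assign it back to itself, apparently to trigger the notify.
; Simple getters and a setter expose the state to other classes.
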(fn `GetPlayerStates`
  (returns (PlayerStates :type "Array of /Game/Core/Blueprints/Lobby/GameMode/BP_PlayerStateLobby Object Reference"))
  (return (`self.PlayerStates`)))

(fn `GetSelectedIsland`
  (returns (SelectedIsland :type "Object Soft Object Reference"))
  (return (`self.SelectedIsland`)))

(fn `OnRep_PlayerStates`
  (`self.OnUpdatedPlayerStates` (`self.PlayerStates`)))

(fn `OnRep_SelectedIsland`
  (`self.OnUpdatedSelectedIsland` (`self.SelectedIsland`)))

(fn `RegisterPlayerState`
  (params (PlayerState :type "/Game/Core/Blueprints/Lobby/GameMode/BP_PlayerStateLobby Object Reference (by ref)"))
  (`KismetArrayLibrary.Array_Add` (`self.PlayerStates`) PlayerState)
  (set `self.PlayerStates` (`self.PlayerStates`)))

(fn `SetSelectedIsland`
  (params (SelectedIsland :type "Object Soft Object Reference"))
  (set `self.SelectedIsland` SelectedIsland))

(fn `UnregisterPlayerState`
  (params (PlayerState :type "/Game/Core/Blueprints/Lobby/GameMode/BP_PlayerStateLobby Object Reference (by ref)"))
  (`KismetArrayLibrary.Array_RemoveItem` (`self.PlayerStates`) PlayerState)
  (set `self.PlayerStates` (`self.PlayerStates`)))

(fn `UserConstructionScript`)