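; Lobby game mode that runs timed team and character selection, then server-travels players into a match on a randomly picked island.
; Game State timer completions chain the phases, balancing unassigned players across teams and giving undecided players random characters.
; At match start it saves each player's ID, character and team, plus the island, to the Game Instance.
; It tracks lobby players and shuts down a dedicated server when the last leaves.
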(event `self.ReceiveBeginPlay`
  (`self.StartTeamSelection`)
  (`self.SelectRandomIsland`))

(event `SelectRandomIsland`
  (bind _outprimaryassetidlist (`KismetSystemLibrary.GetPrimaryAssetIdList` "PDA_IslandBase_C"))
  (`/Game/Core/Blueprints/Lobby/GameMode/BP_GameStateLobby.SetSelectedIsland` (`self.GetGameState`) (`KismetSystemLibrary.GetSoftObjectReferenceFromPrimaryAssetId` (`KismetArrayLibrary.Array_Random` _outprimaryassetidlist))))

(event `self.K2_PostLogin`
  (params (NewPlayer :type "PlayerController Object Reference"))
  (bind _asbp_player_controller_lobby (cast `/Game/Core/Blueprints/Lobby/GameMode/BP_PlayerControllerLobby` NewPlayer))
  (`KismetArrayLibrary.Array_Add` (`self.PCs`) _asbp_player_controller_lobby)
  (bind _asbp_player_state_lobby (cast `/Game/Core/Blueprints/Lobby/GameMode/BP_PlayerStateLobby` (`Controller.PlayerState` _asbp_player_controller_lobby)))
  (`/Game/Core/Blueprints/Lobby/GameMode/BP_GameStateLobby.RegisterPlayerState` (`self.GetGameState`) _asbp_player_state_lobby))

(event `self.K2_OnLogout`
  (params (ExitingController :type "Controller Object Reference"))
  (bind _asbp_player_controller_lobby (cast `/Game/Core/Blueprints/Lobby/GameMode/BP_PlayerControllerLobby` ExitingController))
  (`KismetArrayLibrary.Array_RemoveItem` (`self.PCs`) _asbp_player_controller_lobby)
  (bind _asbp_player_state_lobby (cast `/Game/Core/Blueprints/Lobby/GameMode/BP_PlayerStateLobby` (`Controller.PlayerState` _asbp_player_controller_lobby)))
  (`/Game/Core/Blueprints/Lobby/GameMode/BP_GameStateLobby.UnregisterPlayerState` (`self.GetGameState`) _asbp_player_state_lobby)
  (if (and (== (`KismetArrayLibrary.Array_Length` (`self.PCs`)) 0) (`KismetSystemLibrary.IsDedicatedServer`))
    (`self.ShutdownServer`)))

(event `StartTeamSelection`
  (bind _bpc_timercomponent (`/Game/Core/Blueprints/Lobby/GameMode/BP_GameStateLobby.BPC_TimerComponent` (`self.GetGameState`)))
  (add `/Game/Core/Blueprints/Gameplay/Components/TimerComponent/BPC_TimerComponent.OnTimerCompleted` _bpc_timercomponent (`|CreateDelegate` :!event `OnTeamSelectionTimerCompleted`))
  (`/Game/Core/Blueprints/Gameplay/Components/TimerComponent/BPC_TimerComponent.StartTimer` _bpc_timercomponent (`self.LobbyTime`)))

(event `StartMatch`
  (`self.SelectUnselectedCharacters`)
  (`self.ProcessTransitionData`)
  (bind _object (`|LoadAsset` (`/Game/Core/Blueprints/Lobby/GameMode/BP_GameStateLobby.GetSelectedIsland` (`self.GetGameState`)))
    (:`Completed`
      (bind _aspda_island_base (cast `/Game/Core/Blueprints/Gameplay/Islands/PDA_IslandBase` _object))
      (`KismetSystemLibrary.ExecuteConsoleCommand` (`KismetStringLibrary.Concat_StrStr` "servertravel " (`KismetStringLibrary.Conv_NameToString` (`.LevelName_5_194F572D4FE5B7F8D9EA9E91ED76EDC7` (break `/Game/Core/Blueprints/Gameplay/Islands/Structures/ST_IslandData` (`/Game/Core/Blueprints/Gameplay/Islands/PDA_IslandBase.IslandData` _aspda_island_base))))) null))))

(event `StartCharacterSelection`
  (`self.StartTimer`)
  (`/Game/Core/Blueprints/Lobby/GameMode/BP_GameStateLobby.SetIsTeamSelection` (`self.GetGameState`) false))

(fn `GetGameState`
  (returns (GameState :type "/Game/Core/Blueprints/Lobby/GameMode/BP_GameStateLobby Object Reference"))
  (bind _gamestateref (`self.GameStateRef`)
    (:`then`
      (return _gamestateref))
    (:`else`
      (bind _asbp_game_state_lobby (cast `/Game/Core/Blueprints/Lobby/GameMode/BP_GameStateLobby` (`GameplayStatics.GetGameState`)))
      (return _asbp_game_state_lobby))))

(fn `OnTeamSelectionTimerCompleted`
  (remove `/Game/Core/Blueprints/Gameplay/Components/TimerComponent/BPC_TimerComponent.OnTimerCompleted` (`/Game/Core/Blueprints/Lobby/GameMode/BP_GameStateLobby.BPC_TimerComponent` (`self.GetGameState`)) (`|CreateDelegate` :!event `OnTeamSelectionTimerCompleted`))
  (`self.SelectUnselectedTeams`)
  (`self.StartCharacterSelection`))

(fn `OnTimerCompleted`
  (remove `/Game/Core/Blueprints/Gameplay/Components/TimerComponent/BPC_TimerComponent.OnTimerCompleted` (`/Game/Core/Blueprints/Lobby/GameMode/BP_GameStateLobby.BPC_TimerComponent` (`self.GetGameState`)) (`|CreateDelegate` :!event `OnTimerCompleted`))
  (`self.StartMatch`))

(fn `ProcessTransitionData`
  (locals (PlayerTransitionDataTemp :type "Array of /Game/Core/Blueprints/Lobby/GameMode/Structures/ST_PlayerTransitionData Structure"))
  (`|ExecutionSequence`
    (:`then_0`
      (for _array_element (`self.PCs`)
        (bind _team (message `/Game/Core/Blueprints/Gameplay/Components/TeamComponent/BPI_Teams.GetTeam` _array_element))
        (bind _asbp_player_state_lobby (cast `/Game/Core/Blueprints/Lobby/GameMode/BP_PlayerStateLobby` (`Controller.PlayerState` _array_element)))
        (bind _returnvalue (`KismetSystemLibrary.LoadClassAsset_Blocking` (`/Game/Core/Blueprints/Lobby/GameMode/BP_PlayerStateLobby.GetSelectedCharacter` _asbp_player_state_lobby)))
        (bind _asbp_player_character_base (castclass `/Game/Core/Blueprints/Gameplay/Characters/PlayerCharacters/BP_PlayerCharacterBase` _returnvalue))
        (`KismetArrayLibrary.Array_Add` (`local.PlayerTransitionDataTemp`) (make `/Game/Core/Blueprints/Lobby/GameMode/Structures/ST_PlayerTransitionData` (`PlayerState.BP_GetUniqueId` _asbp_player_state_lobby) _asbp_player_character_base _team))))
    (:`then_1`
      (bind _asbp_game_instance (cast `/Game/Core/Blueprints/GameInstance/BP_GameInstance` (`GameplayStatics.GetGameInstance`)))
      (set `/Game/Core/Blueprints/GameInstance/BP_GameInstance.PlayerTransitionData` (`local.PlayerTransitionDataTemp`) _asbp_game_instance)
      (bind _returnvalue_2 (`KismetSystemLibrary.LoadAsset_Blocking` (`/Game/Core/Blueprints/Lobby/GameMode/BP_GameStateLobby.GetSelectedIsland` (`self.GetGameState`))))
      (bind _aspda_island_base (cast `/Game/Core/Blueprints/Gameplay/Islands/PDA_IslandBase` _returnvalue_2))
      (set `/Game/Core/Blueprints/GameInstance/BP_GameInstance.SelectedIsland` _aspda_island_base _asbp_game_instance))))

(fn `SelectUnselectedCharacters`
  (locals (CharacterAssets :type "Array of PrimaryAssetId Structure"))
  (bind _outprimaryassetidlist (`KismetSystemLibrary.GetPrimaryAssetIdList` "BP_PlayerCharacterBase_C"))
  (set `local.CharacterAssets` _outprimaryassetidlist)
  (for _array_element (`self.PCs`)
    (bind _asbp_player_state_lobby (cast `/Game/Core/Blueprints/Lobby/GameMode/BP_PlayerStateLobby` (`Controller.PlayerState` _array_element)))
    (if (not (`KismetSystemLibrary.IsValidSoftClassReference` (`/Game/Core/Blueprints/Lobby/GameMode/BP_PlayerStateLobby.GetSelectedCharacter` _asbp_player_state_lobby)))
      (`/Game/Core/Blueprints/Lobby/GameMode/BP_PlayerStateLobby.SetSelectedCharacter` _asbp_player_state_lobby (`KismetSystemLibrary.GetSoftClassReferenceFromPrimaryAssetId` (`KismetArrayLibrary.Array_Random` (`local.CharacterAssets`)))))))

(fn `SelectUnselectedTeams`
  (locals (TeamA :type Integer) (TeamB :type Integer) (UnassignedPlayerStates :type "Array of /Game/Core/Blueprints/Lobby/GameMode/BP_PlayerStateLobby Object Reference") (TeamTemp :type Integer))
  (for _array_element (`/Game/Core/Blueprints/Lobby/GameMode/BP_GameStateLobby.GetPlayerStates` (`self.GetGameState`))
    (bind _team (message `/Game/Core/Blueprints/Gameplay/Components/TeamComponent/BPI_Teams.GetTeam` _array_element))
    (switch `int` _team
      (:`-1`
        (`KismetArrayLibrary.Array_Add` (`local.UnassignedPlayerStates`) _array_element))
      (:`0`
        (`/Engine/EditorBlueprintResources/StandardMacros.IncrementInt` (`local.TeamA`)))
      (:`1`
        (`/Engine/EditorBlueprintResources/StandardMacros.IncrementInt` (`local.TeamB`)))))
  (for _index (range (`KismetMathLibrary.Min` (`KismetMathLibrary.Abs_Int` (- (`local.TeamA`) (`local.TeamB`))) (`KismetArrayLibrary.Array_Length` (`local.UnassignedPlayerStates`))))
    (`/Game/Core/Blueprints/Gameplay/Components/TeamComponent/BPC_TeamComponent.SetTeam` (`/Game/Core/Blueprints/Lobby/GameMode/BP_PlayerStateLobby.BPC_TeamComponent` (`|GetArrayItem` (`local.UnassignedPlayerStates`) _index)) (select `bool` (> (`local.TeamA`) (`local.TeamB`)) :`true` 1)))
  (if (> (`KismetArrayLibrary.Array_Length` (`local.UnassignedPlayerStates`)) (`KismetMathLibrary.Abs_Int` (- (`local.TeamA`) (`local.TeamB`))))
    (set `local.TeamTemp` (- 1 (select `bool` (> (`local.TeamA`) (`local.TeamB`)) :`true` 1)))
    (for _index_2 (range (`KismetMathLibrary.Abs_Int` (- (`local.TeamA`) (`local.TeamB`))) (+ (`KismetArrayLibrary.Array_LastIndex` (`local.UnassignedPlayerStates`)) 1))
      (`/Game/Core/Blueprints/Gameplay/Components/TeamComponent/BPC_TeamComponent.SetTeam` (`/Game/Core/Blueprints/Lobby/GameMode/BP_PlayerStateLobby.BPC_TeamComponent` (`|GetArrayItem` (`local.UnassignedPlayerStates`) _index_2)) (`local.TeamTemp`))
      (set `local.TeamTemp` (- 1 (`local.TeamTemp`))))))

(fn `StartTimer`
  (bind _bpc_timercomponent (`/Game/Core/Blueprints/Lobby/GameMode/BP_GameStateLobby.BPC_TimerComponent` (`self.GetGameState`)))
  (add `/Game/Core/Blueprints/Gameplay/Components/TimerComponent/BPC_TimerComponent.OnTimerCompleted` _bpc_timercomponent (`|CreateDelegate` :!event `OnTimerCompleted`))
  (`/Game/Core/Blueprints/Gameplay/Components/TimerComponent/BPC_TimerComponent.StartTimer` _bpc_timercomponent (`self.LobbyTime`)))

(fn `UserConstructionScript`)